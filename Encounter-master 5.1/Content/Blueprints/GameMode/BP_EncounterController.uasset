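; Player controller for encounters that forwards input actions to the player character for four-direction movement and three attack actions.
; On BeginPlay it caches the character and BP_Camera references and sets game-only input.
; The ChargeMods input enters the character's equip mode only when energy is full.
; Pause spawns the pause menu widget, pauses the game and switches to UI-only input with a visible cursor through SetInputMode.
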(event EventBeginPlay
  ;[1 1 1] Event BeginPlay
  (Utilities|CastReferences)
  (Input|SetInputModeGameOnly self false))

(event Input|ActionEvents|InputActionMoveNorth
  (params (Key :type Key%20Structure :default "None"))
  ;[1 1 1] Player Movement
  (:Pressed
    (Default|MoveNorth (Variables|Default|GetCharacterRef))))

(event Input|ActionEvents|InputActionMoveSouth
  (params (Key :type Key%20Structure :default "None"))
  ;[1 1 1] Player Movement
  (:Pressed
    (Default|MoveSouth (Variables|Default|GetCharacterRef))))

(event Input|ActionEvents|InputActionMoveWest
  (params (Key :type Key%20Structure :default "None"))
  ;[1 1 1] Player Movement
  (:Pressed
    (Default|MoveWest (Variables|Default|GetCharacterRef))))

(event Input|ActionEvents|InputActionMoveEast
  (params (Key :type Key%20Structure :default "None"))
  ;[1 1 1] Player Movement
  (:Pressed
    (Default|MoveEast (Variables|Default|GetCharacterRef))))

(event Input|ActionEvents|InputActionAction:1
  (params (Key :type Key%20Structure :default "None"))
  ;[1 1 1] Player Attack
  (:Pressed
    (Default|Action:Basic (Variables|Default|GetCharacterRef))))

(event Input|ActionEvents|InputActionPause
  (params (Key :type Key%20Structure :default "None"))
  ;[1 1 1] Pause
  (:Pressed
    (bind _returnvalue (UserInterface|CreateWidget "/Game/UserInterface/WBP_PauseMenu.WBP_PauseMenu_C"))
    (UserInterface|Viewport|AddtoViewport _returnvalue 0)
    (Game|SetGamePaused true)
    (CallFunction|SetInputMode true)))

(event Input|ActionEvents|InputActionAction:2
  (params (Key :type Key%20Structure :default "None"))
  ;[1 1 1] Player Attack
  (:Pressed
    (Default|Action:Cannon (Variables|Default|GetCharacterRef))))

(event Input|ActionEvents|InputActionChargeMods
  (params (Key :type Key%20Structure :default "None"))
  (bind _characterref (Variables|Default|GetCharacterRef))
  (:Pressed
    (if (>= (Variables|/Game/Character/BP_PlayerCharacter.BP_PlayerCharacter_C|GetCurrentEnergyPoints _characterref) (Variables|/Game/Character/BP_PlayerCharacter.BP_PlayerCharacter_C|GetMaxEnergyPoints _characterref))
      (Default|GoEquipMode _characterref))))

(event Input|ActionEvents|InputActionAction:3
  (params (Key :type Key%20Structure :default "None"))
  ;[1 1 1] Player Attack
  (:Pressed
    (Default|Action:Second (Variables|Default|GetCharacterRef))))

(fn ConstructionScript)

(fn SetInputMode
  (params (InputModeUI :type Boolean))
  (bind _self self)
  (if InputModeUI
    (Input|SetInputModeUIOnly _self 0 "DoNotLock" false)
    (Variables|Default|SetbShowMouseCursor true)
    (else
      (Input|SetInputModeGameOnly _self false)
      (Variables|Default|SetbShowMouseCursor false))))