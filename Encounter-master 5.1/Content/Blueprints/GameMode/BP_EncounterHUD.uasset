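; BP_EncounterHUD is a HUD Blueprint that puts the basic HUD widget on screen and handles switching between UI and game input.
; BeginPlay creates WBP_BasicHUD and adds it to the viewport.
; SetInputMode takes a boolean and sets the first player controller to either UI-only input with an unlocked, visible cursor or game-only input with the cursor hidden.
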(event EventBeginPlay
  (bind _returnvalue (UserInterface|CreateWidget "/Game/UserInterface/WBP_BasicHUD.WBP_BasicHUD_C"))
  (UserInterface|Viewport|AddtoViewport _returnvalue 0))

(fn ConstructionScript)

(fn SetInputMode
  (params (InputModeUI :type Boolean))
  (LocalVariables|SetControllerRef (Game|GetPlayerController 0))
  (if InputModeUI
    (Input|SetInputModeUIOnly (LocalVariables|GetControllerRef) 0 "DoNotLock")
    (Variables|/Script/Engine.PlayerController|SetbShowMouseCursor (LocalVariables|GetControllerRef) true)
    (else
      (Input|SetInputModeGameOnly (LocalVariables|GetControllerRef))
      (Variables|/Script/Engine.PlayerController|SetbShowMouseCursor (LocalVariables|GetControllerRef) false))))