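; BP_GridTile is a single grid tile that tracks its occupying actor and whether it belongs to the player or enemy side.
; Side setters store the grid type and tint a dynamic floor material blue for player or red for enemy.
; Construction caches a world position slightly above the tile.
; After a short BeginPlay delay, it builds its surrounding-tile list from four neighbor references, deriving diagonals through the north and south neighbors.
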(event EventBeginPlay
  (bind _returnvalue (Rendering|Material|CreateDynamicMaterialInstance "/Game/Material/M_NewFloorTile.M_NewFloorTile" "None" "None" :!class /Script/Engine.KismetMaterialLibrary))
  (Variables|Default|SetMaterialInstance _returnvalue)
  (Utilities|FlowControl|Delay 0.2)
  (CallFunction|SetSurroundingTiles))

(fn ConstructionScript
  (Variables|GridInfo|SetGridWorldLocation (+ (Transformation|GetWorldLocation (Variables|Default|GetDefaultSceneRoot)) "0, 0,10.000000")))

(fn OccupyTile
  (params (Actor :type Actor%20Object%20Reference))
  (Variables|GridInfo|SetOccupyingActor Actor)
  (Variables|GridInfo|SetIsOccupied true)
  (return))

(fn EmptyTile
  (Variables|GridInfo|SetOccupyingActor 0)
  (Variables|GridInfo|SetIsOccupied false)
  (return))

(fn SettoPlayerTile
  (Variables|GridInfo|SetGridType "NewEnumerator0")
  (Rendering|Material|SetVectorParameterValue (Variables|Default|GetMaterialInstance) "TileColor" "(R=0.000000,G=0.000000,B=1.000000,A=1.000000)" :!class /Script/Engine.MaterialInstanceDynamic)
  (Rendering|Material|SetMaterial (Variables|Default|GetTile) 0 (Variables|Default|GetMaterialInstance)))

(fn SettoEnemyTile
  (Variables|GridInfo|SetGridType "NewEnumerator1")
  (Rendering|Material|SetVectorParameterValue (Variables|Default|GetMaterialInstance) "TileColor" "(R=1.000000,G=0.000000,B=0.000000,A=1.000000)" :!class /Script/Engine.MaterialInstanceDynamic)
  (Rendering|Material|SetMaterial (Variables|Default|GetTile) 0 (Variables|Default|GetMaterialInstance)))

(fn SetSurroundingTiles
  (bind _neighboreast (Variables|Neighbors|GetNeighborEast)
    (:then
      (Utilities|Array|Add (Variables|Neighbors|GetSurroundingTiles) _neighboreast))
    (:else
      _))
  (bind _neighborwest (Variables|Neighbors|GetNeighborWest)
    (:then
      (Utilities|Array|Add (Variables|Neighbors|GetSurroundingTiles) _neighborwest))
    (:else
      _))
  (bind _neighbornorth (Variables|Neighbors|GetNeighborNorth)
    (:then
      (Utilities|Array|Add (Variables|Neighbors|GetSurroundingTiles) _neighbornorth)
      (bind _neighboreast_2 (Variables|BP_GridTile_C|GetNeighborEast _neighbornorth)
        (:then
          (Utilities|Array|Add (Variables|Neighbors|GetSurroundingTiles) _neighboreast_2))
        (:else
          _))
      (bind _neighborwest_2 (Variables|BP_GridTile_C|GetNeighborWest _neighbornorth)
        (:then
          (Utilities|Array|Add (Variables|Neighbors|GetSurroundingTiles) _neighborwest_2))
        (:else
          _)))
    (:else
      _))
  (bind _neighborsouth (Variables|Neighbors|GetNeighborSouth)
    (:then
      (Utilities|Array|Add (Variables|Neighbors|GetSurroundingTiles) _neighborsouth)
      (bind _neighboreast_3 (Variables|BP_GridTile_C|GetNeighborEast _neighborsouth)
        (:then
          (Utilities|Array|Add (Variables|Neighbors|GetSurroundingTiles) _neighboreast_3))
        (:else
          _))
      (bind _neighborwest_3 (Variables|BP_GridTile_C|GetNeighborWest _neighborsouth)
        (:then
          (Utilities|Array|Add (Variables|Neighbors|GetSurroundingTiles) _neighborwest_3))
        (:else)))
    (:else)))