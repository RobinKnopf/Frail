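; Grid manager that builds the board at BeginPlay, splitting it into a player half and an enemy half.
; SpawnGrid spawns BP_GridTile actors centered on the world origin into a flat GridArray and numbers them by index.
; SetTilesTypes assigns each half its side, then four helpers link orthogonal neighbors through GridY-stride index math with edge checks, also filling each tile's ValidNeighbors.
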(event EventBeginPlay
  (CallFunction|SpawnGrid)
  (CallFunction|SetTilesTypes)
  (CallFunction|SetGridCellNeighbors))

(fn ConstructionScript)

(fn SpawnGrid
  (bind (_offsetx _offsety) (CallFunction|CalculateWorldOffset))
  (bind _tilesize (Variables|Grid|GetTileSize))
  (bind _gridarray (Variables|Grid|GetGridArray))
  (Utilities|Array|Clear (Variables|Grid|GetGridArray))
  (LocalVariables|SetWorldOffsetX _offsetx)
  (LocalVariables|SetWorldOffsetY _offsety)
  (for _index (range 0 (- (Variables|Grid|GetGridX) 1))
    (for _index_2 (range 0 (- (Variables|Grid|GetGridY) 1))
      (bind _returnvalue (Game|SpawnActorfromClass "/Game/Blueprints/Grid/BP_GridTile.BP_GridTile_C" (Math|Transform|MakeTransform (Math|Vector|MakeVector (Math|Conversions|ToFloat(Integer) (- (* _index_2 _tilesize) (Math|Float|Truncate (LocalVariables|GetWorldOffsetY)))) (Math|Conversions|ToFloat(Integer) (- (* _tilesize _index) (Math|Float|Truncate (LocalVariables|GetWorldOffsetX)))) 0.0) "0, 0, 0" "1,1,1") "AlwaysSpawn" 0 0))
      (Utilities|Array|Add _gridarray _returnvalue)
      (for (_array_element _array_index) _gridarray
        (Variables|/Game/Blueprints/Grid/BP_GridTile.BP_GridTile_C|SetTileNumber _array_element _array_index)))))

(fn CalculateWorldOffset
  (bind _tilesize (Variables|Grid|GetTileSize))
  (bind _tilesize_2 (Variables|Grid|GetTileSize))
  (return (- (* (* (Variables|Grid|GetGridX) _tilesize_2) 0.5) (* _tilesize_2 0.5)) (- (* (* (Variables|Grid|GetGridY) _tilesize) 0.5) (* _tilesize 0.5))))

(fn SetGridCellNeighbors
  (for (_array_element _array_index) (Variables|Grid|GetGridArray)
    (Utilities|GetNeighborWest _array_element _array_index
      (:then
        _)
      (:false
        _))
    (Utilities|GetNeighborEast _array_element _array_index
      (:then
        _)
      (:false
        _))
    (Utilities|GetNeighborSouth _array_element _array_index
      (:true
        _)
      (:then
        _))
    (Utilities|GetNeighborNorth _array_element _array_index)))

(fn SetTilesTypes
  (bind _gridarray (Variables|Grid|GetGridArray))
  (bind _returnvalue (Utilities|Array|Length _gridarray))
  (bind _returnvalue_2 (/ _returnvalue 2))
  (for _index (range 0 (- _returnvalue_2 1))
    (Default|SettoPlayerTile (Utilities|Array|Get(acopy) (Variables|Grid|GetGridArray) _index)))
  (for _index_2 (range _returnvalue_2 (- _returnvalue 1))
    (Default|SettoEnemyTile (Utilities|Array|Get(acopy) (Variables|Grid|GetGridArray) _index_2))))