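; A world camera actor that becomes player 0's view target on BeginPlay and offers camera shake functions for player and boss events.
; PlayerCameraShake and BossCameraShake both play BP_CameraShake as a world shake centred on the camera component, with different outer radii.
; BossCameraShake also plays an Earthquake sound at the world origin.
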(event EventBeginPlay
  (Game|Player|SetViewTargetwithBlend (Game|GetPlayerController 0) self 0.0 "VTBlend_Linear" 0.0 false))

(fn ConstructionScript)

(fn PlayerCameraShake
  (Camera|PlayWorldCameraShake "/Game/Blueprints/BP_CameraShake.BP_CameraShake_C" (Transformation|GetWorldLocation (Variables|Default|GetCamera)) 0.0 1e+03))

(fn BossCameraShake
  (Camera|PlayWorldCameraShake "/Game/Blueprints/BP_CameraShake.BP_CameraShake_C" (Transformation|GetWorldLocation (Variables|Default|GetCamera)) 0.0 1e+02)
  (Audio|PlaySoundatLocation "/Game/Audio/SoundEffects/Boss_Bulldozer/earthquake.earthquake" "0, 0, 0" "0, 0, 0" 1.0 1.0 0.0 0 0 0 0))