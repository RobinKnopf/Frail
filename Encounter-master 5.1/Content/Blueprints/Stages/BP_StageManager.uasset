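; BP_StageManager manages stage progression, loading each stage's row from the StagesData table by stage number.
; Ending a stage switches input mode and shows a rewards screen, or the victory screen once past stage six.
; NextStage advances the stage, restarts BP_EnemySpawner waves, resets the player, clears shockwave attacks and closes the rewards screen.
; RaiseDifficulty increments the health and damage multipliers.
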(event Custom|AddVictoryScreen
  ;[1 1 1] Adds the current stage victory screen.
  (Default|SetInputMode (Variables|References|GetControllerRef) true)
  (if (> (Variables|StageData|GetCurrentStage) 6)
    (bind _returnvalue (UserInterface|CreateWidget "/Game/UserInterface/WBP_Victory.WBP_Victory_C"))
    (UserInterface|Viewport|AddtoViewport _returnvalue 0)
    (else
      (bind _returnvalue_2 (UserInterface|CreateWidget "/Game/UserInterface/WBP_StageRewardsScreen.WBP_StageRewardsScreen_C"))
      (bind _output_get (Variables|References|SetStageRewardScreen _returnvalue_2))
      (UserInterface|Viewport|AddtoViewport _output_get 0))))

(event Custom|NextStage
  (bind _enemyspawner (Variables|References|GetEnemySpawner))
  ;[1 1 1] Moves to next stage & spawns the new wave.
  (Math|Integer|IncrementInt (Variables|StageData|GetCurrentStage)
    (:%20%20
      (CallFunction|SetStage)
      (Variables|/Game/Enemies/BP_EnemySpawner.BP_EnemySpawner_C|SetCurrentWave _enemyspawner 1)
      (bind _enemiesamount (Default|GetWaveEnemiesAmount _enemyspawner))
      (Default|SpawnEnemies _enemyspawner _enemiesamount)
      (Default|ResetCharacter (Variables|References|GetCharacterRef))
      (CallFunction|DestroyAllonMap)
      (Variables|StageData|SetWavesCompleted false)
      (Widget|RemovefromParent (Variables|References|GetStageRewardScreen))
      (Default|SetInputMode (Variables|References|GetControllerRef) false))))

(event EventBeginPlay
  (Utilities|CastReferences))

(fn ConstructionScript)

(fn SetStage
  (bind _outrownames (DataTable|GetDataTableRowNames (.datatable (Variables|StageData|GetStagesData))))
  (bind _structout (Utilities|Struct|SetmembersinDataTableRowHandle (Variables|StageData|GetStagesData) (Utilities|Array|Get(acopy) _outrownames (- (Variables|StageData|GetCurrentStage) 1))))
  (bind _returnvalue (Utilities|GetDataTableRow (.datatable _structout) (.rowname _structout))
    (:then
      (Variables|StageData|SetCurrentStageStruct _returnvalue))))

(fn DestroyAllonMap
  (bind _outactors (Actor|GetAllActorsOfClass "/Game/Enemies/EnemyAttacks/BP_EnemyAttack_Shockwave.BP_EnemyAttack_Shockwave_C"))
  (for _array_element _outactors
    (Actor|DestroyActor _array_element)))

(fn RaiseDifficulty
  (Variables|Default|SetHealthMultiplier (+ (Variables|Default|GetHealthMultiplier) (Variables|Default|GetAddMultiplier)))
  (Variables|Default|SetDamageMultiplier (+ (Variables|Default|GetDamageMultiplier) (Variables|Default|GetAddMultiplier))))