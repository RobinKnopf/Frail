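; Base enemy for grid-based combat that claims a spawner tile and scales its hit points by the stage's health multiplier.
; MoveToTile blinks it onto free tiles, updating occupancy, while helpers pick targets randomly or toward the player's row using tile-number modulo on three rows.
; Damage lowers HP and triggers death cleanup and dispatch; stun is a five-second flag.
; CreateHPBar's widget setup is disconnected, though damage still calls that widget.
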(event Custom|SetStunned
  (Variables|Default|SetStunned true)
  (Utilities|FlowControl|Delay 5.0)
  (Variables|Default|SetStunned false))

(event Custom|MoveToTile
  (params (GridTile :type BP%20Grid%20Tile%20Object%20Reference))
  ;[1 1 1] Move Enemy to the selected tile
  (Utilities|IsValid GridTile
    (:Is%20Valid
      (if (and (Utilities|Enum|NotEqual(Enum) (Variables|/Game/Blueprints/Grid/BP_GridTile.BP_GridTile_C|GetGridType GridTile) "NewEnumerator0") (not (Variables|/Game/Blueprints/Grid/BP_GridTile.BP_GridTile_C|GetIsOccupied GridTile)))
        (Rendering|SetVisibility (Variables|Default|GetSkeletalMesh) false false)
        (Transformation|SetWorldLocation (Variables|Default|GetDefaultSceneRoot) (Variables|/Game/Blueprints/Grid/BP_GridTile.BP_GridTile_C|GetGridWorldLocation GridTile) false false)
        (Default|EmptyTile (Variables|Grid|GetCurrentGridTile))
        (bind _output_get (Variables|Grid|SetCurrentGridTile GridTile))
        (Default|OccupyTile _output_get self)
        (Utilities|FlowControl|Delay 0.1)
        (Rendering|SetVisibility (Variables|Default|GetSkeletalMesh) true false)))))

(event EventBeginPlay
  ;[1 1 1] Event BeginPlay
  (Utilities|CastReferences)
  (CallFunction|SetStartingTile)
  (CallFunction|SetHP)
  (CallFunction|CreateHPBar))

(event Game|Damage|EventAnyDamage
  (params (Damage :type Float%20%28single-precision%29) (DamageType :type Damage%20Type%20Object%20Reference) (InstigatedBy :type Controller%20Object%20Reference) (DamageCauser :type Actor%20Object%20Reference))
  ;[1 1 1] Apply any Damage
  (Default|ShowDamageTaken (Variables|Health|GetHPBarWidget) Damage)
  (bind _output_get (Variables|Health|SetHitPoints (- (Variables|Health|GetHitPoints) Damage)))
  (if (<= _output_get 0.0)
    (CallFunction|KillMe)))

(fn ConstructionScript)

(fn SetStartingTile
  (bind _returnvalue (Actor|GetActorOfClass "/Game/Enemies/BP_EnemySpawner.BP_EnemySpawner_C"))
  (bind _output_get (Variables|References|SetEnemySpawner _returnvalue))
  (bind _spawntile (Default|SetEnemySpawnTile _output_get))
  (bind _output_get_2 (Variables|Grid|SetCurrentGridTile _spawntile))
  (Default|OccupyTile _output_get_2 self))

(fn GetRandomNeighborTile
  (switch int (Math|Random|RandomIntegerinRange 0 3)
    (:0
      (Variables|Grid|SetMovementTargetTile (Variables|/Game/Blueprints/Grid/BP_GridTile.BP_GridTile_C|GetNeighborEast (Variables|Grid|GetCurrentGridTile))))
    (:1
      (Variables|Grid|SetMovementTargetTile (Variables|/Game/Blueprints/Grid/BP_GridTile.BP_GridTile_C|GetNeighborNorth (Variables|Grid|GetCurrentGridTile))))
    (:2
      (Variables|Grid|SetMovementTargetTile (Variables|/Game/Blueprints/Grid/BP_GridTile.BP_GridTile_C|GetNeighborSouth (Variables|Grid|GetCurrentGridTile))))
    (:3
      (Variables|Grid|SetMovementTargetTile (Variables|/Game/Blueprints/Grid/BP_GridTile.BP_GridTile_C|GetNeighborWest (Variables|Grid|GetCurrentGridTile))))))

(fn IsBottomRow
  (params (GridTile :type BP%20Grid%20Tile%20Object%20Reference))
  (return (== (Math|Integer|%(Integer) (Variables|/Game/Blueprints/Grid/BP_GridTile.BP_GridTile_C|GetTileNumber GridTile) (Variables|/Game/Blueprints/Grid/BP_GridManager.BP_GridManager_C|GetGridY (Variables|Grid|GetGridManager))) 0)))

(fn IsTopRow
  (params (GridTile :type BP%20Grid%20Tile%20Object%20Reference))
  (return (== (Math|Integer|%(Integer) (+ (Variables|/Game/Blueprints/Grid/BP_GridTile.BP_GridTile_C|GetTileNumber GridTile) 1) (Variables|/Game/Blueprints/Grid/BP_GridManager.BP_GridManager_C|GetGridY (Variables|Grid|GetGridManager))) 0)))

(fn IsMiddleRow
  (params (GridTile :type BP%20Grid%20Tile%20Object%20Reference))
  (return (== (Math|Integer|%(Integer) (- (Variables|/Game/Blueprints/Grid/BP_GridTile.BP_GridTile_C|GetTileNumber GridTile) 1) (Variables|/Game/Blueprints/Grid/BP_GridManager.BP_GridManager_C|GetGridY (Variables|Grid|GetGridManager))) 0)))

(fn FindthePlayerRow
  (bind _playerreference (Variables|References|GetPlayerReference))
  (bind _playerreference_2 (Variables|References|GetPlayerReference))
  (bind _currenttile (Variables|/Game/Character/BP_PlayerCharacter.BP_PlayerCharacter_C|GetCurrentTile _playerreference))
  (bind _currenttile_2 (Variables|/Game/Character/BP_PlayerCharacter.BP_PlayerCharacter_C|GetCurrentTile _playerreference_2))
  (if (CallFunction|IsMiddleRow (Variables|Grid|GetCurrentGridTile))
    (if (CallFunction|IsBottomRow (Variables|/Game/Character/BP_PlayerCharacter.BP_PlayerCharacter_C|GetCurrentTile (Variables|References|GetPlayerReference)))
      (Variables|Grid|SetMovementTargetTile (Variables|/Game/Blueprints/Grid/BP_GridTile.BP_GridTile_C|GetNeighborSouth (Variables|Grid|GetCurrentGridTile)))
      (elif (CallFunction|IsTopRow (Variables|/Game/Character/BP_PlayerCharacter.BP_PlayerCharacter_C|GetCurrentTile (Variables|References|GetPlayerReference)))
        (Variables|Grid|SetMovementTargetTile (Variables|/Game/Blueprints/Grid/BP_GridTile.BP_GridTile_C|GetNeighborNorth (Variables|Grid|GetCurrentGridTile)))))
    (elif (CallFunction|IsBottomRow (Variables|Grid|GetCurrentGridTile))
      (if (or (CallFunction|IsMiddleRow _currenttile_2) (CallFunction|IsTopRow _currenttile_2))
        (Variables|Grid|SetMovementTargetTile (Variables|/Game/Blueprints/Grid/BP_GridTile.BP_GridTile_C|GetNeighborNorth (Variables|Grid|GetCurrentGridTile))))
      (elif (CallFunction|IsTopRow (Variables|Grid|GetCurrentGridTile))
        (if (or (CallFunction|IsMiddleRow _currenttile) (CallFunction|IsBottomRow _currenttile))
          (Variables|Grid|SetMovementTargetTile (Variables|/Game/Blueprints/Grid/BP_GridTile.BP_GridTile_C|GetNeighborSouth (Variables|Grid|GetCurrentGridTile))))))))

(fn CreateHPBar)

(fn RandomizeMovement
  (switch int (Math|Random|RandomIntegerinRange 0 1)
    (:0
      (CallFunction|FindthePlayerRow))
    (:1
      (CallFunction|GetRandomNeighborTile)))
  (return))

(fn KillMe
  (Utilities|Array|RemoveItem (Variables|/Game/Enemies/BP_EnemySpawner.BP_EnemySpawner_C|GetEnemies (Variables|References|GetEnemySpawner)) self)
  (Default|EmptyTile (Variables|Grid|GetCurrentGridTile))
  (Variables|Health|SetImDead true)
  (Default|CallDeathDispatcher)
  (Actor|DestroyActor))

(fn SetHP
  (bind _returnvalue (Actor|GetActorOfClass "/Game/Blueprints/Stages/BP_StageManager.BP_StageManager_C"))
  (Variables|Health|SetHitPoints (* (Variables|/Game/Blueprints/Stages/BP_StageManager.BP_StageManager_C|GetHealthMultiplier _returnvalue) (Variables|Health|GetHitPoints))))

(fn SetEnemySpawnTile
  (return 0))