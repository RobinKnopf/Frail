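; Grid-based laser turret enemy that periodically fires a laser attack from its current tile.
; Tick runs through a five-second Delay, then, unless stunned, spawns a laser attack actor at that tile with itself as owner and resets the cooldown.
; LaserCountdown decrements the timer to restore LaserReady, but the firing path never checks that flag and nothing here calls the function.
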(event EventBeginPlay
  (|CallParentFunction))

(event EventTick
  (params (DeltaSeconds :type Float%20%28single-precision%29))
  (bind _self self)
  (bind _currentgridtile (Variables|Default|GetCurrentGridTile))
  (Utilities|FlowControl|Delay 5.0)
  (if (not (Variables|Default|GetStunned))
    (bind _returnvalue (Game|SpawnActorfromClass "/Game/Enemies/EnemyAttacks/BP_EnemyAttack_Laser.BP_EnemyAttack_Laser_C" (Transformation|GetActorTransform _currentgridtile) "Undefined" 0 _currentgridtile _self _self))
    (Variables|Default|SetLaser _returnvalue)
    (Variables|Default|SetLaserReady false)
    (Variables|Default|SetLaserTimer (Variables|Default|GetLaserCooldown))))

(fn ConstructionScript
  (|CallParentFunction))

(fn LaserCountdown
  (if (not (Variables|Default|GetLaserReady))
    (bind _result (Math|Integer|DecrementInt (Variables|Default|GetLaserTimer))
      (:%20%20
        (if (== _result 0)
          (Variables|Default|SetLaserReady true))))))