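; Enemy bomb attack on the tile grid that hits the tile a set range west of its starting tile, plus that tile's valid neighbours.
; On BeginPlay it scales damage by the stage manager's multiplier and spawns telegraphs over the area.
; A one-second timer then clears the telegraphs, destroys the actor and plays explosions on each tile, damaging the player if standing there.
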(event Custom|PassTurn
  (Utilities|FlowControl|Sequence
    (:then_0
      (Utilities|FlowControl|DoOnce false
        (:Completed
          (for _array_element (Variables|Default|GetAbilityTelegraph)
            (Actor|DestroyActor _array_element)
            (Actor|DestroyActor)))))
    (:then_1
      (for _array_element_2 (Variables|Default|GetAbilityAOE)
        (CallFunction|DamagePlayer&Particle _array_element_2)
        (Audio|PlaySound2D "/Game/Audio/SoundEffects/Sci_Fi_Grenade_2.Sci_Fi_Grenade_2" 1.0 1.0 0.0 0 0)))))

(event EventBeginPlay
  (CallFunction|SetSpawnLocation)
  (CallFunction|SetDamage)
  (CallFunction|GetTargetTile)
  (CallFunction|SpawnTelegraph)
  (Utilities|Time|SetTimerbyEvent (delegate Custom|PassTurn) 1.0))

(fn ConstructionScript)

(fn GetTargetTile
  (LocalVariables|SetCurrentTile (Variables|Default|GetStartingTile))
  (for _index (range 0 (- (Variables|Default|GetAbilityRange) 1))
    (LocalVariables|SetCurrentTile (Variables|/Game/Blueprints/Grid/BP_GridTile.BP_GridTile_C|GetNeighborWest (LocalVariables|GetCurrentTile))))
  (Variables|Default|SetTargetTile (LocalVariables|GetCurrentTile))
  (return))

(fn SpawnTelegraph
  (CallFunction|SetAbilityAOE)
  (for _array_element (Variables|Default|GetAbilityAOE)
    (bind _returnvalue (Game|SpawnActorfromClass "/Game/Enemies/EnemyAttacks/BP_Telegraph.BP_Telegraph_C" (Math|Transform|MakeTransform (Variables|/Game/Blueprints/Grid/BP_GridTile.BP_GridTile_C|GetGridWorldLocation _array_element) "0, 0, 0" "1.000000,1.000000,1.000000") "Undefined" 0 0))
    (Utilities|Array|Add (Variables|Default|GetAbilityTelegraph) _returnvalue)))

(fn SetAbilityAOE
  (bind _targettile (Variables|Default|GetTargetTile))
  (bind _output_get (Variables|Default|SetAbilityAOE (Variables|/Game/Blueprints/Grid/BP_GridTile.BP_GridTile_C|GetValidNeighbors _targettile)))
  (Utilities|Array|Add _output_get _targettile))

(fn DamagePlayer&Particle
  (params (GridTile :type BP%20Grid%20Tile%20Object%20Reference))
  (bind _occupyingactor (Variables|/Game/Blueprints/Grid/BP_GridTile.BP_GridTile_C|GetOccupyingActor GridTile))
  (Niagara|SpawnSystematLocation "/Game/Sci-Fi_Starter_VFX_Pack_Niagara/Niagara/Explosion/NS_Explosion_C4_2.NS_Explosion_C4_2" (Variables|/Game/Blueprints/Grid/BP_GridTile.BP_GridTile_C|GetGridWorldLocation GridTile) "0, 0, 0" "0.200000,0.200000,0.200000")
  (if (== _occupyingactor (Game|GetPlayerCharacter 0))
    (Game|Damage|ApplyDamage _occupyingactor (Variables|Default|GetDamage) 0 (Variables|Actor|GetInstigator))))

(fn SetSpawnLocation
  (bind _collisioncomponent (Variables|Default|GetCollisionComponent))
  (Transformation|SetWorldLocation _collisioncomponent (+ (Transformation|GetWorldLocation _collisioncomponent) "0, 0,150.000000") false false))

(fn SetDamage
  (bind _returnvalue (Actor|GetActorOfClass "/Game/Blueprints/Stages/BP_StageManager.BP_StageManager_C"))
  (Variables|Default|SetDamage (* (Variables|/Game/Blueprints/Stages/BP_StageManager.BP_StageManager_C|GetDamageMultiplier _returnvalue) (Variables|Default|GetDamage))))