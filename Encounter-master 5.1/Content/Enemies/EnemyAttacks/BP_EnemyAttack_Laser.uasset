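; Enemy laser attack actor that hits the player along a straight row of grid tiles west of its starting tile.
; On spawn it scales damage by the stage manager's multiplier, collects neighbouring tiles up to a cap, places telegraphs and briefly plays then pauses the laser particle.
; A timer then damages the player if standing on those tiles, skipped if the enemy owner is invalid, and cleans up telegraphs, particle and itself.
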(event Custom|PassTurn
  (Utilities|IsValid (Variables|Default|GetEnemyOwner)
    (:Is%20Valid
      (Utilities|FlowControl|Sequence
        (:then_0
          (for _array_element (Variables|Default|GetAbilityAOE)
            (CallFunction|DamagePlayer _array_element)))
        (:then_1
          (Utilities|FlowControl|DoOnce false :!label _label
            (:Completed
              (for _array_element_2 (Variables|Default|GetAbilityTelegraph)
                (Actor|DestroyActor _array_element_2)
                (Default|Unpause&Kill (Variables|Default|GetLaserParticle))
                (Actor|DestroyActor)))))))
    (:Is%20Not%20Valid
      (goto _label))))

(event EventBeginPlay
  (CallFunction|SetSpawnLocation)
  (CallFunction|SetDamage)
  (CallFunction|GetTargetTiles)
  (CallFunction|SpawnTelegraph)
  (Utilities|Time|SetTimerbyEvent (delegate Custom|PassTurn) 1.0)
  (Utilities|FlowControl|Delay 0.125)
  (Default|Pause (Variables|Default|GetLaserParticle)))

(fn ConstructionScript)

(fn SetSpawnLocation
  (bind _returnvalue (Game|SpawnActorfromClass "/Game/Enemies/EnemyAttacks/Particles/P_EnemyLaser.P_EnemyLaser_C" (Math|Transform|MakeTransform (+ (Transformation|GetWorldLocation (Variables|Default|GetDefaultSceneRoot)) "0,-50.000000,75.000000") "0, 0, 0" "1.000000,1.000000,1.000000") "Undefined" 0 0))
  (Variables|Default|SetLaserParticle _returnvalue))

(fn GetTargetTiles
  (Variables|Default|SetCurrentTile (Variables|Default|GetStartingTile))
  (Utilities|FlowControl|ForLoopwithBreak 0 10 :!label _label
    (:LoopBody
      (Utilities|IsValid (Variables|/Game/Blueprints/Grid/BP_GridTile.BP_GridTile_C|GetNeighborWest (Variables|Default|GetCurrentTile))
        (:Is%20Valid
          (bind _output_get (Variables|Default|SetCurrentTile (Variables|/Game/Blueprints/Grid/BP_GridTile.BP_GridTile_C|GetNeighborWest (Variables|Default|GetCurrentTile))))
          (Utilities|Array|Add (Variables|Default|GetAbilityAOE) _output_get))
        (:Is%20Not%20Valid
          (goto _label Break))))
    (:Completed
      (return))))

(fn SpawnTelegraph
  (for _array_element (Variables|Default|GetAbilityAOE)
    (bind _returnvalue (Game|SpawnActorfromClass "/Game/Enemies/EnemyAttacks/BP_Telegraph.BP_Telegraph_C" (Math|Transform|MakeTransform (Variables|/Game/Blueprints/Grid/BP_GridTile.BP_GridTile_C|GetGridWorldLocation _array_element) "0, 0, 0" "1.000000,1.000000,1.000000") "Undefined" 0 0))
    (Utilities|Array|Add (Variables|Default|GetAbilityTelegraph) _returnvalue)))

(fn DamagePlayer
  (params (GridTile :type BP%20Grid%20Tile%20Object%20Reference))
  (bind _occupyingactor (Variables|/Game/Blueprints/Grid/BP_GridTile.BP_GridTile_C|GetOccupyingActor GridTile))
  (if (== _occupyingactor (Game|GetPlayerCharacter 0))
    (Game|Damage|ApplyDamage _occupyingactor (Variables|Default|GetDamage) 0 (Variables|Actor|GetInstigator))))

(fn SetDamage
  (bind _returnvalue (Actor|GetActorOfClass "/Game/Blueprints/Stages/BP_StageManager.BP_StageManager_C"))
  (Variables|Default|SetDamage (* (Variables|/Game/Blueprints/Stages/BP_StageManager.BP_StageManager_C|GetDamageMultiplier _returnvalue) (Variables|Default|GetDamage))))