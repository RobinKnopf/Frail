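; Landslide boss attack actor that drops a few falling rocks onto random grid tiles, then destroys itself.
; On BeginPlay it finds BP_GridManager and builds a shuffled list of indices covering the first half of its GridArray.
; A short randomized loop spawns BP_FallingRock at the picked tiles, passing each as CurrentTile and removing entries from the list so tiles do not repeat.
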(event EventBeginPlay
  (bind _returnvalue (Actor|GetActorOfClass "/Game/Blueprints/Grid/BP_GridManager.BP_GridManager_C"))
  (Variables|Default|SetGridManager _returnvalue)
  (CallFunction|MakeRandomIntArray)
  (for _index (range 0 (Math|Random|RandomIntegerinRange 1 2))
    (Game|SpawnActorfromClass "/Game/Enemies/EnemyAttacks/BossAttacks/BP_FallingRock.BP_FallingRock_C" (Transformation|GetActorTransform (Utilities|Array|Get(acopy) (Variables|/Game/Blueprints/Grid/BP_GridManager.BP_GridManager_C|GetGridArray (Variables|Default|GetGridManager)) (Utilities|Array|Get(acopy) (Variables|Default|GetRandomIntArray) _index))) "Undefined" 0 (Utilities|Array|Get(acopy) (Variables|/Game/Blueprints/Grid/BP_GridManager.BP_GridManager_C|GetGridArray (Variables|Default|GetGridManager)) (Utilities|Array|Get(acopy) (Variables|Default|GetRandomIntArray) _index)) 0)
    (Utilities|Array|RemoveIndex (Variables|Default|GetRandomIntArray) _index))
  (Actor|DestroyActor))

(fn ConstructionScript)

(fn MakeRandomIntArray
  (bind _randomintarray (Variables|Default|GetRandomIntArray))
  (for _index (range 0 (- (/ (Utilities|Array|Length (Variables|/Game/Blueprints/Grid/BP_GridManager.BP_GridManager_C|GetGridArray (Variables|Default|GetGridManager))) 2) 1))
    (Utilities|Array|Add _randomintarray _index))
  (Utilities|Array|Shuffle _randomintarray))