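; Boss shockwave attack that travels west across the tile grid from a starting tile, damaging the player in its path.
; A looping one-second timer moves the collision component along west-neighbor links, raising and lowering the Arrow with a rock-smash sound.
; Hits are detected by comparing each tile's occupying actor to the player character rather than by overlap.
; The actor destroys itself when no west tile remains.
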(event Custom|PassTurn
  (CallFunction|MovetoNextTile)
  (Components|MoveComponentTo (Variables|Default|GetArrow) "0, 0,-60.000000" "90.000000, 0, 0" false false 0.3 false)
  (Audio|PlaySoundatLocation "/Game/Audio/SoundEffects/Boss_Bulldozer/NiceRockSmash.NiceRockSmash" "0, 0, 0" "0, 0, 0" 1.0 1.0 0.0 0 0 0 0)
  (Utilities|FlowControl|Delay 0.3)
  (Components|MoveComponentTo (Variables|Default|GetArrow) "0,0.000000,-150.000000" "90.000000, 0, 0" false false 0.5 false))

(event EventBeginPlay
  (Variables|Default|SetCurrentTile (Variables|Default|GetStartingTile))
  (Transformation|SetWorldLocation (Variables|Default|GetQuake) (Variables|/Game/Blueprints/Grid/BP_GridTile.BP_GridTile_C|GetGridWorldLocation (Variables|/Game/Blueprints/Grid/BP_GridTile.BP_GridTile_C|GetNeighborWest (Variables|Default|GetCurrentTile))) false false)
  (Utilities|Time|SetTimerbyEvent (delegate Custom|PassTurn) 1.0 true))

(fn ConstructionScript)

(fn MovetoNextTile
  (Utilities|IsValid (Variables|/Game/Blueprints/Grid/BP_GridTile.BP_GridTile_C|GetNeighborWest (Variables|Default|GetCurrentTile))
    (:Is%20Valid
      (Transformation|SetWorldLocation (Variables|Default|GetCollisionComponent) (Variables|/Game/Blueprints/Grid/BP_GridTile.BP_GridTile_C|GetGridWorldLocation (Variables|/Game/Blueprints/Grid/BP_GridTile.BP_GridTile_C|GetNeighborWest (Variables|Default|GetCurrentTile))) false false)
      (Variables|Default|SetCurrentTile (Variables|/Game/Blueprints/Grid/BP_GridTile.BP_GridTile_C|GetNeighborWest (Variables|Default|GetCurrentTile)))
      (CallFunction|CheckTargetHit))
    (:Is%20Not%20Valid
      (Actor|DestroyActor))))

(fn CheckTargetHit
  (bind _currenttile (Variables|Default|GetCurrentTile))
  (bind _occupyingactor (Variables|/Game/Blueprints/Grid/BP_GridTile.BP_GridTile_C|GetOccupyingActor _currenttile))
  (if (== _occupyingactor (Game|GetPlayerCharacter 0))
    (Game|Damage|ApplyDamage _occupyingactor 1e+01 0 0)))