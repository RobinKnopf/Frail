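; Drill stab attack for the Bulldozer boss that hits a straight line of grid tiles west of its starting tile.
; On BeginPlay it gathers tiles through west-neighbor links, spawns a telegraph on each and starts a delay timer.
; PassTurn damages the player on those tiles, triggers the drill animation and sound, and removes telegraphs.
; A second timer then clears the boss's occupied flag and destroys the attack actor.
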(event Custom|PassTurn
  (Utilities|FlowControl|Sequence
    (:then_0
      (Utilities|FlowControl|DoOnce false
        (:Completed
          (for _array_element (Variables|Default|GetAbilityAOE)
            (CallFunction|DamagePlayer _array_element)
            (Components|Animation|PlayAnimation (Variables|/Game/Enemies/BP_Enemy_Master.BP_Enemy_Master_C|GetSkeletalMesh (.AsBP%20Boss%20Bulldozer (Utilities|Casting|CastToBP_Boss_Bulldozer (Variables|Default|GetBossActor)))) "/Game/MiningMech/Animations/ANIM_MiningMech_DirectDrillAttackForward_RM_Montage.ANIM_MiningMech_DirectDrillAttackForward_RM_Montage" false)
            (Audio|PlaySoundatLocation "/Game/Audio/SoundEffects/Boss_Bulldozer/DrillTelegraph.DrillTelegraph" "0, 0, 0" "0, 0, 0" 1.0 1.0 0.0 0 0 0 0)))))
    (:then_1
      (Utilities|FlowControl|DoOnce false
        (:Completed
          (for _array_element_2 (Variables|Default|GetAbilityTelegraph)
            (Actor|DestroyActor _array_element_2)
            (Utilities|Time|SetTimerbyEvent (delegate Custom|FinishAttack) 2.0)))))))

(event Custom|FinishAttack
  (Variables|/Game/Enemies/BP_Boss_Bulldozer.BP_Boss_Bulldozer_C|SetOcuppied (.AsBP%20Boss%20Bulldozer (Utilities|Casting|CastToBP_Boss_Bulldozer (Variables|Default|GetBossActor))) false)
  (Actor|DestroyActor))

(event EventBeginPlay
  (CallFunction|GetTargetTiles)
  (CallFunction|SpawnTelegraph)
  (Utilities|Time|SetTimerbyEvent (delegate Custom|PassTurn) 2.0))

(fn ConstructionScript)

(fn SetSpawnLocation
  (Game|SpawnActorfromClass "/Game/Enemies/EnemyAttacks/Particles/P_EnemyLaser.P_EnemyLaser_C" (Math|Transform|MakeTransform (+ (Transformation|GetWorldLocation (Variables|Default|GetDefaultSceneRoot)) "0,-50.000000,75.000000") "0, 0, 0" "1.000000,1.000000,1.000000") "Undefined" 0 0))

(fn GetTargetTiles
  (Variables|Default|SetCurrentTile (Variables|Default|GetStartingTile))
  (Utilities|FlowControl|ForLoopwithBreak 0 10 :!label _label
    (:LoopBody
      (Utilities|IsValid (Variables|/Game/Blueprints/Grid/BP_GridTile.BP_GridTile_C|GetNeighborWest (Variables|Default|GetCurrentTile))
        (:Is%20Valid
          (bind _output_get (Variables|Default|SetCurrentTile (Variables|/Game/Blueprints/Grid/BP_GridTile.BP_GridTile_C|GetNeighborWest (Variables|Default|GetCurrentTile))))
          (Utilities|Array|Add (Variables|Default|GetAbilityAOE) _output_get))
        (:Is%20Not%20Valid
          (goto _label Break))))
    (:Completed
      (return))))

(fn SpawnTelegraph
  (for _array_element (Variables|Default|GetAbilityAOE)
    (bind _returnvalue (Game|SpawnActorfromClass "/Game/Enemies/EnemyAttacks/BP_Telegraph.BP_Telegraph_C" (Math|Transform|MakeTransform (Variables|/Game/Blueprints/Grid/BP_GridTile.BP_GridTile_C|GetGridWorldLocation _array_element) "0, 0, 0" "1.000000,1.000000,1.000000") "Undefined" 0 0))
    (Utilities|Array|Add (Variables|Default|GetAbilityTelegraph) _returnvalue)))

(fn DamagePlayer
  (params (GridTile :type BP%20Grid%20Tile%20Object%20Reference))
  (bind _occupyingactor (Variables|/Game/Blueprints/Grid/BP_GridTile.BP_GridTile_C|GetOccupyingActor GridTile))
  (if (== _occupyingactor (Game|GetPlayerCharacter 0))
    (Game|Damage|ApplyDamage _occupyingactor 25.0 0 0)))