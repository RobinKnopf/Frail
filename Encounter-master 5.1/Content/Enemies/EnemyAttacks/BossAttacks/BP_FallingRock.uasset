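; Boss-attack falling rock that telegraphs its target grid tile, then drops and damages the player if they stand on it.
; On BeginPlay it plays a warning sound, spawns a BP_Telegraph on CurrentTile and starts a one-second timer calling PassTurn.
; PassTurn activates projectile movement, immediately checks the tile occupant for damage and plays an impact sound.
; The rock and telegraph are destroyed after a short delay.
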(event Custom|PassTurn
  (Utilities|FlowControl|Sequence
    (:then_0
      (Utilities|FlowControl|Delay 0.3)
      (Actor|DestroyActor (Variables|Default|GetTelegraph))
      (Actor|DestroyActor))
    (:then_1
      (Components|Activation|Activate (Variables|Default|GetProjectileMovement) false)
      (CallFunction|CheckDamage)
      (Audio|PlaySoundatLocation "/Game/Audio/SoundEffects/Boss_Bulldozer/rockhittingstuff.rockhittingstuff" "0, 0, 0" "0, 0, 0" 1.0 1.0 0.0 0 0 0 0))))

(event EventBeginPlay
  (Audio|PlaySoundatLocation "/Game/Audio/SoundEffects/Boss_Bulldozer/Rockfalltelegraph.Rockfalltelegraph" "0, 0, 0" "0, 0, 0" 1.0 1.0 0.0 0 0 0 0)
  (CallFunction|SpawnTelegraph)
  (Utilities|Time|SetTimerbyEvent (delegate Custom|PassTurn) 1.0 true))

(fn ConstructionScript)

(fn SpawnTelegraph
  (bind _returnvalue (Game|SpawnActorfromClass "/Game/Enemies/EnemyAttacks/BP_Telegraph.BP_Telegraph_C" (Math|Transform|MakeTransform (Variables|/Game/Blueprints/Grid/BP_GridTile.BP_GridTile_C|GetGridWorldLocation (Variables|Default|GetCurrentTile)) "0, 0, 0" "1.000000,1.000000,1.000000") "Undefined" 0 0))
  (Variables|Default|SetTelegraph _returnvalue))

(fn CheckDamage
  (bind _currenttile (Variables|Default|GetCurrentTile))
  (bind _occupyingactor (Variables|/Game/Blueprints/Grid/BP_GridTile.BP_GridTile_C|GetOccupyingActor _currenttile))
  (if (== _occupyingactor (Game|GetPlayerCharacter 0))
    (Game|Damage|ApplyDamage _occupyingactor 25.0 0 0)))