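; Boss attack actor that spawns pairs of BP_BossAttack_Shockwave actors on grid tiles, starting with a north pair on BeginPlay.
; Each pair covers the starting tile plus its north or south neighbor.
; A looping one-second turn timer uses AttackCounter parity to fire every other turn, with a FlipFlop alternating south and north.
; The actor destroys itself once the counter reaches its limit.
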(event Custom|PassTurn
  (if (< (Variables|Default|GetAttackCounter) 11)
    (if (!= (Math|Integer|%(Integer) (Variables|Default|GetAttackCounter) 2) 0)
      (Utilities|FlowControl|FlipFlop
        (:A
          (CallFunction|SouthShockwave))
        (:B
          (CallFunction|NorthShockwave)))
      (else
        (Math|Integer|IncrementInt (Variables|Default|GetAttackCounter))))
    (else
      (Actor|DestroyActor))))

(event EventBeginPlay
  (Variables|Default|SetCurrentTile (Variables|Default|GetStartingTile))
  (Utilities|Time|SetTimerbyEvent (delegate Custom|PassTurn) 1.0 true)
  (CallFunction|NorthShockwave))

(fn ConstructionScript)

(fn NorthShockwave
  (bind _currenttile (Variables|Default|GetCurrentTile))
  (bind _neighbornorth (Variables|/Game/Blueprints/Grid/BP_GridTile.BP_GridTile_C|GetNeighborNorth _currenttile))
  (Utilities|FlowControl|Sequence
    (:then_0
      (Game|SpawnActorfromClass "/Game/Enemies/EnemyAttacks/BossAttacks/BP_BossAttack_Shockwave.BP_BossAttack_Shockwave_C" (Transformation|GetActorTransform _currenttile) "Undefined" 0 _currenttile 0))
    (:then_1
      (Game|SpawnActorfromClass "/Game/Enemies/EnemyAttacks/BossAttacks/BP_BossAttack_Shockwave.BP_BossAttack_Shockwave_C" (Transformation|GetActorTransform _neighbornorth) "Undefined" 0 _neighbornorth 0)
      (Math|Integer|IncrementInt (Variables|Default|GetAttackCounter)))))

(fn SouthShockwave
  (bind _currenttile (Variables|Default|GetCurrentTile))
  (bind _neighborsouth (Variables|/Game/Blueprints/Grid/BP_GridTile.BP_GridTile_C|GetNeighborSouth _currenttile))
  (Utilities|FlowControl|Sequence
    (:then_0
      (Game|SpawnActorfromClass "/Game/Enemies/EnemyAttacks/BossAttacks/BP_BossAttack_Shockwave.BP_BossAttack_Shockwave_C" (Transformation|GetActorTransform _currenttile) "Undefined" 0 _currenttile 0))
    (:then_1
      (Game|SpawnActorfromClass "/Game/Enemies/EnemyAttacks/BossAttacks/BP_BossAttack_Shockwave.BP_BossAttack_Shockwave_C" (Transformation|GetActorTransform _neighborsouth) "Undefined" 0 _neighborsouth 0)
      (Math|Integer|IncrementInt (Variables|Default|GetAttackCounter)))))