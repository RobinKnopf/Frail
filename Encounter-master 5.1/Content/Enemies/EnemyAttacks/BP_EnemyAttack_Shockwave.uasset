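; BP_EnemyAttack_Shockwave is an enemy attack that travels west across the tile grid, hurting the player.
; On BeginPlay it scales damage by the stage manager's multiplier and starts a looping one-second timer from its starting tile.
; Each tick of that timer moves the collision component one tile, damages the player if occupying it, then retriggers the explosion effect.
; It destroys itself when no west neighbor remains.
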(event Custom|PassTurn
  (CallFunction|MovetoNextTile)
  (Utilities|FlowControl|Delay 0.1)
  (Components|Activation|Activate (Variables|Default|GetExplosion) true))

(event EventBeginPlay
  (CallFunction|SetDamage)
  (Variables|Default|SetCurrentTile (Variables|Default|GetStartingTile))
  (Utilities|Time|SetTimerbyEvent (delegate Custom|PassTurn) 1.0 true)
  (Components|Activation|Activate (Variables|Default|GetExplosion) false))

(fn ConstructionScript)

(fn MovetoNextTile
  (Utilities|IsValid (Variables|/Game/Blueprints/Grid/BP_GridTile.BP_GridTile_C|GetNeighborWest (Variables|Default|GetCurrentTile))
    (:Is%20Valid
      (Transformation|SetWorldLocation (Variables|Default|GetCollisionComponent) (Variables|/Game/Blueprints/Grid/BP_GridTile.BP_GridTile_C|GetGridWorldLocation (Variables|/Game/Blueprints/Grid/BP_GridTile.BP_GridTile_C|GetNeighborWest (Variables|Default|GetCurrentTile))) false false)
      (Variables|Default|SetCurrentTile (Variables|/Game/Blueprints/Grid/BP_GridTile.BP_GridTile_C|GetNeighborWest (Variables|Default|GetCurrentTile)))
      (CallFunction|CheckTargetHit))
    (:Is%20Not%20Valid
      (Actor|DestroyActor))))

(fn CheckTargetHit
  (bind _currenttile (Variables|Default|GetCurrentTile))
  (bind _occupyingactor (Variables|/Game/Blueprints/Grid/BP_GridTile.BP_GridTile_C|GetOccupyingActor _currenttile))
  (if (== _occupyingactor (Game|GetPlayerCharacter 0))
    (Game|Damage|ApplyDamage _occupyingactor (Variables|Default|GetDamage) 0 (Variables|Actor|GetInstigator))))

(fn SetDamage
  (bind _returnvalue (Actor|GetActorOfClass "/Game/Blueprints/Stages/BP_StageManager.BP_StageManager_C"))
  (Variables|Default|SetDamage (* (Variables|/Game/Blueprints/Stages/BP_StageManager.BP_StageManager_C|GetDamageMultiplier _returnvalue) (Variables|Default|GetDamage))))