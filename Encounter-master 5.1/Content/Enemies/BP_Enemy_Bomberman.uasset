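; Grid-based bomber enemy that wanders between tiles and drops bombs on the tile it occupies.
; A Delay on Tick paces its decisions: while not stunned, it advances the bomb cooldown, then randomly picks between moving, attempting a bomb attack or idling.
; The attack only spawns a bomb when ready, then restarts the cooldown, which counts decision steps rather than seconds.
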(event Custom|Attack:Bomb
  (bind _currentgridtile (Variables|Default|GetCurrentGridTile))
  ;[1 1 1] Bomb Attack
  (if (Variables|Bomb|GetBombReady)
    (Game|SpawnActorfromClass "/Game/Enemies/EnemyAttacks/BP_EnemyAttack_Bomb.BP_EnemyAttack_Bomb_C" (Transformation|GetActorTransform _currentgridtile) "Undefined" 0 _currentgridtile self)
    (Variables|Bomb|SetBombReady false)
    (Variables|Bomb|SetBombTimer (Variables|Bomb|GetBombCooldown))))

(event EventBeginPlay
  (|CallParentFunction))

(event EventTick
  (params (DeltaSeconds :type Float%20%28single-precision%29))
  ;[1 1 1] Enemy Actions
  (Utilities|FlowControl|Delay 0.3)
  (if (not (Variables|Default|GetStunned))
    (Utilities|FlowControl|Sequence
      (:then_0
        (CallFunction|BombCountdown))
      (:then_1
        (switch int (Math|Random|RandomIntegerinRange 0 2)
          (:0
            (CallFunction|RandomizeMovement)
            (CallFunction|MovetoTile (Variables|Default|GetMovementTargetTile)))
          (:1
            (CallFunction|Attack:Bomb)))))))

(fn ConstructionScript
  (|CallParentFunction))

(fn BombCountdown
  (if (not (Variables|Bomb|GetBombReady))
    (bind _result (Math|Integer|DecrementInt (Variables|Bomb|GetBombTimer))
      (:%20%20
        (if (== _result 0)
          (Variables|Bomb|SetBombReady true))))))