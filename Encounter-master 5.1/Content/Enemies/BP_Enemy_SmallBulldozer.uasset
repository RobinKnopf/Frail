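; Small bulldozer enemy that roams a tile grid and fires shockwave attacks.
; A 0.3-second Delay on Tick paces its decisions: unless stunned, it advances the cooldown, then randomly moves to a random tile, attempts a shockwave or idles.
; When ready, the shockwave spawns on the west neighbor of its current tile and restarts a cooldown counted in decision steps rather than seconds.
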(event Custom|Attack1:Shockwave
  (bind _currentgridtile (Variables|Default|GetCurrentGridTile))
  (bind _neighborwest (Variables|/Game/Blueprints/Grid/BP_GridTile.BP_GridTile_C|GetNeighborWest _currentgridtile))
  (if (Variables|Shockwave|GetShockwaveReady)
    (Game|SpawnActorfromClass "/Game/Enemies/EnemyAttacks/BP_EnemyAttack_Shockwave.BP_EnemyAttack_Shockwave_C" (Transformation|GetActorTransform _neighborwest) "Undefined" 0 _neighborwest self)
    (Variables|Shockwave|SetShockwaveReady false)
    (Variables|Shockwave|SetShockwaveTimer (Variables|Shockwave|GetShockwaveCooldown))))

(event EventBeginPlay
  (|CallParentFunction))

(event EventTick
  (params (DeltaSeconds :type Float%20%28single-precision%29))
  (Utilities|FlowControl|Delay 0.3)
  (if (not (Variables|Default|GetStunned))
    (Utilities|FlowControl|Sequence
      (:then_0
        (CallFunction|ShockwaveCountdown))
      (:then_1
        (switch int (Math|Random|RandomIntegerinRange 0 2)
          (:0
            (CallFunction|RandomizeMovement)
            (CallFunction|MovetoTile (Variables|Default|GetMovementTargetTile)))
          (:1
            (CallFunction|Attack1:Shockwave)))))))

(fn ConstructionScript
  (|CallParentFunction))

(fn ShockwaveCountdown
  (if (not (Variables|Shockwave|GetShockwaveReady))
    (bind _result (Math|Integer|DecrementInt (Variables|Shockwave|GetShockwaveTimer))
      (:%20%20
        (if (== _result 0)
          (Variables|Shockwave|SetShockwaveReady true))))))