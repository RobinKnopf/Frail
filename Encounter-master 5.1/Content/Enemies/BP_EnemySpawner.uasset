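; Wave spawner that populates the grid with enemies and drives a stage's wave progression.
; Wave sizes come from the StageManager's stage struct; enemies are picked randomly from a pool, except a Bulldozer boss on stage 7, wave 3.
; Spawning rerolls occupied tiles within a fixed index range of the GridManager's array.
; Death dispatchers trigger the next wave once the enemy list empties, or the victory screen after the last.
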(event Custom|SpawnEnemies
  (params (#%20of%20Enemies :type Integer))
  ;[1 1 1] Spawn a given amount of enemies, avoids to spawn them on the same grid tile
  (for _index (range 1 #%20of%20Enemies)
    (bind _output_get (Variables|Default|SetSpawnTile (Utilities|Array|Get(acopy) (Variables|/Game/Blueprints/Grid/BP_GridManager.BP_GridManager_C|GetGridArray (Variables|Default|GetGridManager)) (Math|Random|RandomIntegerinRange 12 23)) :!label _label))
    (if (Variables|/Game/Blueprints/Grid/BP_GridTile.BP_GridTile_C|GetIsOccupied _output_get)
      (goto _label)
      (else
        (bind _enemy (CallFunction|GetRandomEnemy))
        (bind _returnvalue (Game|SpawnActorfromClass _enemy (Math|Transform|MakeTransform (Variables|/Game/Blueprints/Grid/BP_GridTile.BP_GridTile_C|GetGridWorldLocation (Variables|Default|GetSpawnTile)) "0, 0, 0" "1.000000,1.000000,1.000000") "AlwaysSpawn" 0 0))
        (Utilities|Array|Add (Variables|Default|GetEnemies) _returnvalue)
        (bind _asbp_enemy_master (Utilities|Casting|CastToBP_Enemy_Master _returnvalue))
        (EventDispatchers|BindEventtoDeathDispatcher _asbp_enemy_master (delegate Custom|DeathChecker))
        (Variables|Default|SetEnemyRespawnAnimation false)))))

(event Custom|NextWave
  (if (CallFunction|AllEnemiesDead?)
    (Variables|Default|SetEnemyRespawnAnimation true)
    (bind _enemiesamount (CallFunction|GetWaveEnemiesAmount))
    (Variables|Default|SetAmountEnemies _enemiesamount)
    (bind _result (Math|Integer|IncrementInt (Variables|Default|GetCurrentWave))
      (:%20%20
        (if (> _result (.waveamount (Variables|/Game/Blueprints/Stages/BP_StageManager.BP_StageManager_C|GetCurrentStageStruct (Variables|Default|GetStageManager))))
          (Variables|/Game/Blueprints/Stages/BP_StageManager.BP_StageManager_C|SetWavesCompleted (Variables|Default|GetStageManager) true)
          (Variables|Default|SetCurrentWave (.waveamount (Variables|/Game/Blueprints/Stages/BP_StageManager.BP_StageManager_C|GetCurrentStageStruct (Variables|Default|GetStageManager))))
          (Utilities|FlowControl|Delay 2.0)
          (Default|AddVictoryScreen (Variables|Default|GetStageManager))
          (else
            (Utilities|FlowControl|Delay 2.0)
            (bind _enemiesamount_2 (CallFunction|GetWaveEnemiesAmount))
            (CallFunction|SpawnEnemies _enemiesamount_2)))))))

(event Custom|DeathChecker
  ;[1 1 1] Spawn a given amount of enemies, avoids to spawn them on the same grid tile
  (if (Utilities|Array|IsEmpty (Variables|Default|GetEnemies))
    (CallFunction|NextWave)))

(event EventBeginPlay
  (CallFunction|SetEnemiesPool)
  (bind _returnvalue (Actor|GetActorOfClass "/Game/Blueprints/Grid/BP_GridManager.BP_GridManager_C"))
  (Variables|Default|SetGridManager _returnvalue)
  (bind _returnvalue_2 (Actor|GetActorOfClass "/Game/Blueprints/Stages/BP_StageManager.BP_StageManager_C"))
  (Variables|Default|SetStageManager _returnvalue_2)
  (Utilities|FlowControl|Delay 0.1)
  (bind _enemiesamount (CallFunction|GetWaveEnemiesAmount))
  (CallFunction|SpawnEnemies _enemiesamount))

(fn ConstructionScript)

(fn SetEnemiesPool
  (Utilities|Array|Add (Variables|Default|GetEnemiesPool) (Variables|Enemies|GetEnemy_Bulldozer))
  (Utilities|Array|Add (Variables|Default|GetEnemiesPool) (Variables|Enemies|GetEnemy_LaserTurret))
  (Utilities|Array|Add (Variables|Default|GetEnemiesPool) (Variables|Enemies|GetEnemy_Bomberman)))

(fn GetRandomEnemy
  (bind _enemiespool (Variables|Default|GetEnemiesPool))
  (if (and (== (Variables|/Game/Blueprints/Stages/BP_StageManager.BP_StageManager_C|GetCurrentStage (Variables|Default|GetStageManager)) 7) (== (Variables|Default|GetCurrentWave) 3))
    (LocalVariables|SetEnemyToSpawn "/Game/Enemies/BP_Boss_Bulldozer.BP_Boss_Bulldozer_C")
    (else
      (LocalVariables|SetEnemyToSpawn (Utilities|Array|Get(acopy) _enemiespool (Math|Random|RandomInteger (Utilities|Array|Length _enemiespool))))))
  (return (LocalVariables|GetEnemyToSpawn)))

(fn AllEnemiesDead?
  (return (== (Utilities|Array|Length (Variables|Default|GetEnemies)) 0)))

(fn GetWaveEnemiesAmount
  (bind _stagemanager (Variables|Default|GetStageManager))
  (bind _currentstagestruct (Variables|/Game/Blueprints/Stages/BP_StageManager.BP_StageManager_C|GetCurrentStageStruct _stagemanager))
  (switch int (Variables|Default|GetCurrentWave)
    (:1
      (LocalVariables|SetNumberEnemies (.wave1_enemiesamount _currentstagestruct)))
    (:2
      (LocalVariables|SetNumberEnemies (.wave2_enemiesamount _currentstagestruct)))
    (:3
      (LocalVariables|SetNumberEnemies (.wave3_enemiesamount _currentstagestruct))))
  (return (LocalVariables|GetNumberEnemies)))

(fn SetEnemySpawnTile
  (return (Variables|Default|GetSpawnTile)))