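; Bulldozer boss, a grid-based mining mech enemy that randomly moves or attacks whenever it is neither stunned nor occupied.
; A delayed Tick counts down separate light, medium and heavy cooldowns, then rolls the next action.
; Attacks spawn Drill Stab, Landslide or Giant Shockwave actors alongside montages or animations.
; The shockwave first moves the boss to a fixed tile, then holds it occupied through timer-chained smashes with camera shakes.
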(event Custom|HeavyAttack:GiantShockwave
  (bind _currentgridtile (Variables|Default|GetCurrentGridTile))
  (bind _neighborwest (Variables|/Game/Blueprints/Grid/BP_GridTile.BP_GridTile_C|GetNeighborWest _currentgridtile))
  (if (Variables|HeavyAttack|GetHeavyAttackReady)
    (CallFunction|MovetoTile (Utilities|Array|Get(acopy) (Variables|/Game/Blueprints/Grid/BP_GridManager.BP_GridManager_C|GetGridArray (Variables|Default|GetGridManager)) 22))
    (Components|Animation|PlayAnimation (Variables|Default|GetSkeletalMesh) "/Game/MiningMech/Animations/ANIM_MiningMech_JumpSmashAttack_Montage.ANIM_MiningMech_JumpSmashAttack_Montage" false)
    (Variables|Default|SetOcuppied true)
    (Utilities|FlowControl|Delay 1.0)
    (bind _returnvalue (Actor|GetActorOfClass "/Game/Blueprints/BP_Camera.BP_Camera_C"))
    (Default|BossCameraShake _returnvalue)
    (Game|SpawnActorfromClass "/Game/Enemies/EnemyAttacks/BossAttacks/BP_BossAttack_GiantShockwave.BP_BossAttack_GiantShockwave_C" (Transformation|GetActorTransform _neighborwest) "Undefined" 0 _neighborwest 0)
    (Variables|HeavyAttack|SetHeavyAttackReady false)
    (Variables|HeavyAttack|SetHeavyAttackTimer (Variables|HeavyAttack|GetHeavyAttackCooldown))
    (Variables|Default|SetHeavyAttackCounter 4)
    (Utilities|Time|SetTimerbyEvent (delegate Custom|KeepSmashing) 1.6)))

(event Custom|MediumAttack:Landslide
  (if (Variables|MediumAttack|GetMediumAttackReady)
    (Components|Animation|PlayAnimation (Variables|Default|GetSkeletalMesh) "/Game/MiningMech/Animations/ANIM_MiningMech_SmashAttack_Montage.ANIM_MiningMech_SmashAttack_Montage" false)
    (Game|SpawnActorfromClass "/Game/Enemies/EnemyAttacks/BossAttacks/BP_BossAttack_Landslide.BP_BossAttack_Landslide_C" (Transformation|GetActorTransform (Variables|Default|GetCurrentGridTile)) "Undefined" 0 0)
    (Variables|MediumAttack|SetMediumAttackReady false)
    (Variables|MediumAttack|SetMediumAttackTimer (Variables|MediumAttack|GetMediumAttackCooldown))
    (Utilities|FlowControl|Delay 0.2)
    (bind _returnvalue (Actor|GetActorOfClass "/Game/Blueprints/BP_Camera.BP_Camera_C"))
    (Default|BossCameraShake _returnvalue)))

(event Custom|LightAttack:DrillStab
  (bind _currentgridtile (Variables|Default|GetCurrentGridTile))
  (if (Variables|LightAttack|GetLightAttackReady)
    (Components|Animation|PlayAnimation (Variables|Default|GetSkeletalMesh) "/Game/MiningMech/Animations/ANIM_MiningMech_UppercutDrillAttack.ANIM_MiningMech_UppercutDrillAttack" false)
    (Audio|PlaySoundatLocation "/Game/Audio/SoundEffects/Boss_Bulldozer/Drillcharge.Drillcharge" "0, 0, 0" "0, 0, 0" 1.0 1.0 0.0 0 0 0 0)
    (Game|SpawnActorfromClass "/Game/Enemies/EnemyAttacks/BossAttacks/BP_BossAttack_DrillStab.BP_BossAttack_DrillStab_C" (Transformation|GetActorTransform _currentgridtile) "Undefined" 0 self _currentgridtile 0)
    (Variables|LightAttack|SetLightAttackReady false)
    (Variables|LightAttack|SetLightAttackTimer (Variables|LightAttack|GetLightAttackCooldown))
    (Variables|Default|SetOcuppied true)))

(event Custom|KeepSmashing
  (if (!= (Variables|Default|GetHeavyAttackCounter) 0)
    (if (Variables|Default|GetOcuppied)
      (Components|Animation|PlayAnimation (Variables|Default|GetSkeletalMesh) "/Game/MiningMech/Animations/ANIM_MiningMech_SmashAttack_Montage.ANIM_MiningMech_SmashAttack_Montage" false)
      (Utilities|FlowControl|Delay 0.4)
      (bind _returnvalue (Actor|GetActorOfClass "/Game/Blueprints/BP_Camera.BP_Camera_C"))
      (Default|BossCameraShake _returnvalue)
      (Math|Integer|DecrementInt (Variables|Default|GetHeavyAttackCounter)
        (:%20%20
          (Utilities|Time|SetTimerbyEvent (delegate Custom|KeepSmashing) 1.6))))
    (else
      (Variables|Default|SetOcuppied false)
      (Variables|Default|SetHeavyAttackCounter 4))))

(event EventBeginPlay
  (|CallParentFunction))

(event EventTick
  (params (DeltaSeconds :type Float%20%28single-precision%29))
  (Utilities|FlowControl|Delay 0.5)
  (if (not (Variables|Default|GetStunned))
    (Utilities|FlowControl|Sequence
      (:then_0
        (CallFunction|LightAttackCountdown)
        (CallFunction|MediumAttackCountdown)
        (CallFunction|HeavyAttackCountdown))
      (:then_1
        (if (not (Variables|Default|GetOcuppied))
          (switch int (Math|Random|RandomIntegerinRange 0 4)
            (:0
              (CallFunction|RandomizeMovement)
              (CallFunction|MovetoTile (Variables|Default|GetMovementTargetTile))
              (Components|Animation|PlayAnimation (Variables|Default|GetSkeletalMesh) "/Game/MiningMech/Animations/ANIM_MiningMech_Landing.ANIM_MiningMech_Landing" false))
            (:1
              (CallFunction|LightAttack:DrillStab))
            (:2
              (CallFunction|MediumAttack:Landslide))
            (:3
              (CallFunction|HeavyAttack:GiantShockwave))))))))

(fn ConstructionScript
  (|CallParentFunction))

(fn LightAttackCountdown
  (if (not (Variables|LightAttack|GetLightAttackReady))
    (bind _result (Math|Integer|DecrementInt (Variables|LightAttack|GetLightAttackTimer))
      (:%20%20
        (if (== _result 0)
          (Variables|LightAttack|SetLightAttackReady true))))))

(fn MediumAttackCountdown
  (if (not (Variables|MediumAttack|GetMediumAttackReady))
    (bind _result (Math|Integer|DecrementInt (Variables|MediumAttack|GetMediumAttackTimer))
      (:%20%20
        (if (== _result 0)
          (Variables|MediumAttack|SetMediumAttackReady true))))))

(fn HeavyAttackCountdown
  (if (not (Variables|HeavyAttack|GetHeavyAttackReady))
    (bind _result (Math|Integer|DecrementInt (Variables|HeavyAttack|GetHeavyAttackTimer))
      (:%20%20
        (if (== _result 0)
          (Variables|HeavyAttack|SetHeavyAttackReady true))))))