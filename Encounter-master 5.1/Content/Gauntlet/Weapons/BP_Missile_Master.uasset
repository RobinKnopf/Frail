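; Base homing missile projectile that chases the player weapon's locked target.
; On BeginPlay it reads MissileTarget from the player's BP_Weapon_Master, homes on that BP_Steve's mesh and stores its location once as Destination.
; Overlapping any BPI_Enemy actor reports that stored Destination to the weapon and destroys the missile; direct damage exists only in unused backup logic.
; LockedTargetDied also destroys it, and SetWeaponTrail attaches a trail effect.
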(event OnComponentBeginOverlap(Cylinder)
  (params (OverlappedComponent :type Primitive%20Component%20Object%20Reference) (OtherActor :type Actor%20Object%20Reference) (OtherComp :type Primitive%20Component%20Object%20Reference) (OtherBodyIndex :type Integer) (bFromSweep :type Boolean) (SweepResult :type Hit%20Result%20Structure%20%28by%20ref%29))
  (if (Utilities|DoesObjectImplementInterface OtherActor "/Game/Gauntlet/Blueprints/BPI_Enemy.BPI_Enemy_C")
    (Variables|Default|SetHit%20Actor OtherActor)
    (Class|BPIWeapons|ProjectileReachedDestination(Message) (Variables|Default|GetAs%20BP%20Weapon%20Master) (Variables|Default|GetDestination) 0 false)
    (Actor|DestroyActor)))

(event Custom|Set%20Weapon%20Trail
  (Niagara|SpawnSystemAttached "/Game/Gauntlet/Weapons/Niagara/Projectile_Trail_Master_System.Projectile_Trail_Master_System" (Variables|Default|GetCylinder) "None" "0, 0, 0" "90.000000,0.000000,0.000000" "KeepRelativeOffset" false))

(event EventBeginPlay
  (bind _asbp_player_character (Utilities|Casting|CastToBP_PlayerCharacter (Game|GetPlayerCharacter 0)))
  (bind _output_get (Variables|Default|SetAs%20BP%20Player%20Character _asbp_player_character))
  (bind _asbp_weapon_master (Utilities|Casting|CastToBP_Weapon_Master (Variables|/Script/Engine.ChildActorComponent|GetChildActor (Variables|/Game/Character/BP_PlayerCharacter.BP_PlayerCharacter_C|GetWeaponAttachment _output_get))))
  (bind _output_get_2 (Variables|Default|SetAs%20BP%20Weapon%20Master _asbp_weapon_master))
  (bind _output_get_3 (Variables|Default|SetMissile%20Target (Variables|/Game/Gauntlet/Weapons/BP_Weapon_Master.BP_Weapon_Master_C|GetMissile%20Target _output_get_2)))
  (bind _asbp_steve (Utilities|Casting|CastToBP_Steve _output_get_3))
  (Variables|/Script/Engine.ProjectileMovementComponent|SetHomingTargetComponent (Variables|Default|GetProjectileMovement) (Variables|/Script/Engine.Character|GetMesh _asbp_steve))
  (Variables|Default|SetDestination (Transformation|GetWorldLocation (Variables|/Script/Engine.Character|GetMesh _asbp_steve))))

(event EventLockedTargetDied
  (Actor|DestroyActor))

(fn ConstructionScript)