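; Base projectile for player and BP_Steve weapons, covering bullets, rockets, missiles and grenades.
; BeginPlay caches the owner and sets homing targets for player missiles and all Steve projectiles.
; On overlap, bullets apply damage and pierce with modified damage until their hit count runs out; impacts report to the weapon or Steve.
; Grenades can follow a spline via timeline, reporting the endpoint with a decremented bounce count before destroying themselves.
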(event OnComponentBeginOverlap(ProjectileMesh)
  (params (OverlappedComponent :type Primitive%20Component%20Object%20Reference) (OtherActor :type Actor%20Object%20Reference) (OtherComp :type Primitive%20Component%20Object%20Reference) (OtherBodyIndex :type Integer) (bFromSweep :type Boolean) (SweepResult :type Hit%20Result%20Structure%20%28by%20ref%29))
  (bind _returnvalue (Components|GetOwner))
  (bind _rootcomponent (Variables|/Script/Engine.Actor|GetRootComponent OtherActor))
  (bind _returnvalue_2 (Transformation|GetWorldLocation _rootcomponent))
  ;[1 1 1] Bullet, Rocket Missile
  (if (!= OtherActor _returnvalue)
    (switch Utilities|FlowControl|Switch|SwitchonProjectileType_Enum (Variables|Default|GetProjectile%20Type)
      (:NewEnumerator0
        (Game|Damage|ApplyDamage OtherActor (Variables|Default|GetProjectile%20Damage) 0 _returnvalue)
        (if (Variables|Default|GetIsPlayerCharacter)
          (Default|ProjectileReachedDestination (Variables|Default|GetAs%20BP%20Weapon%20Master) _returnvalue_2 0 false OtherActor)
          (else
            (Default|ProjectileReachedDestination (Variables|Default|GetAs%20BP%20Steve) _returnvalue_2 0 false OtherActor))))
      (:NewEnumerator3
        (if (Variables|Default|GetIsPlayerCharacter) :!label _label
          (Default|ProjectileReachedDestination (Variables|Default|GetAs%20BP%20Weapon%20Master) _returnvalue_2 0 false)
          (else
            (Default|ProjectileReachedDestination (Variables|Default|GetAs%20BP%20Steve) _returnvalue_2 0 false))))
      (:NewEnumerator1
        (goto _label))
      (:NewEnumerator2
        (goto _label)))
    (switch Utilities|FlowControl|Switch|SwitchonProjectileType_Enum (Variables|Default|GetProjectile%20Type)
      (:NewEnumerator0
        (Math|Integer|DecrementInt (Variables|Default|GetHitCount)
          (:%20%20
            (if true
              (Variables|Default|SetProjectile%20Damage (* (Variables|Default|GetProjectile%20Damage) (Variables|Default|GetSHD%20Modifier))))
            (if (== (Variables|Default|GetHitCount) 0)
              (Actor|DestroyActor)))))
      (:NewEnumerator3
        (Actor|DestroyActor))
      (:NewEnumerator1
        (Actor|DestroyActor)))))

(event Custom|Move%20Grenade
  (bind _track_reference (Variables|Default|GetTrack%20Reference))
  (bind _bounce_counter (Variables|Default|GetBounce%20Counter))
  (bind _track_reference_2 (Variables|Default|GetTrack%20Reference))
  (bind _trajectory_spline (Variables|/Game/Gauntlet/Weapons/BP_Trajectory.BP_Trajectory_C|GetTrajectory%20Spline _track_reference_2))
  (bind _spline_end (Variables|/Game/Gauntlet/Weapons/BP_Trajectory.BP_Trajectory_C|GetSpline%20End _track_reference))
  (bind _returnvalue (Spline|GetSplineLength _trajectory_spline))
  ;[1 1 1] Grenade
  (Collision|SetCollisionEnabled (Variables|Default|GetProjectileMesh) "NoCollision")
  (Components|DestroyComponent (Variables|Default|GetProjectileMovement))
  (Components|Timeline|SetPlayRate (Variables|Default|GetTrajectory) (/ 1.0 (Variables|Default|GetDuration)))
  (Components|Timeline|SetNewTime (Variables|Default|GetTrajectory) (Variables|Default|GetStart%20Offset))
  (bind _alpha (Timeline|Trajectory Play)
    (:Update
      (Variables|Default|SetAlpha _alpha)
      (Transformation|SetActorLocationAndRotation (Spline|GetLocationatDistanceAlongSpline _trajectory_spline (Math|Float|Lerp 0.0 _returnvalue (Variables|Default|GetAlpha)) "World") (Spline|GetRotationatDistanceAlongSpline _trajectory_spline _returnvalue "World"))
      (if (> (Variables|Default|GetAlpha) 0.95)
        (Math|Integer|DecrementInt (Variables|Default|GetBounce%20Counter)
          (:%20%20
            (if (Variables|Default|GetIsPlayerCharacter)
              (Default|ProjectileReachedDestination (Variables|Default|GetAs%20BP%20Weapon%20Master) _spline_end _bounce_counter true)
              (else
                (Default|ProjectileReachedDestination (Variables|Default|GetAs%20BP%20Steve) _spline_end _bounce_counter true)))
            (Actor|DestroyActor (Variables|Default|GetTrack%20Reference))
            (Actor|DestroyActor)))))))

(event Custom|Set%20Weapon%20Trail
  (Niagara|SpawnSystemAttached "/Game/Gauntlet/Weapons/Niagara/Projectile_Trail_Master_System.Projectile_Trail_Master_System" (Variables|Default|GetProjectileMesh) "None" "0, 0, 0" "180.000000, 0, 0" "KeepRelativeOffset" false))

(event EventBeginPlay
  (bind _returnvalue (Game|GetPlayerCharacter 0))
  (bind _returnvalue_2 (Components|GetOwner))
  (bind _returnvalue_3 (== _returnvalue_2 _returnvalue))
  ;[1 1 1] Setup
  (Variables|Default|SetIsPlayerCharacter _returnvalue_3)
  (if _returnvalue_3
    (bind _asbp_player_character (Utilities|Casting|CastToBP_PlayerCharacter _returnvalue))
    (bind _output_get (Variables|Default|SetAs%20BP%20Player%20Character _asbp_player_character))
    (bind _asbp_weapon_master (Utilities|Casting|CastToBP_Weapon_Master (Variables|/Script/Engine.ChildActorComponent|GetChildActor (Variables|/Game/Character/BP_PlayerCharacter.BP_PlayerCharacter_C|GetWeaponAttachment _output_get))))
    (bind _output_get_2 (Variables|Default|SetAs%20BP%20Weapon%20Master _asbp_weapon_master))
    (switch Utilities|FlowControl|Switch|SwitchonProjectileType_Enum (Variables|Default|GetProjectile%20Type)
      (:NewEnumerator1
        (bind _output_get_3 (Variables|/Script/Engine.ProjectileMovementComponent|SetHomingTargetComponent (Variables|Default|GetProjectileMovement) (Variables|/Script/Engine.Actor|GetRootComponent (Variables|/Game/Gauntlet/Weapons/BP_Weapon_Master.BP_Weapon_Master_C|GetMissile%20Target _output_get_2))))
        (Development|PrintString (Utilities|GetDisplayName _output_get_3))))
    (else
      (bind _asbp_steve (Utilities|Casting|CastToBP_Steve _returnvalue_2))
      (Variables|Default|SetAs%20BP%20Steve _asbp_steve)
      (Variables|/Script/Engine.ProjectileMovementComponent|SetHomingTargetComponent (Variables|Default|GetProjectileMovement) (Variables|/Script/Engine.Actor|GetRootComponent (Variables|/Game/Gauntlet/BP_Steve.BP_Steve_C|GetTarget _asbp_steve))))))

(fn ConstructionScript)