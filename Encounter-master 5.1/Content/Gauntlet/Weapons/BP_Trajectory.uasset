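; Weapon trajectory Blueprint that shapes a spline into an arc between a start and an end location.
; The RemakeSpline event pins the first and third points of TrajectorySpline to SplineStart and SplineEnd in world space.
; It places the middle point at their midpoint, raised by a fixed height to form the arc.
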(event Custom|Remake%20Spline
  (bind _spline_end (Variables|Default|GetSpline%20End))
  (bind _spline_start (Variables|Default|GetSpline%20Start))
  (bind _returnvalue (+ _spline_start _spline_end))
  (bind _returnvalue_2 (/ _returnvalue 2))
  (Spline|SetLocationatSplinePoint (Variables|Default|GetTrajectory%20Spline) 0 (Variables|Default|GetSpline%20Start) "World" true)
  (Spline|SetLocationatSplinePoint (Variables|Default|GetTrajectory%20Spline) 2 (Variables|Default|GetSpline%20End) "World" true)
  (Spline|SetLocationatSplinePoint (Variables|Default|GetTrajectory%20Spline) 1 (Math|Vector|MakeVector (.x _returnvalue_2) (.y _returnvalue_2) (+ (.z _returnvalue_2) 2e+02)) "World" true))

(fn ConstructionScript)