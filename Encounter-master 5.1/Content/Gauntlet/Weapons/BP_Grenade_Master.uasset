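; Master grenade actor that flies along a spline trajectory and reports back to the player's weapon when it nears the end.
; BeginPlay caches the player character and its attached weapon.
; MoveGrenade runs a timeline scaled by duration and start offset, positioning the grenade along the referenced spline with the end-point rotation.
; Past 95%, it passes its location and decremented bounce counter to the weapon as a bounce, then destroys the track and itself.
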(event Custom|MoveGrenade
  (bind _track_reference (Variables|Default|GetTrack%20Reference))
  (bind _trajectory_spline (Variables|/Game/Gauntlet/Weapons/BP_Trajectory.BP_Trajectory_C|GetTrajectory%20Spline _track_reference))
  (bind _returnvalue (Spline|GetSplineLength _trajectory_spline))
  (Components|Timeline|SetPlayRate (Variables|Default|GetTrajectory) (/ 1.0 (Variables|Default|GetDuration)))
  (Components|Timeline|SetNewTime (Variables|Default|GetTrajectory) (Variables|Default|GetStart%20Offset))
  (bind _alpha (Timeline|Trajectory Play)
    (:Update
      (Variables|Default|SetAlpha _alpha)
      (Transformation|SetActorLocationAndRotation (Spline|GetLocationatDistanceAlongSpline _trajectory_spline (Math|Float|Lerp 0.0 _returnvalue (Variables|Default|GetAlpha)) "World") (Spline|GetRotationatDistanceAlongSpline _trajectory_spline _returnvalue "World"))
      (if (> (Variables|Default|GetAlpha) 0.95)
        (bind _result (Math|Integer|DecrementInt (Variables|Default|GetBounce%20Counter))
          (:%20%20
            (Default|ProjectileReachedDestination (Variables|Default|GetAs%20BP%20Weapon%20Master) (Transformation|GetWorldLocation (Variables|Default|GetGrenade)) _result true)
            (Actor|DestroyActor (Variables|Default|GetTrack%20Reference))
            (Actor|DestroyActor)))))))

(event EventBeginPlay
  (bind _asbp_player_character (Utilities|Casting|CastToBP_PlayerCharacter (Game|GetPlayerCharacter 0)))
  (bind _output_get (Variables|Default|SetAs%20BP%20Player%20Character _asbp_player_character))
  (bind _asbp_weapon_master (Utilities|Casting|CastToBP_Weapon_Master (Variables|/Script/Engine.ChildActorComponent|GetChildActor (Variables|/Game/Character/BP_PlayerCharacter.BP_PlayerCharacter_C|GetWeaponAttachment _output_get))))
  (Variables|Default|SetAs%20BP%20Weapon%20Master _asbp_weapon_master))

(fn ConstructionScript)