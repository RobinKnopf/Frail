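; BP_Steve is an enemy with a health bar widget and a self-repeating, delayed projectile attack.
; The attack loops while PlayerInSight holds; leaving EyeSight clears it, but the overlap logic that sets it and starts attacks is disconnected.
; Projectiles reaching their destination trigger an area secondary effect with bounced-grenade parameters.
; Damage updates the bar, reduces health and spawns material-based impact effects, with no death handling here.
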(event OnComponentEndOverlap(EyeSight)
  (params (OverlappedComponent :type Primitive%20Component%20Object%20Reference) (OtherActor :type Actor%20Object%20Reference) (OtherComp :type Primitive%20Component%20Object%20Reference) (OtherBodyIndex :type Integer))
  (if (== OtherActor (Game|GetPlayerCharacter 0))
    (Variables|Default|SetPlayer%20In%20Sight false)))

(event OnComponentBeginOverlap(EyeSight)
  (params (OverlappedComponent :type Primitive%20Component%20Object%20Reference) (OtherActor :type Actor%20Object%20Reference) (OtherComp :type Primitive%20Component%20Object%20Reference) (OtherBodyIndex :type Integer) (bFromSweep :type Boolean) (SweepResult :type Hit%20Result%20Structure%20%28by%20ref%29)))

(event Custom|Make%20Steve%20Attack
  (Utilities|FlowControl|Delay (Variables|Default|GetReactionTime))
  (Utilities|SpawnProjectile 1 (Variables|Default|GetModify%20Subsequent%20Hit%20Damage) "/Game/Sci-Fi_Starter_VFX_Pack_Niagara/Niagara/MuzzleFlash/NS_MuzzleFlash_1.NS_MuzzleFlash_1" (Transformation|GetWorldLocation (Variables|Collision|GetCapsuleComponent)) "/Game/Gauntlet/Weapons/BP_Projectile_Master.BP_Projectile_Master_C" 12.0 self (Variables|Default|GetSubsequent%20Hit%20Damage%20Multiplier) false 0 false
    (:__
      (Utilities|FlowControl|Delay 0.5)
      (if (Variables|Default|GetPlayer%20In%20Sight)
        (CallFunction|MakeSteveAttack)))))

(event EventBeginPlay
  (CallFunction|CreateHPBar))

(event Game|Damage|EventAnyDamage
  (params (Damage :type Float%20%28single-precision%29) (DamageType :type Damage%20Type%20Object%20Reference) (InstigatedBy :type Controller%20Object%20Reference) (DamageCauser :type Actor%20Object%20Reference))
  ;[1 1 1] Damage Application
  (Default|ShowDamageTaken (Variables|Default|GetHPBarWidget) Damage)
  (Variables|Default|SetHealthPoints (- (Variables|Default|GetHealthPoints) Damage))
  (Niagara|SpawnSystematLocation (Utilities|Select :Index (Variables|Default|GetGeneral%20Material) :NewEnumerator0 "/Game/Sci-Fi_Starter_VFX_Pack_Niagara/Niagara/Impact/NS_Impact_Metal_1.NS_Impact_Metal_1" :NewEnumerator1 "/Game/Sci-Fi_Starter_VFX_Pack_Niagara/Niagara/Blood/NS_Blood_Mesh_5.NS_Blood_Mesh_5") (Transformation|GetWorldLocation (Variables|Character|GetMesh)))
  (Development|PrintString "ouch"))

(event EventProjectileReachedDestination
  (params (Destination :type Vector :default "0, 0, 0") (Bounce%20Counter :type Integer) (Bounced%20Grenade :type Boolean) (Actor%20To%20Ignore :type Actor%20Object%20Reference) (Instigator :type Character%20Object%20Reference))
  (Utilities|SecondaryEffect true Destination "NewEnumerator1" "NewEnumerator0" 1 Bounced%20Grenade Actor%20To%20Ignore Bounce%20Counter (Variables|Default|GetAOE%20Niagara%20System) self "/Game/Gauntlet/Weapons/BP_Projectile_Master.BP_Projectile_Master_C" (* (Variables|Default|GetBounced%20Grenade%20Range) -1) 5e+01))

(fn ConstructionScript)

(fn CreateHPBar
  (bind _returnvalue (UserInterface|CreateWidget "/Game/UserInterface/WBP_EnemyHP.WBP_EnemyHP_C"))
  (bind _output_get (Variables|Default|SetHPBarWidget _returnvalue))
  (Default|SetOwner _output_get self)
  (UserInterface|SetWidget (Variables|Default|GetHPBar) (Variables|Default|GetHPBarWidget)))