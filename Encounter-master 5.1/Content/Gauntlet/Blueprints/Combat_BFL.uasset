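; Blueprint function library of combat helpers for trace-based weapon attacks and area-of-effect damage.
; PerformTraceAttack fires a forward sphere trace at fixed height, damaging unique actors up to a penetration count with optional per-hit damage scaling, plus muzzle flash and beam trail effects.
; SelectAOEType dispatches to box, plus, cross, horizontal, vertical or chained-arc box traces.
; Hit pools prevent duplicate damage; most AOE shapes only damage BPI_Enemy implementers, and debug drawing remains on.
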(fn SetTraceLocations
  (params (Actor%20Reference :type Actor%20Object%20Reference) (Length :type Integer))
  (bind _returnvalue (* Length 100))
  (bind _rootcomponent (Variables|/Script/Engine.Actor|GetRootComponent Actor%20Reference))
  (bind _returnvalue_2 (Transformation|GetWorldLocation _rootcomponent))
  (bind _returnvalue_3 (Math|Vector|GetForwardVector _rootcomponent))
  (bind (_x _y) (Math|Vector|BreakVector _returnvalue_2))
  (bind _returnvalue_4 (* _returnvalue_3 _returnvalue))
  (bind _returnvalue_5 (+ _returnvalue_2 _returnvalue_4))
  (bind (_x_2 _y_2) (Math|Vector|BreakVector _returnvalue_5))
  (return (Math|Vector|MakeVector _x _y 1e+02) (Math|Vector|MakeVector _x_2 _y_2 1e+02)))

(fn PerformTraceAttack
  (params (Effective%20Range :type Integer) (Penetration%20Amount :type Integer) (Modify%20Subsequent%20Hit%20Damage :type Boolean) (Muzzle%20Flash%20System :type Niagara%20System%20Object%20Reference) (Muzzle%20Flash%20Location :type Vector) (Actor%20that%20Fires :type Actor%20Object%20Reference) (Base%20Damage :type Float%20%28double-precision%29) (Subsequent%20Damage%20Modifier :type Float%20%28double-precision%29) (DrawDebugType :type EDrawDebugTrace%20Enum :default "None") (Weapon%20Trail%20System :type Niagara%20System%20Object%20Reference) (Weapon%20Trail%20Duration :type Float%20%28double-precision%29) (Has%20Weapon%20Trail :type Boolean))
  (bind (_actor_location _trace_end_location) (CallFunction|SetTraceLocations Actor%20that%20Fires Effective%20Range))
  (Niagara|SpawnSystematLocation 0 Muzzle%20Flash%20System Muzzle%20Flash%20Location)
  (LocalVariables|SetPen%20Counter Penetration%20Amount)
  (LocalVariables|SetTemp%20Base%20Damage Base%20Damage)
  (LocalVariables|SetHit%20Damage%20Modifier Subsequent%20Damage%20Modifier)
  (LocalVariables|SetTrace%20End _trace_end_location)
  (bind _outhits (Collision|MultiSphereTraceByChannel 0 _actor_location _trace_end_location 1e+01 "TraceTypeQuery3" false (Utilities|Array|MakeArray Actor%20that%20Fires) DrawDebugType))
  (bind _array_element (Utilities|Array|ForEachLoopwithBreak _outhits :!label _label)
    (:LoopBody
      (bind _output_get (LocalVariables|SetImpact%20Point (.ImpactPoint (Collision|BreakHitResult _array_element))))
      (LocalVariables|SetTrace%20End _output_get)
      (if (not (Utilities|Array|ContainsItem (LocalVariables|GetActor%20Hit%20Pool) (.HitActor (Collision|BreakHitResult _array_element))))
        (Development|PrintString 0 (Utilities|GetDisplayName (.HitActor (Collision|BreakHitResult _array_element))))
        (Game|Damage|ApplyDamage (.HitActor (Collision|BreakHitResult _array_element)) (LocalVariables|GetTemp%20Base%20Damage) 0 0)
        (Utilities|Array|Add (LocalVariables|GetActor%20Hit%20Pool) (.HitActor (Collision|BreakHitResult _array_element)))
        (bind _new_temp_base_damage (CallFunction|SubsequentHitDamageModifier Modify%20Subsequent%20Hit%20Damage (LocalVariables|GetTemp%20Base%20Damage) (LocalVariables|GetHit%20Damage%20Modifier)))
        (LocalVariables|SetTemp%20Base%20Damage _new_temp_base_damage)
        (Math|Integer|DecrementInt (LocalVariables|GetPen%20Counter)
          (:%20%20
            (if (<= (LocalVariables|GetPen%20Counter) 0)
              (goto _label Break))))))
    (:Completed
      (Utilities|Array|Clear (LocalVariables|GetActor%20Hit%20Pool))
      (CallFunction|WeaponTrail Has%20Weapon%20Trail Weapon%20Trail%20System Muzzle%20Flash%20Location (LocalVariables|GetTrace%20End) Weapon%20Trail%20Duration)
      (return (LocalVariables|GetTrace%20End) (.HitActor (Collision|BreakHitResult _array_element))))))

(fn SubsequentHitDamageModifier
  (params (Modify%20Subsequent%20Hit%20Damage :type Boolean) (Temp%20Base%20Damage :type Float%20%28double-precision%29) (Hit%20Damage%20Modifier :type Float%20%28double-precision%29))
  (if Modify%20Subsequent%20Hit%20Damage
    (return (* Temp%20Base%20Damage Hit%20Damage%20Modifier))
    (else
      (return Temp%20Base%20Damage))))

(fn WeaponTrail
  (params (Has%20Weapon%20Trail :type Boolean) (Weapon%20Trail%20System :type Niagara%20System%20Object%20Reference) (Trail%20Start%20Location :type Vector) (Trail%20End%20Location :type Vector) (Weapon%20Trail%20Duration :type Float%20%28double-precision%29))
  (if Has%20Weapon%20Trail
    (bind _returnvalue (Niagara|SpawnSystematLocation 0 Weapon%20Trail%20System Trail%20Start%20Location))
    (bind _output_get (LocalVariables|SetWeapon%20Trail _returnvalue))
    (Effects|Components|ParticleSystem|SetVectorParameter _output_get "User.Beam End" Trail%20End%20Location)
    (Effects|Components|ParticleSystem|SetFloatParameter _output_get "User.Weapon Trail Duration" Weapon%20Trail%20Duration)))

(fn SelectAOEType
  (params (AOE%20Type :type AOEType_Enum%20Enum :default "NewEnumerator0") (AOE%20Size :type Integer) (Actor%20To%20Ignore :type Actor%20Object%20Reference) (Origin :type Vector) (AOE%20System :type Niagara%20System%20Object%20Reference) (AOE%20Damage :type Float%20%28double-precision%29))
  (Utilities|FlowControl|Sequence
    (:then_0
      (LocalVariables|SetType AOE%20Type)
      (LocalVariables|SetSize AOE%20Size)
      (LocalVariables|SetIgnore Actor%20To%20Ignore)
      (LocalVariables|SetLocation Origin)
      (LocalVariables|SetSystem AOE%20System)
      (LocalVariables|SetDamage AOE%20Damage))
    (:then_1
      (switch Utilities|FlowControl|Switch|SwitchonAOEType_Enum (LocalVariables|GetType)
        (:NewEnumerator0
          ;[1 1 1] Box AOE
          (CallFunction|BoxAOE (LocalVariables|GetLocation) (LocalVariables|GetSize) (LocalVariables|GetIgnore) (LocalVariables|GetSystem) (LocalVariables|GetDamage))
          (Development|PrintString 0 "Box AOE"))
        (:NewEnumerator1
          ;[1 1 1] Plus AOE
          (CallFunction|+AOE (LocalVariables|GetLocation) (LocalVariables|GetSystem) (LocalVariables|GetDamage) (LocalVariables|GetIgnore) (LocalVariables|GetSize))
          (Development|PrintString 0 "+ AOE"))
        (:NewEnumerator2
          ;[1 1 1] Cross AOE
          (CallFunction|CrossAOE (LocalVariables|GetLocation) (LocalVariables|GetSystem) (LocalVariables|GetDamage) (LocalVariables|GetIgnore) (LocalVariables|GetSize))
          (Development|PrintString 0 "X AOE"))
        (:NewEnumerator3
          ;[1 1 1] Horizontal AOE
          (CallFunction|HorizontalAOE (LocalVariables|GetLocation) (LocalVariables|GetSystem) (LocalVariables|GetDamage) (LocalVariables|GetIgnore) (LocalVariables|GetSize))
          (Development|PrintString 0 "Horizontal  AOE"))
        (:NewEnumerator4
          ;[1 1 1] Vertical AOE
          (CallFunction|VerticalAOE (LocalVariables|GetLocation) (LocalVariables|GetSystem) (LocalVariables|GetDamage) (LocalVariables|GetIgnore) (LocalVariables|GetSize))
          (Development|PrintString 0 "Vertical AOE"))
        (:NewEnumerator5
          ;[1 1 1] Arc AOE
          (CallFunction|ArcAOE (LocalVariables|GetLocation) (LocalVariables|GetSystem) (LocalVariables|GetDamage) 0 (LocalVariables|GetIgnore))
          (Development|PrintString 0 "ARC AOE"))))))

(fn BoxAOE
  (params (Origin :type Vector) (AOE%20Size :type Integer) (Actor%20To%20Ignore :type Actor%20Object%20Reference) (AOE%20System :type Niagara%20System%20Object%20Reference) (AOE%20Damage :type Float%20%28double-precision%29))
  (bind _returnvalue (- AOE%20Size 1))
  (bind _returnvalue_2 (* _returnvalue 1e+02))
  (bind _returnvalue_3 (+ _returnvalue_2 2e+01))
  (Niagara|SpawnSystematLocation 0 AOE%20System Origin "0, 0, 0" "0.400000,0.400000,0.400000")
  (bind _outhits (Class|KismetSystemLibrary|BoxTraceMulti 0 Origin Origin (Math|Vector|MakeVector _returnvalue_3 _returnvalue_3 2e+01) "0, 0, 0" "TraceTypeQuery3" false (Utilities|Array|MakeArray Actor%20To%20Ignore) "ForDuration" true))
  (for _array_element _outhits
    (if (not (Utilities|Array|ContainsItem (LocalVariables|GetHit%20Actor%20Pool) (.HitActor (Collision|BreakHitResult _array_element))))
      (Game|Damage|ApplyDamage (.HitActor (Collision|BreakHitResult _array_element)) AOE%20Damage 0 0)
      (Utilities|Array|Add (LocalVariables|GetHit%20Actor%20Pool) (.HitActor (Collision|BreakHitResult _array_element)))))
  (Utilities|Array|Clear (LocalVariables|GetHit%20Actor%20Pool)))

(fn ArcAOE
  (params (Origin :type Vector) (Arc%20Trail%20Effect :type Niagara%20System%20Object%20Reference) (Chained%20Hit%20Damage :type Float%20%28double-precision%29) (Ignore :type Actor%20Object%20Reference%20%28by%20ref%29))
  (LocalVariables|SetLocation Origin)
  (LocalVariables|SetChain%20Effect Arc%20Trail%20Effect)
  (LocalVariables|SetDamage Chained%20Hit%20Damage)
  (Utilities|Array|Add (LocalVariables|GetHit%20Actor%20Pool) Ignore)
  (Utilities|FlowControl|Sequence
    (:then_0
      (bind _outhits (Class|KismetSystemLibrary|BoxTraceMulti 0 (Math|Vector|MakeVector (+ (.X (Math|Vector|BreakVector (LocalVariables|GetLocation))) 1e+02) (+ (.Y (Math|Vector|BreakVector (LocalVariables|GetLocation))) 1.5e+02) (+ (.Z (Math|Vector|BreakVector (LocalVariables|GetLocation))) 0.0)) (Math|Vector|MakeVector (+ (.X (Math|Vector|BreakVector (LocalVariables|GetLocation))) -1e+02) (+ (.Y (Math|Vector|BreakVector (LocalVariables|GetLocation))) 1.5e+02) (+ (.Z (Math|Vector|BreakVector (LocalVariables|GetLocation))) 0.0)) "20.000000,20.000000,20.000000" "90.000000,0.000000,90.000000" "TraceTypeQuery3" false 0 "ForDuration" true))
      (for _array_element _outhits
        (if (Utilities|DoesObjectImplementInterface (.HitActor (Collision|BreakHitResult _array_element)) "/Game/Gauntlet/Blueprints/BPI_Enemy.BPI_Enemy_C")
          (if (not (Utilities|Array|ContainsItem (LocalVariables|GetHit%20Actor%20Pool) (.HitActor (Collision|BreakHitResult _array_element))))
            (Game|Damage|ApplyDamage (.HitActor (Collision|BreakHitResult _array_element)) (LocalVariables|GetDamage) 0 0)
            (Utilities|Array|Add (LocalVariables|GetHit%20Actor%20Pool) (.HitActor (Collision|BreakHitResult _array_element)))
            (bind _returnvalue (Niagara|SpawnSystematLocation 0 (LocalVariables|GetChain%20Effect) (LocalVariables|GetLocation) "0, 0, 0" (Math|Vector|MakeVector 1.0 1.0 1.0)))
            (Effects|Components|ParticleSystem|SetVectorParameter _returnvalue "User.Beam End" (.ImpactPoint (Collision|BreakHitResult _array_element))))))
      (Utilities|Array|Clear (LocalVariables|GetHit%20Actor%20Pool)))
    (:then_1
      (bind _outhits_2 (Class|KismetSystemLibrary|BoxTraceMulti 0 (Math|Vector|MakeVector (+ (.X (Math|Vector|BreakVector (LocalVariables|GetLocation))) 2e+02) (+ (.Y (Math|Vector|BreakVector (LocalVariables|GetLocation))) 2.5e+02) (+ (.Z (Math|Vector|BreakVector (LocalVariables|GetLocation))) 0.0)) (Math|Vector|MakeVector (+ (.X (Math|Vector|BreakVector (LocalVariables|GetLocation))) -2e+02) (+ (.Y (Math|Vector|BreakVector (LocalVariables|GetLocation))) 2.5e+02) (+ (.Z (Math|Vector|BreakVector (LocalVariables|GetLocation))) 0.0)) "20.000000,20.000000,20.000000" "90.000000,0.000000,90.000000" "TraceTypeQuery1" false 0 "ForDuration" true "(R=0.737699,G=0.295815,B=1.000000,A=1.000000)"))
      (for _array_element_2 _outhits_2
        (if (Utilities|DoesObjectImplementInterface (.HitActor (Collision|BreakHitResult _array_element_2)) "/Game/Gauntlet/Blueprints/BPI_Enemy.BPI_Enemy_C")
          (if (not (Utilities|Array|ContainsItem (LocalVariables|GetHit%20Actor%20Pool) (.HitActor (Collision|BreakHitResult _array_element_2))))
            (Game|Damage|ApplyDamage (.HitActor (Collision|BreakHitResult _array_element_2)) (LocalVariables|GetDamage) 0 0)
            (Utilities|Array|Add (LocalVariables|GetHit%20Actor%20Pool) (.HitActor (Collision|BreakHitResult _array_element_2)))
            (bind _returnvalue_2 (Niagara|SpawnSystematLocation 0 (LocalVariables|GetChain%20Effect) (LocalVariables|GetLocation) "0, 0, 0" (Math|Vector|MakeVector 1.0 1.0 1.0)))
            (Effects|Components|ParticleSystem|SetVectorParameter _returnvalue_2 "User.Beam End" (.ImpactPoint (Collision|BreakHitResult _array_element_2))))))
      (Utilities|Array|Clear (LocalVariables|GetHit%20Actor%20Pool)))))

(fn HorizontalAOE
  (params (Origin :type Vector) (AOE%20Effect :type Niagara%20System%20Object%20Reference) (AOE%20Damage :type Float%20%28double-precision%29) (Ignore :type Actor%20Object%20Reference%20%28by%20ref%29) (AOE%20Size :type Integer))
  (LocalVariables|SetLocation Origin)
  (LocalVariables|SetAOE%20System AOE%20Effect)
  (LocalVariables|SetDamage AOE%20Damage)
  (Utilities|Array|Add (LocalVariables|GetHit%20Actor%20Pool) Ignore)
  (LocalVariables|SetSize AOE%20Size)
  (Niagara|SpawnSystematLocation 0 (LocalVariables|GetAOE%20System) (LocalVariables|GetLocation) "0, 0, 0" "0.400000,0.400000,0.400000")
  (bind _outhits (Class|KismetSystemLibrary|BoxTraceMulti 0 (LocalVariables|GetLocation) (LocalVariables|GetLocation) (Math|Vector|MakeVector 2e+01 (* (LocalVariables|GetSize) 1e+02) 2e+01) "0, 0, 0" "TraceTypeQuery3" false 0 "ForDuration" true))
  (for _array_element _outhits
    (if (Utilities|DoesObjectImplementInterface (.HitActor (Collision|BreakHitResult _array_element)) "/Game/Gauntlet/Blueprints/BPI_Enemy.BPI_Enemy_C")
      (if (not (Utilities|Array|ContainsItem (LocalVariables|GetHit%20Actor%20Pool) (.HitActor (Collision|BreakHitResult _array_element))))
        (Game|Damage|ApplyDamage (.HitActor (Collision|BreakHitResult _array_element)) (LocalVariables|GetDamage) 0 0)
        (Utilities|Array|Add (LocalVariables|GetHit%20Actor%20Pool) (.HitActor (Collision|BreakHitResult _array_element))))))
  (Utilities|Array|Clear (LocalVariables|GetHit%20Actor%20Pool)))

(fn VerticalAOE
  (params (Origin :type Vector) (AOE%20Effect :type Niagara%20System%20Object%20Reference) (AOE%20Damage :type Float%20%28double-precision%29) (Ignore :type Actor%20Object%20Reference%20%28by%20ref%29) (AOE%20Size :type Integer) (__WorldContext :type Object%20Object%20Reference))
  (LocalVariables|SetLocation Origin)
  (LocalVariables|SetAOE%20System AOE%20Effect)
  (LocalVariables|SetDamage AOE%20Damage)
  (Utilities|Array|Add (LocalVariables|GetHit%20Actor%20Pool) Ignore)
  (LocalVariables|SetSize AOE%20Size)
  (Niagara|SpawnSystematLocation 0 (LocalVariables|GetAOE%20System) (LocalVariables|GetLocation) "0, 0, 0" "0.400000,0.400000,0.400000")
  (bind _outhits (Class|KismetSystemLibrary|BoxTraceMulti 0 (LocalVariables|GetLocation) (LocalVariables|GetLocation) (Math|Vector|MakeVector (* (LocalVariables|GetSize) 1e+02) 2e+01 2e+01) "0, 0, 0" "TraceTypeQuery3" false 0 "ForDuration" true))
  (for _array_element _outhits
    (if (Utilities|DoesObjectImplementInterface (.HitActor (Collision|BreakHitResult _array_element)) "/Game/Gauntlet/Blueprints/BPI_Enemy.BPI_Enemy_C")
      (if (not (Utilities|Array|ContainsItem (LocalVariables|GetHit%20Actor%20Pool) (.HitActor (Collision|BreakHitResult _array_element))))
        (Game|Damage|ApplyDamage (.HitActor (Collision|BreakHitResult _array_element)) (LocalVariables|GetDamage) 0 0)
        (Utilities|Array|Add (LocalVariables|GetHit%20Actor%20Pool) (.HitActor (Collision|BreakHitResult _array_element))))))
  (Utilities|Array|Clear (LocalVariables|GetHit%20Actor%20Pool)))

(fn +AOE
  (params (Origin :type Vector) (AOE%20Effect :type Niagara%20System%20Object%20Reference) (AOE%20Damage :type Float%20%28double-precision%29) (Ignore :type Actor%20Object%20Reference%20%28by%20ref%29) (AOE%20Size :type Integer) (__WorldContext :type Object%20Object%20Reference))
  (LocalVariables|SetLocation Origin)
  (LocalVariables|SetAOE%20System AOE%20Effect)
  (LocalVariables|SetDamage AOE%20Damage)
  (Utilities|Array|Add (LocalVariables|GetHit%20Actor%20Pool) Ignore)
  (LocalVariables|SetSize AOE%20Size)
  (Utilities|FlowControl|Sequence
    (:then_0
      ;[1 1 1] Horizontal
      (Niagara|SpawnSystematLocation 0 (LocalVariables|GetAOE%20System) (LocalVariables|GetLocation) "0, 0, 0" "0.400000,0.400000,0.400000")
      (bind _outhits (Class|KismetSystemLibrary|BoxTraceMulti 0 (LocalVariables|GetLocation) (LocalVariables|GetLocation) (Math|Vector|MakeVector 2e+01 (* (LocalVariables|GetSize) 1e+02) 2e+01) "0, 0, 0" "TraceTypeQuery3" false 0 "ForDuration" true))
      (for _array_element _outhits
        (if (Utilities|DoesObjectImplementInterface (.HitActor (Collision|BreakHitResult _array_element)) "/Game/Gauntlet/Blueprints/BPI_Enemy.BPI_Enemy_C")
          (if (not (Utilities|Array|ContainsItem (LocalVariables|GetHit%20Actor%20Pool) (.HitActor (Collision|BreakHitResult _array_element))))
            (Game|Damage|ApplyDamage (.HitActor (Collision|BreakHitResult _array_element)) (LocalVariables|GetDamage) 0 0)
            (Utilities|Array|Add (LocalVariables|GetHit%20Actor%20Pool) (.HitActor (Collision|BreakHitResult _array_element)))))))
    (:then_1
      ;[1 1 1] Vertical
      (Niagara|SpawnSystematLocation 0 (LocalVariables|GetAOE%20System) (LocalVariables|GetLocation) "0, 0, 0" "0.400000,0.400000,0.400000")
      (bind _outhits_2 (Class|KismetSystemLibrary|BoxTraceMulti 0 (LocalVariables|GetLocation) (LocalVariables|GetLocation) (Math|Vector|MakeVector (* (LocalVariables|GetSize) 1e+02) 2e+01 2e+01) "0, 0, 0" "TraceTypeQuery3" false 0 "ForDuration" true))
      (for _array_element_2 _outhits_2
        (if (Utilities|DoesObjectImplementInterface (.HitActor (Collision|BreakHitResult _array_element_2)) "/Game/Gauntlet/Blueprints/BPI_Enemy.BPI_Enemy_C")
          (if (not (Utilities|Array|ContainsItem (LocalVariables|GetHit%20Actor%20Pool) (.HitActor (Collision|BreakHitResult _array_element_2))))
            (Game|Damage|ApplyDamage (.HitActor (Collision|BreakHitResult _array_element_2)) (LocalVariables|GetDamage) 0 0)
            (Utilities|Array|Add (LocalVariables|GetHit%20Actor%20Pool) (.HitActor (Collision|BreakHitResult _array_element_2))))))
      (Utilities|Array|Clear (LocalVariables|GetHit%20Actor%20Pool)))))

(fn CrossAOE
  (params (Origin :type Vector) (AOE%20Effect :type Niagara%20System%20Object%20Reference) (AOE%20Damage :type Float%20%28double-precision%29) (Ignore :type Actor%20Object%20Reference%20%28by%20ref%29) (AOE%20Size :type Integer) (__WorldContext :type Object%20Object%20Reference))
  (LocalVariables|SetLocation Origin)
  (LocalVariables|SetAOE%20System AOE%20Effect)
  (LocalVariables|SetDamage AOE%20Damage)
  (Utilities|Array|Add (LocalVariables|GetHit%20Actor%20Pool) Ignore)
  (LocalVariables|SetSize AOE%20Size)
  (Utilities|FlowControl|Sequence
    (:then_0
      ;[1 1 1] Horizontal
      (Niagara|SpawnSystematLocation 0 (LocalVariables|GetAOE%20System) (LocalVariables|GetLocation) "0, 0, 0" "0.400000,0.400000,0.400000")
      (bind _outhits (Class|KismetSystemLibrary|BoxTraceMulti 0 (LocalVariables|GetLocation) (LocalVariables|GetLocation) (Math|Vector|MakeVector 1e+01 (* (LocalVariables|GetSize) 1e+02) 1e+01) "0.000000,45.000000,0.000000" "TraceTypeQuery3" false 0 "ForDuration" true))
      (for _array_element _outhits
        (if (Utilities|DoesObjectImplementInterface (.HitActor (Collision|BreakHitResult _array_element)) "/Game/Gauntlet/Blueprints/BPI_Enemy.BPI_Enemy_C")
          (if (not (Utilities|Array|ContainsItem (LocalVariables|GetHit%20Actor%20Pool) (.HitActor (Collision|BreakHitResult _array_element))))
            (Game|Damage|ApplyDamage (.HitActor (Collision|BreakHitResult _array_element)) (LocalVariables|GetDamage) 0 0)
            (Utilities|Array|Add (LocalVariables|GetHit%20Actor%20Pool) (.HitActor (Collision|BreakHitResult _array_element)))))))
    (:then_1
      ;[1 1 1] Vertical
      (Niagara|SpawnSystematLocation 0 (LocalVariables|GetAOE%20System) (LocalVariables|GetLocation) "0, 0, 0" "0.400000,0.400000,0.400000")
      (bind _outhits_2 (Class|KismetSystemLibrary|BoxTraceMulti 0 (LocalVariables|GetLocation) (LocalVariables|GetLocation) (Math|Vector|MakeVector (* (LocalVariables|GetSize) 1e+02) 1e+01 1e+01) "0.000000,45.000000,0.000000" "TraceTypeQuery3" false 0 "ForDuration" true))
      (for _array_element_2 _outhits_2
        (if (Utilities|DoesObjectImplementInterface (.HitActor (Collision|BreakHitResult _array_element_2)) "/Game/Gauntlet/Blueprints/BPI_Enemy.BPI_Enemy_C")
          (if (not (Utilities|Array|ContainsItem (LocalVariables|GetHit%20Actor%20Pool) (.HitActor (Collision|BreakHitResult _array_element_2))))
            (Game|Damage|ApplyDamage (.HitActor (Collision|BreakHitResult _array_element_2)) (LocalVariables|GetDamage) 0 0)
            (Utilities|Array|Add (LocalVariables|GetHit%20Actor%20Pool) (.HitActor (Collision|BreakHitResult _array_element_2))))))
      (Utilities|Array|Clear (LocalVariables|GetHit%20Actor%20Pool)))))