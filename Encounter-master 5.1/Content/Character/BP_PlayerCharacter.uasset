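; Player character for grid-based combat that teleports between neighboring tiles, updating tile occupancy.
; Number keys swap child-actor weapons, with rapid fire spending tick-regenerated mana and secondary attacks sent by message.
; Separate Action events drive an attached weapon, gating abilities on energy, Juiced state and cooldown.
; Damage directly reduces health, as the shield, armor, mod-effect, death and energy-tick chains are disconnected; debug inputs alter fire interval and destroy locked targets.
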(event Custom|MoveNorth
  ;[1 1 1] Player Movement
  (CallFunction|MovetoTile (Variables|/Game/Blueprints/Grid/BP_GridTile.BP_GridTile_C|GetNeighborNorth (Variables|GridManagement|GetCurrentTile)))
  (Animation|PlayAnimMontage "/Game/Character/FemaleCyborg/Animations/Anim_Move_Montage.Anim_Move_Montage" 1.0 "None"))

(event Custom|MoveSouth
  ;[1 1 1] Player Movement
  (CallFunction|MovetoTile (Variables|/Game/Blueprints/Grid/BP_GridTile.BP_GridTile_C|GetNeighborSouth (Variables|GridManagement|GetCurrentTile)))
  (Animation|PlayAnimMontage "/Game/Character/FemaleCyborg/Animations/Anim_Move_Montage.Anim_Move_Montage" 1.0 "None"))

(event Custom|MoveEast
  ;[1 1 1] Player Movement
  (CallFunction|MovetoTile (Variables|/Game/Blueprints/Grid/BP_GridTile.BP_GridTile_C|GetNeighborEast (Variables|GridManagement|GetCurrentTile)))
  (Animation|PlayAnimMontage "/Game/Character/FemaleCyborg/Animations/Anim_Move_Montage.Anim_Move_Montage" 1.0 "None"))

(event Custom|MoveWest
  ;[1 1 1] Player Movement
  (CallFunction|MovetoTile (Variables|/Game/Blueprints/Grid/BP_GridTile.BP_GridTile_C|GetNeighborWest (Variables|GridManagement|GetCurrentTile)))
  (Animation|PlayAnimMontage "/Game/Character/FemaleCyborg/Animations/Anim_Move_Montage.Anim_Move_Montage" 1.0 "None"))

(event Custom|Action:Basic
  ;[1 1 1] Attacks
  (Default|BasicAttack (Variables|References|GetWeaponAttached)))

(event Custom|Action:Cannon
  (bind _weaponattached (Variables|References|GetWeaponAttached))
  (bind _first_ability_cost (Variables|/Game/Character/Attachments/BP_WeaponAttachment_Blaster.BP_WeaponAttachment_Blaster_C|GetFirst%20Ability%20Cost _weaponattached))
  ;[1 1 1] Attacks
  (if (CallFunction|EnoughEnergy&Juiced _first_ability_cost)
    (CallFunction|SpendEnergy _first_ability_cost)
    (Default|FirstAbility (Variables|References|GetWeaponAttached))
    (Variables|Abilities|SetAbilityReady false)
    (Utilities|Time|SetTimerbyFunctionName 0 "AbilityReset" (Variables|Abilities|GetAbilityCooldown))))

(event Custom|EquipWeaponAttachment
  (params (WeaponAttachmentClass :type Actor%20Class%20Reference))
  (bind _weaponattachment (Variables|Default|GetWeaponAttachment))
  ;[1 1 1] Weapon Attachment
  (ChildActorComponent|SetChildActorClass _weaponattachment WeaponAttachmentClass)
  (bind _asbp_weapon_attachment_blaster (Utilities|Casting|CastToBP_WeaponAttachment_Blaster (Variables|/Script/Engine.ChildActorComponent|GetChildActor _weaponattachment)))
  (Variables|References|SetWeaponAttached _asbp_weapon_attachment_blaster))

(event Custom|MoveToTile
  (params (GridTile :type BP%20Grid%20Tile%20Object%20Reference))
  ;[1 1 1] Move the Chracter to the selected tile
  (Utilities|IsValid GridTile
    (:Is%20Valid
      (if (Utilities|Enum|NotEqual(Enum) (Variables|/Game/Blueprints/Grid/BP_GridTile.BP_GridTile_C|GetGridType GridTile) "NewEnumerator1")
        (Rendering|SetVisibility (Variables|Character|GetMesh) false true)
        (Transformation|SetWorldLocation (Variables|Collision|GetCapsuleComponent) (Variables|/Game/Blueprints/Grid/BP_GridTile.BP_GridTile_C|GetGridWorldLocation GridTile) false false)
        (Default|EmptyTile (Variables|GridManagement|GetCurrentTile))
        (bind _output_get (Variables|GridManagement|SetCurrentTile GridTile))
        (Default|OccupyTile _output_get self)
        (Audio|SpawnSound2D "/Game/Audio/SoundEffects/S_MovingTIle.S_MovingTIle" 1.0 1.0 0.0 0)
        (Utilities|FlowControl|Delay 0.1)
        (Rendering|SetVisibility (Variables|Character|GetMesh) true true)))))

(event Custom|Action:Second
  (bind _weaponattached (Variables|References|GetWeaponAttached))
  (bind _second_ability_cost (Variables|/Game/Character/Attachments/BP_WeaponAttachment_Blaster.BP_WeaponAttachment_Blaster_C|GetSecond%20Ability%20Cost _weaponattached))
  ;[1 1 1] Attacks
  (if (CallFunction|EnoughEnergy&Juiced _second_ability_cost)
    (CallFunction|SpendEnergy _second_ability_cost)
    (Default|SecondAbility (Variables|References|GetWeaponAttached))
    (Variables|Abilities|SetAbilityReady false)
    (Utilities|Time|SetTimerbyFunctionName 0 "AbilityReset" (Variables|Abilities|GetAbilityCooldown))))

(event Input|EnhancedActionEvents|EnhancedInputActionChargeToFire
  (params (ActionValue :type Boolean) (ElapsedSeconds :type Float%20%28double-precision%29) (TriggeredSeconds :type Float%20%28double-precision%29) (InputAction :type Input%20Action%20Object%20Reference :default "/Game/Gauntlet/Weapons/Input/ChargeToFire.ChargeToFire")))

(event Input|EnhancedActionEvents|EnhancedInputActionRapidFire
  (params (ActionValue :type Boolean) (ElapsedSeconds :type Float%20%28double-precision%29) (TriggeredSeconds :type Float%20%28double-precision%29) (InputAction :type Input%20Action%20Object%20Reference :default "/Game/Gauntlet/Weapons/Input/RapidFire.RapidFire"))
  (:Triggered
    (bind _asbp_weapon_master (Utilities|Casting|CastToBP_Weapon_Master (Variables|/Script/Engine.ChildActorComponent|GetChildActor (Variables|Default|GetWeaponAttachment))))
    (if (<= (Variables|/Game/Gauntlet/Weapons/BP_Weapon_Master.BP_Weapon_Master_C|GetManaCost _asbp_weapon_master) (Variables|Default|GetMana))
      (Class|BPIWeapons|PrimaryAttack(Message) (Variables|/Script/Engine.ChildActorComponent|GetChildActor (Variables|Default|GetWeaponAttachment)) 0.0 0 false)
      (Variables|Default|SetMana (- (Variables|Default|GetMana) (Variables|/Game/Gauntlet/Weapons/BP_Weapon_Master.BP_Weapon_Master_C|GetManaCost _asbp_weapon_master)))
      (else
        (Development|PrintString "YOU HAVE NO MANAAAAA")))))

(event Input|EnhancedActionEvents|EnhancedInputActionChargeToFire
  (params (ActionValue :type Boolean) (ElapsedSeconds :type Float%20%28double-precision%29) (TriggeredSeconds :type Float%20%28double-precision%29) (InputAction :type Input%20Action%20Object%20Reference :default "/Game/Gauntlet/Weapons/Input/ChargeToFire.ChargeToFire")))

(event EventBeginPlay
  (bind _returnvalue (Game|GetPlayerController 0))
  (bind _returnvalue_2 (PlayerController|LocalPlayerSubsystems|GetEnhancedInputLocalPlayerSubsystem _returnvalue))
  ;[1 1 1] Event BeginPlay
  (Utilities|IsValid _returnvalue_2
    (:Is%20Valid
      (Input|AddMappingContext _returnvalue_2 (Variables|Default|GetMapping%20Context) 0 "(bIgnoreAllPressedKeysUntilRelease=True,bForceImmediately=False)")
      (Utilities|CastReferences)
      (CallFunction|SetStartingTile)
      (bind _returnvalue_3 (UserInterface|CreateWidget "/Game/Gauntlet/Widgets/PlayerCanvas.PlayerCanvas_C"))
      (bind _output_get (Variables|Default|SetPlayerCanvas _returnvalue_3))
      (UserInterface|Viewport|AddtoViewport _output_get 0))))

(event Game|Damage|EventAnyDamage
  (params (Damage :type Float%20%28single-precision%29) (DamageType :type Damage%20Type%20Object%20Reference) (InstigatedBy :type Controller%20Object%20Reference) (DamageCauser :type Actor%20Object%20Reference))
  (CallFunction|DamageHealth Damage))

(event EventTick
  (params (DeltaSeconds :type Float%20%28single-precision%29))
  (if (>= (Variables|Default|GetMana) 1e+02)
    (Variables|Default|SetMana 1e+02)
    (else
      (Variables|Default|SetMana (+ (Variables|Default|GetMana) 0.05)))))

(event Input|ActionEvents|InputActionKillLockedTarget
  (params (Key :type Key%20Structure :default "None"))
  (:Pressed
    (bind _asbp_weapon_master (Utilities|Casting|CastToBP_Weapon_Master (Variables|/Script/Engine.ChildActorComponent|GetChildActor (Variables|Default|GetWeaponAttachment))))
    (Actor|DestroyActor (Variables|/Game/Gauntlet/Weapons/BP_Weapon_Master.BP_Weapon_Master_C|GetMissile%20Target _asbp_weapon_master))
    (Default|LockedTargetDied _asbp_weapon_master)))

(event Input|ActionEvents|InputActionEquipWeapon1
  (params (Key :type Key%20Structure :default "None"))
  (:Pressed
    (ChildActorComponent|SetChildActorClass (Variables|Default|GetWeaponAttachment) "/Game/Gauntlet/Weapons/WeaponCache/BPC_Blaster.BPC_Blaster_C")))

(event Input|ActionEvents|InputActionSecondaryAbility
  (params (Key :type Key%20Structure :default "None"))
  (:Pressed
    (Class|BPIWeapons|SecondaryAbility(Message) (Variables|/Script/Engine.ChildActorComponent|GetChildActor (Variables|Default|GetWeaponAttachment)))))

(event Input|ActionEvents|InputActionPrimaryAttack
  (params (Key :type Key%20Structure :default "None")))

(event Input|ActionEvents|InputActionEquipWeapon2
  (params (Key :type Key%20Structure :default "None"))
  (:Pressed
    (ChildActorComponent|SetChildActorClass (Variables|Default|GetWeaponAttachment) "/Game/Gauntlet/Weapons/WeaponCache/BPC_Shotgun.BPC_Shotgun_C")))

(event Input|ActionEvents|InputActionEquipWeapon3
  (params (Key :type Key%20Structure :default "None"))
  (:Pressed
    (ChildActorComponent|SetChildActorClass (Variables|Default|GetWeaponAttachment) "/Game/Gauntlet/Weapons/WeaponCache/BPC_GrenadeLauncher.BPC_GrenadeLauncher_C")))

(event Input|ActionEvents|InputActionEquipWeapon4
  (params (Key :type Key%20Structure :default "None"))
  (:Pressed
    (ChildActorComponent|SetChildActorClass (Variables|Default|GetWeaponAttachment) "/Game/Gauntlet/Weapons/WeaponCache/BPC_MissileLauncher.BPC_MissileLauncher_C")))

(event Input|ActionEvents|InputActionDamagePlayer
  (params (Key :type Key%20Structure :default "None")))

(event Input|ActionEvents|InputActionSecretBUtton
  (params (Key :type Key%20Structure :default "None"))
  (:Pressed
    (for _array_element (Variables|/Script/EnhancedInput.InputMappingContext|GetMappings (Variables|Default|GetMapping%20Context))
      (if (== (.Action (Utilities|Struct|BreakEnhancedActionKeyMapping _array_element)) "/Game/Gauntlet/Weapons/Input/ChargeToFire.ChargeToFire")
        (for _array_element_2 (Variables|/Script/EnhancedInput.InputAction|GetTriggers (.Action (Utilities|Struct|BreakEnhancedActionKeyMapping _array_element)))
          (bind _aspulse (Utilities|Casting|CastToInputTriggerPulse _array_element_2))
          (Variables|/Script/EnhancedInput.InputTriggerPulse|SetInterval _aspulse 0.1))))))

(fn ConstructionScript)

(fn SetStartingTile
  (bind _output_get (Variables|GridManagement|SetCurrentTile (Utilities|Array|Get(acopy) (Variables|/Game/Blueprints/Grid/BP_GridManager.BP_GridManager_C|GetGridArray (Variables|GridManagement|GetGridManager)) (Variables|GridManagement|GetStartingTile))))
  (Transformation|SetWorldLocation (Variables|Collision|GetCapsuleComponent) (Variables|/Game/Blueprints/Grid/BP_GridTile.BP_GridTile_C|GetGridWorldLocation _output_get) false false)
  (Default|OccupyTile (Variables|GridManagement|GetCurrentTile) self))

(fn SpendEnergy
  (params (Amount :type Float%20%28double-precision%29))
  (Variables|PlayerResources|SetCurrentEnergyPoints (- (Variables|PlayerResources|GetCurrentEnergyPoints) Amount)))

(fn GainEnergy
  (params (Amount :type Float%20%28double-precision%29))
  (if (< (Variables|PlayerResources|GetCurrentEnergyPoints) (Variables|PlayerResources|GetMaxEnergyPoints))
    (bind _output_get (Variables|PlayerResources|SetCurrentEnergyPoints (+ Amount (Variables|PlayerResources|GetCurrentEnergyPoints))))
    (if (>= _output_get (Variables|PlayerResources|GetMaxEnergyPoints))
      (Variables|PlayerResources|SetCurrentEnergyPoints (Variables|PlayerResources|GetMaxEnergyPoints)))))

(fn ShieldDamageReduction
  (params (Damage%20In :type Float%20%28double-precision%29))
  (bind _output_get (LocalVariables|SetDamageOut (CallFunction|ReduceFloatby% Damage%20In (Variables|Abilities|GetShieldReduction%25))))
  (return _output_get))

(fn ReduceFloatby%
  (params (Value :type Float%20%28double-precision%29) (Percentage :type Float%20%28double-precision%29))
  (return (- Value (* Value (/ Percentage 1e+02)))))

(fn KillPlayer
  (bind _returnvalue (Game|GetPlayerController 0))
  (Variables|PlayerResources|SetImDead true)
  (bind _returnvalue_2 (UserInterface|CreateWidget "/Game/UserInterface/WBP_GameOver.WBP_GameOver_C"))
  (UserInterface|Viewport|AddtoViewport _returnvalue_2 0)
  (Input|SetInputModeUIOnly _returnvalue _returnvalue_2 "DoNotLock" false)
  (Variables|/Script/Engine.PlayerController|SetbShowMouseCursor _returnvalue true))

(fn IsPlayerAlive?
  (return (not (Variables|PlayerResources|GetImDead))))

(fn GoEquipMode
  (bind _returnvalue (Game|GetPlayerController 0))
  (if (not (Variables|Abilities|GetEquipMode))
    (Input|SetInputModeGameandUI _returnvalue 0 "DoNotLock" true false)
    (Variables|/Script/Engine.PlayerController|SetbShowMouseCursor _returnvalue true)
    (Game|SetGamePaused true)
    (Default|RefreshModSelection (Variables|References|GetModsHUD))
    (Variables|Abilities|SetEquipMode true)
    (else
      (Default|SetInputMode (Variables|References|GetControllerRef) false)
      (Game|SetGamePaused false)
      (Default|HideInventory (Variables|References|GetModsHUD))
      (Variables|Abilities|SetEquipMode false))))

(fn DamageReduction
  (params (Damage%20In :type Float%20%28double-precision%29))
  (return (CallFunction|ReduceFloatby% Damage%20In (Variables|Abilities|GetArmorReduction%25))))

(fn ResetCharacter
  (Variables|PlayerResources|SetCurrentEnergyPoints 0.0))

(fn DestroyComponent
  (params (ModComponent :type BP%20Mod%20Master%20Object%20Reference)))

(fn SpawnDamageEffect
  (Niagara|SpawnSystematLocation "/Game/Sci-Fi_Starter_VFX_Pack_Niagara/Niagara/Blood/NS_Blood_Splat_2D_2.NS_Blood_Splat_2D_2" (+ (Variables|/Game/Blueprints/Grid/BP_GridTile.BP_GridTile_C|GetGridWorldLocation (Variables|GridManagement|GetCurrentTile)) "0,0,100.000000"))
  (Animation|PlayAnimMontage "/Game/Character/FemaleCyborg/Animations/Anim_TakeDamage_Montage.Anim_TakeDamage_Montage" 1.0 "None")
  (bind _returnvalue (Actor|GetActorOfClass "/Game/Blueprints/BP_Camera.BP_Camera_C"))
  (Default|PlayerCameraShake _returnvalue))

(fn EnoughEnergy&Juiced
  (params (EnergyCost :type Float%20%28double-precision%29))
  (return (Math|Boolean|ANDBoolean (>= (Variables|PlayerResources|GetCurrentEnergyPoints) EnergyCost) (Variables|PlayerResources|GetJuiced) (Variables|Abilities|GetAbilityReady))))

(fn GetFloat%
  (params (Value :type Float%20%28double-precision%29) (%25 :type Float%20%28double-precision%29))
  (return (* Value (/ %25 1e+02))))

(fn CheckThorns
  (params (Attacker :type Actor%20Object%20Reference) (Damage :type Float%20%28double-precision%29))
  (if (Variables|ModBools|GetThorns)
    (Game|Damage|ApplyDamage Attacker (CallFunction|GetFloat% Damage (Variables|/Game/Character/ModInventory/ModActors/BP_Mod_Kinetic_Thorns.BP_Mod_Kinetic_Thorns_C|GetReturn%25 (Actor|GetComponentbyClass "/Game/Character/ModInventory/ModActors/BP_Mod_Kinetic_Thorns.BP_Mod_Kinetic_Thorns_C"))) 0 0))
  (return))

(fn DamageShield
  (params (Amount :type Float%20%28double-precision%29))
  (Default|ShowDamageTaken (Variables|References|GetHPWidget) Amount)
  (bind _output_get (Variables|PlayerResources|SetCurrentShield (- (Variables|PlayerResources|GetCurrentShield) Amount)))
  (CallFunction|SpawnShieldDamageEffect)
  (return _output_get))

(fn SpawnShieldDamageEffect
  (Niagara|SpawnSystematLocation "/Game/Sci-Fi_Starter_VFX_Pack_Niagara/Niagara/Explosion/NS_Explosion_Small_2.NS_Explosion_Small_2" (+ (Variables|/Game/Blueprints/Grid/BP_GridTile.BP_GridTile_C|GetGridWorldLocation (Variables|GridManagement|GetCurrentTile)) "0,0,100.000000"))
  (bind _returnvalue (Actor|GetActorOfClass "/Game/Blueprints/BP_Camera.BP_Camera_C"))
  (Default|PlayerCameraShake _returnvalue))

(fn DamageHealth
  (params (Amount :type Float%20%28double-precision%29))
  (Default|ShowDamageTaken (Variables|References|GetHPWidget) Amount)
  (bind _output_get (Variables|PlayerResources|SetCurrentHP (- (Variables|PlayerResources|GetCurrentHP) Amount)))
  (CallFunction|SpawnDamageEffect)
  (return _output_get))

(fn RegenerateShield
  (if (not (Variables|PlayerResources|GetShieldUp))
    (bind _output_get (Variables|PlayerResources|SetCurrentShield (+ (Variables|PlayerResources|GetShieldRegeneration) (Variables|PlayerResources|GetCurrentShield))))
    (if (>= _output_get (Variables|PlayerResources|GetMaxShield))
      (Variables|PlayerResources|SetCurrentShield (Variables|PlayerResources|GetMaxShield))
      (Variables|PlayerResources|SetShieldUp true))))

(fn EnergySystem
  (if (Variables|PlayerResources|GetJuiced)
    (CallFunction|SpendEnergy 0.1)
    (if (<= (Variables|PlayerResources|GetCurrentEnergyPoints) 0.0)
      (Variables|PlayerResources|SetCurrentEnergyPoints 0.0)
      (Variables|PlayerResources|SetJuiced false))
    (else
      (CallFunction|GainEnergy 0.2))))

(fn GainHealth
  (params (Amount :type Float%20%28double-precision%29))
  (Variables|PlayerResources|SetCurrentHP (+ Amount (Variables|PlayerResources|GetCurrentHP)))
  (return))

(fn CheckCauterize
  (params (Amount :type Float%20%28double-precision%29))
  (bind _returnvalue (Actor|GetComponentbyClass "/Game/Character/ModInventory/ModActors/BP_Mod_Solar_Cauterize.BP_Mod_Solar_Cauterize_C"))
  (if (Variables|ModBools|GetCauterize)
    (if (< (Math|Random|RandomIntegerinRange 0 100) (Variables|/Game/Character/ModInventory/ModActors/BP_Mod_Solar_Cauterize.BP_Mod_Solar_Cauterize_C|GetChance%25 _returnvalue))
      (CallFunction|GainHealth (* Amount (/ (Variables|/Game/Character/ModInventory/ModActors/BP_Mod_Solar_Cauterize.BP_Mod_Solar_Cauterize_C|GetHeal%25 _returnvalue) 1e+02))))))

(fn AbilityReset
  (Variables|Abilities|SetAbilityReady true))

(fn GetPlayerTile
  (return (Variables|GridManagement|GetCurrentTile)))

(fn SetChargingAttack
  (params (IsChargingAttack :type Boolean)))