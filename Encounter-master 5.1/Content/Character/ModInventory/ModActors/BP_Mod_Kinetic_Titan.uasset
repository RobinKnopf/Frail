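; BP_Mod_Kinetic_Titan is an equippable character mod that raises health by a flat amount based on its rarity.
; On Equip, SetModifier picks the bonus for Common, Rare or Epic, which is then added to both MaxHP and CurrentHP on CharacterRef.
; Unequip subtracts the bonus from MaxHP only, leaving CurrentHP unchanged and unclamped.
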(event EventBeginPlay
  (|CallParentFunction))

(event EventEquip
  (params (Rarity :type E_ModRarity%20Enum :default "NewEnumerator0"))
  (bind _characterref (Variables|Default|GetCharacterRef))
  (CallFunction|SetModifier Rarity)
  (Variables|/Game/Character/BP_PlayerCharacter.BP_PlayerCharacter_C|SetMaxHP _characterref (+ (Variables|Default|GetModifier) (Variables|/Game/Character/BP_PlayerCharacter.BP_PlayerCharacter_C|GetMaxHP _characterref)))
  (Variables|/Game/Character/BP_PlayerCharacter.BP_PlayerCharacter_C|SetCurrentHP _characterref (+ (Variables|Default|GetModifier) (Variables|/Game/Character/BP_PlayerCharacter.BP_PlayerCharacter_C|GetCurrentHP _characterref))))

(event EventUnequip
  (bind _characterref (Variables|Default|GetCharacterRef))
  (Variables|/Game/Character/BP_PlayerCharacter.BP_PlayerCharacter_C|SetMaxHP _characterref (- (Variables|/Game/Character/BP_PlayerCharacter.BP_PlayerCharacter_C|GetMaxHP _characterref) (Variables|Default|GetModifier))))

(fn SetModifier
  (params (Rarity :type E_ModRarity%20Enum :default "NewEnumerator0"))
  (switch Utilities|FlowControl|Switch|SwitchonE_ModRarity Rarity
    (:NewEnumerator0
      (Variables|Default|SetModifier 25.0))
    (:NewEnumerator1
      (Variables|Default|SetModifier 5e+01))
    (:NewEnumerator2
      (Variables|Default|SetModifier 75.0))))