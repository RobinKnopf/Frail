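; BP_Mod_Arc_Juice is an equippable character mod that raises the owning character's maximum energy points.
; On Equip, SetModifier picks a flat bonus from the item's rarity (Common, Rare or Epic) and adds it to the character's MaxEnergyPoints.
; Unequip subtracts the stored Modifier to undo the bonus.
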(event EventBeginPlay
  (|CallParentFunction) ; This node is disabled and will not be called.\nDrag off pins to build functionality.
)

(event EventEquip
  (params (Rarity :type E_ModRarity%20Enum :default "NewEnumerator0"))
  (bind _characterref (Variables|Default|GetCharacterRef))
  (CallFunction|SetModifier Rarity)
  (Variables|/Game/Character/BP_PlayerCharacter.BP_PlayerCharacter_C|SetMaxEnergyPoints _characterref (+ (Variables|/Game/Character/BP_PlayerCharacter.BP_PlayerCharacter_C|GetMaxEnergyPoints _characterref) (Variables|Default|GetModifier))))

(event EventUnequip
  (bind _characterref (Variables|Default|GetCharacterRef))
  (Variables|/Game/Character/BP_PlayerCharacter.BP_PlayerCharacter_C|SetMaxEnergyPoints _characterref (- (Variables|/Game/Character/BP_PlayerCharacter.BP_PlayerCharacter_C|GetMaxEnergyPoints _characterref) (Variables|Default|GetModifier))))

(fn SetModifier
  (params (Rarity :type E_ModRarity%20Enum :default "NewEnumerator0"))
  (switch Utilities|FlowControl|Switch|SwitchonE_ModRarity Rarity
    (:NewEnumerator0
      (Variables|Default|SetModifier 25.0))
    (:NewEnumerator1
      (Variables|Default|SetModifier 5e+01))
    (:NewEnumerator2
      (Variables|Default|SetModifier 1e+02)))
  (return))