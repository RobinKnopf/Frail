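; Solar Cauterize mod actor for the character mod inventory, which toggles the Cauterize ability on its owning character.
; Equip maps the mod's rarity (Common, Rare or Epic) to a rising Chance value, then sets the Cauterize flag on CharacterRef.
; Unequip clears the flag and zeroes Chance.
; The actor only holds this state; the Cauterize effect and the Chance roll are not implemented here.
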(event EventBeginPlay
  (|CallParentFunction))

(event EventEquip
  (params (Rarity :type E_ModRarity%20Enum :default "NewEnumerator0"))
  (CallFunction|SetRarity Rarity)
  (Variables|/Game/Character/BP_PlayerCharacter.BP_PlayerCharacter_C|SetCauterize (Variables|Default|GetCharacterRef) true))

(event EventUnequip
  (Variables|/Game/Character/BP_PlayerCharacter.BP_PlayerCharacter_C|SetCauterize (Variables|Default|GetCharacterRef) false)
  (Variables|Default|SetChance%25 0))

(fn SetRarity
  (params (Selection :type E_ModRarity%20Enum :default "NewEnumerator0"))
  (switch Utilities|FlowControl|Switch|SwitchonE_ModRarity Selection
    (:NewEnumerator0
      (Variables|Default|SetChance%25 20))
    (:NewEnumerator1
      (Variables|Default|SetChance%25 40))
    (:NewEnumerator2
      (Variables|Default|SetChance%25 60)))
  (return))