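; BP_Mod_Solar_Tempering is an equippable mod actor that sets the character's ShieldReduction while equipped.
; On Equip, SetShieldPercentage maps the mod's rarity (Common, Rare or Epic) to a rising percentage, which is written directly to the referenced character.
; Unequip resets ShieldReduction to zero rather than restoring any earlier value.
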(event EventBeginPlay
  (|CallParentFunction) ; This node is disabled and will not be called.\nDrag off pins to build functionality.
)

(event EventEquip
  (params (Rarity :type E_ModRarity%20Enum :default "NewEnumerator0"))
  (bind _reduction_ (CallFunction|SetShieldPercentage Rarity))
  (Variables|/Game/Character/BP_PlayerCharacter.BP_PlayerCharacter_C|SetShieldReduction%25 (Variables|Default|GetCharacterRef) _reduction_))

(event EventUnequip
  (Variables|/Game/Character/BP_PlayerCharacter.BP_PlayerCharacter_C|SetShieldReduction%25 (Variables|Default|GetCharacterRef) 0.0))

(fn SetShieldPercentage
  (params (Rarity :type E_ModRarity%20Enum :default "NewEnumerator0"))
  (switch Utilities|FlowControl|Switch|SwitchonE_ModRarity Rarity
    (:NewEnumerator0
      (LocalVariables|SetPercentage 1e+01))
    (:NewEnumerator1
      (LocalVariables|SetPercentage 2e+01))
    (:NewEnumerator2
      (LocalVariables|SetPercentage 3e+01)))
  (return (LocalVariables|GetPercentage)))