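; BP_Mod_Kinetic_Explosive is an equippable kinetic mod that turns on an explosive effect, with strength set by rarity.
; Equip calls SetRarity, which maps Common, Rare or Epic to a rising ExplosiveValue, then sets the Explosive flag.
; Unequip clears the flag and zeroes the value.
; The file only maintains this state; it contains no explosion logic.
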(event EventBeginPlay
  (|CallParentFunction))

(event EventEquip
  (params (Rarity :type E_ModRarity%20Enum :default "NewEnumerator0"))
  (CallFunction|SetRarity Rarity)
  (Variables|Default|SetExplosive true))

(event EventUnequip
  (Variables|Default|SetExplosive false)
  (Variables|Default|SetExplosiveValue 0.0))

(fn SetRarity
  (params (Selection :type E_ModRarity%20Enum :default "NewEnumerator0"))
  (switch Utilities|FlowControl|Switch|SwitchonE_ModRarity Selection
    (:NewEnumerator0
      (Variables|Default|SetExplosiveValue 1e+01))
    (:NewEnumerator1
      (Variables|Default|SetExplosiveValue 2e+01))
    (:NewEnumerator2
      (Variables|Default|SetExplosiveValue 3e+01)))
  (return))