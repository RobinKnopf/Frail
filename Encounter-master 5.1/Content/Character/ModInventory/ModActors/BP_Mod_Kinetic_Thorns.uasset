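; BP_Mod_Kinetic_Thorns is a mod actor that grants the Thorns effect to its character while equipped.
; Equip sets the Thorns flag on CharacterRef and picks a Return value that rises with rarity across Common, Rare and Epic.
; Unequip clears the flag and zeroes Return; the file only sets this state and does not apply the effect itself.
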(event EventBeginPlay
  (|CallParentFunction))

(event EventEquip
  (params (Rarity :type E_ModRarity%20Enum :default "NewEnumerator0"))
  (Variables|/Game/Character/BP_PlayerCharacter.BP_PlayerCharacter_C|SetThorns (Variables|Default|GetCharacterRef) true)
  (switch Utilities|FlowControl|Switch|SwitchonE_ModRarity Rarity
    (:NewEnumerator0
      (Variables|Default|SetReturn%25 5.0))
    (:NewEnumerator1
      (Variables|Default|SetReturn%25 1e+01))
    (:NewEnumerator2
      (Variables|Default|SetReturn%25 2e+01))))

(event EventUnequip
  (Variables|/Game/Character/BP_PlayerCharacter.BP_PlayerCharacter_C|SetThorns (Variables|Default|GetCharacterRef) false)
  (Variables|Default|SetReturn%25 0.0))