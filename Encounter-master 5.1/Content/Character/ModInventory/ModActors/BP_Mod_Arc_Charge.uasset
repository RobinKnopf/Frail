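; BP_Mod_Arc_Charge is an equippable character mod that boosts shield regeneration.
; On Equip, SetModifier maps the mod's rarity to a percentage, which is added on top of the character's current ShieldRegeneration.
; Unequip resets ShieldRegeneration to a hardcoded base value instead of reversing the applied bonus.
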(event EventBeginPlay
  (|CallParentFunction) ; This node is disabled and will not be called.\nDrag off pins to build functionality.
)

(event EventEquip
  (params (Rarity :type E_ModRarity%20Enum :default "NewEnumerator0"))
  (bind _characterref (Variables|Default|GetCharacterRef))
  (CallFunction|SetModifier Rarity)
  (Variables|/Game/Character/BP_PlayerCharacter.BP_PlayerCharacter_C|SetShieldRegeneration (Variables|Default|GetCharacterRef) (+ (Variables|/Game/Character/BP_PlayerCharacter.BP_PlayerCharacter_C|GetShieldRegeneration _characterref) (* (Variables|/Game/Character/BP_PlayerCharacter.BP_PlayerCharacter_C|GetShieldRegeneration _characterref) (/ (Variables|Default|GetModifier) 1e+02)))))

(event EventUnequip
  (Variables|/Game/Character/BP_PlayerCharacter.BP_PlayerCharacter_C|SetShieldRegeneration (Variables|Default|GetCharacterRef) 0.05))

(fn SetModifier
  (params (Rarity :type E_ModRarity%20Enum :default "NewEnumerator0"))
  (switch Utilities|FlowControl|Switch|SwitchonE_ModRarity Rarity
    (:NewEnumerator0
      (Variables|Default|SetModifier 1e+01))
    (:NewEnumerator1
      (Variables|Default|SetModifier 2e+01))
    (:NewEnumerator2
      (Variables|Default|SetModifier 3e+01)))
  (return))