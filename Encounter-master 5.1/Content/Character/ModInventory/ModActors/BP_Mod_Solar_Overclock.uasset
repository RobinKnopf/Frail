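; BP_Mod_Solar_Overclock is an equippable mod actor that changes the attack speed of the character's attached weapon.
; On Equip, SetRarity maps the Common, Rare or Epic rarity to a modifier value, which is written to the weapon's AttackSpeedModifier.
; On Unequip, it resets that modifier to zero, overwriting the value directly rather than subtracting its own contribution.
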(event EventBeginPlay
  (|CallParentFunction))

(event EventEquip
  (params (Rarity :type E_ModRarity%20Enum :default "NewEnumerator0"))
  (bind _value (CallFunction|SetRarity Rarity))
  (Variables|/Game/Character/Attachments/BP_WeaponAttachment_Blaster.BP_WeaponAttachment_Blaster_C|SetAttackSpeedModifier (Variables|/Game/Character/BP_PlayerCharacter.BP_PlayerCharacter_C|GetWeaponAttached (Variables|Default|GetCharacterRef)) _value))

(event EventUnequip
  (Variables|/Game/Character/Attachments/BP_WeaponAttachment_Blaster.BP_WeaponAttachment_Blaster_C|SetAttackSpeedModifier (Variables|/Game/Character/BP_PlayerCharacter.BP_PlayerCharacter_C|GetWeaponAttached (Variables|Default|GetCharacterRef)) 0.0))

(fn SetRarity
  (params (Selection :type E_ModRarity%20Enum :default "NewEnumerator0"))
  (switch Utilities|FlowControl|Switch|SwitchonE_ModRarity Selection
    (:NewEnumerator0
      (LocalVariables|SetModifier 1e+01))
    (:NewEnumerator1
      (LocalVariables|SetModifier 15.0))
    (:NewEnumerator2
      (LocalVariables|SetModifier 2e+01)))
  (return (LocalVariables|GetModifier)))