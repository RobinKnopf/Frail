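; Kinetic Ironclad mod actor that modifies the owning character's ArmorReduction while equipped.
; On Equip, a helper function maps the mod's rarity (Common, Rare or Epic) to a fixed percentage, which overwrites the character's ArmorReduction rather than adding to it.
; On Unequip, ArmorReduction is set back to DefaultValue.
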(event EventBeginPlay
  (|CallParentFunction) ; This node is disabled and will not be called.\nDrag off pins to build functionality.
)

(event EventEquip
  (params (Rarity :type E_ModRarity%20Enum :default "NewEnumerator0"))
  (bind _reduction_ (CallFunction|SetArmorReduction% Rarity))
  (Variables|/Game/Character/BP_PlayerCharacter.BP_PlayerCharacter_C|SetArmorReduction%25 (Variables|Default|GetCharacterRef) _reduction_))

(event EventUnequip
  (Variables|/Game/Character/BP_PlayerCharacter.BP_PlayerCharacter_C|SetArmorReduction%25 (Variables|Default|GetCharacterRef) (Variables|Default|GetDefaultValue)))

(fn SetArmorReduction%
  (params (Rarity :type E_ModRarity%20Enum :default "NewEnumerator0"))
  (switch Utilities|FlowControl|Switch|SwitchonE_ModRarity Rarity
    (:NewEnumerator0
      (LocalVariables|SetPercentage 5.0))
    (:NewEnumerator1
      (LocalVariables|SetPercentage 1e+01))
    (:NewEnumerator2
      (LocalVariables|SetPercentage 15.0)))
  (return (LocalVariables|GetPercentage)))