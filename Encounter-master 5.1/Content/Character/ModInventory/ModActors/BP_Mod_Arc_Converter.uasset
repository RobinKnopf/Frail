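; Arc Converter mod actor that converts hits taken on the player's raised shield into energy.
; On BeginPlay it binds to the character's on-hit effect event, granting a set energy amount whenever that fires with the shield up.
; Equip sets that amount from the mod's rarity and turns on the character's on-hit effects flag, which Unequip turns off.
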(event Custom|OnHitEffect
  (bind _characterref (Variables|Default|GetCharacterRef))
  (if (Variables|/Game/Character/BP_PlayerCharacter.BP_PlayerCharacter_C|GetShieldUp _characterref)
    (Default|GainEnergy _characterref (Variables|Default|GetAbsorbedEnergy))))

(event EventBeginPlay
  (|CallParentFunction)
  (EventDispatchers|AssignOnHitEffect (Variables|Default|GetCharacterRef) (delegate Custom|OnHitEffect)))

(event EventEquip
  (params (Rarity :type E_ModRarity%20Enum :default "NewEnumerator0"))
  (CallFunction|SetAmounttoAbsorb Rarity)
  (Variables|/Game/Character/BP_PlayerCharacter.BP_PlayerCharacter_C|SetOnHitEffectsActive (Variables|Default|GetCharacterRef) true))

(event EventUnequip
  (Variables|/Game/Character/BP_PlayerCharacter.BP_PlayerCharacter_C|SetOnHitEffectsActive (Variables|Default|GetCharacterRef) false))

(fn SetAmounttoAbsorb
  (params (Rarity :type E_ModRarity%20Enum :default "NewEnumerator0"))
  (switch Utilities|FlowControl|Switch|SwitchonE_ModRarity Rarity
    (:NewEnumerator0
      (Variables|Default|SetAbsorbedEnergy 1e+01))
    (:NewEnumerator1
      (Variables|Default|SetAbsorbedEnergy 3e+01))
    (:NewEnumerator2
      (Variables|Default|SetAbsorbedEnergy 5e+01))))