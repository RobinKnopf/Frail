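; BP_Attack_Sweep is a one-shot sweep attack actor for the player on a tile grid.
; On BeginPlay it targets the tile east of the player plus that tile's north and south neighbors.
; It spawns a BP_Cone above each tile, damages occupants tagged Enemy, then destroys itself.
; The direction is fixed east, and GetPlayerTile and SetChargingAttack are empty stubs.
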(event EventBeginPlay
  (bind _playertile (Class|BPIAttackSystem|GetPlayerTile(Message) (Game|GetPlayerCharacter 0)))
  (bind _output_get (Variables|Default|SetCurrentTile (Variables|/Game/Blueprints/Grid/BP_GridTile.BP_GridTile_C|GetNeighborEast _playertile)))
  (CallFunction|GetTargetTiles _output_get)
  (CallFunction|SpawnEffect)
  (CallFunction|CheckDamage)
  (Actor|DestroyActor))

(fn ConstructionScript)

(fn CheckDamage
  (for _array_element (Variables|Default|GetAbilityAOE)
    (Utilities|IsValid (Variables|/Game/Blueprints/Grid/BP_GridTile.BP_GridTile_C|GetOccupyingActor _array_element)
      (:Is%20Valid
        (if (Actor|ActorHasTag (Variables|/Game/Blueprints/Grid/BP_GridTile.BP_GridTile_C|GetOccupyingActor _array_element) "Enemy")
          (Game|Damage|ApplyDamage (Variables|/Game/Blueprints/Grid/BP_GridTile.BP_GridTile_C|GetOccupyingActor _array_element) (Variables|Default|GetBase%20Damage) 0 0))))))

(fn GetTargetTiles
  (params (CurrentTile :type BP%20Grid%20Tile%20Object%20Reference))
  (Variables|Default|SetAbilityAOE (Utilities|Array|MakeArray CurrentTile (Variables|/Game/Blueprints/Grid/BP_GridTile.BP_GridTile_C|GetNeighborNorth CurrentTile) (Variables|/Game/Blueprints/Grid/BP_GridTile.BP_GridTile_C|GetNeighborSouth CurrentTile))))

(fn SpawnEffect
  (for _array_element (Variables|Default|GetAbilityAOE)
    (Game|SpawnActorfromClass "/Game/Enemies/TempAssets/BP_COne.BP_Cone_C" (Math|Transform|MakeTransform (+ (Variables|/Game/Blueprints/Grid/BP_GridTile.BP_GridTile_C|GetGridWorldLocation _array_element) "0, 0,100.000000") "0, 0, 0" "1,1,1") "Undefined" 0 0)))

(fn GetPlayerTile
  (return 0))

(fn SetChargingAttack
  (params (IsChargingAttack :type Boolean))
  (return false))