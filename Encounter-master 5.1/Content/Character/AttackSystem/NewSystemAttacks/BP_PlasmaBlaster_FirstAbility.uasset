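; Plasma blaster first ability: a short-lived attack actor that fires in a straight line east across the tile grid from the player's tile.
; On BeginPlay it plays the shot sound and follows east neighbor links up to a fixed range to build its area of effect.
; Enemy-tagged occupants of those tiles take damage with a Niagara impact effect, then the actor destroys itself after a brief delay.
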(event EventBeginPlay
  (bind _playertile (Class|BPIAttackSystem|GetPlayerTile(Message) (Game|GetPlayerCharacter 0)))
  (bind _output_get (Variables|Default|SetStartingTile _playertile))
  (Variables|Default|SetCurrentTile _output_get)
  (Transformation|SetWorldRotation (Variables|Default|GetDefaultSceneRoot) "0, 0, 0" false false)
  (Audio|PlaySound2D "/Game/Audio/SoundEffects/417730__wcoltd__emplaser.417730__wcoltd__emplaser" 1.0 1.0 0.0 0 0)
  (CallFunction|GetTargetTiles)
  (for _array_element (Variables|Default|GetAbilityAOE)
    (CallFunction|DamageEnemies _array_element))
  (Utilities|FlowControl|Delay 0.4)
  (Actor|DestroyActor))

(fn ConstructionScript)

(fn GetTargetTiles
  (Utilities|FlowControl|ForLoopwithBreak 0 10 :!label _label
    (:LoopBody
      (Utilities|IsValid (Variables|/Game/Blueprints/Grid/BP_GridTile.BP_GridTile_C|GetNeighborEast (Variables|Default|GetCurrentTile))
        (:Is%20Valid
          (bind _output_get (Variables|Default|SetCurrentTile (Variables|/Game/Blueprints/Grid/BP_GridTile.BP_GridTile_C|GetNeighborEast (Variables|Default|GetCurrentTile))))
          (Utilities|Array|Add (Variables|Default|GetAbilityAOE) _output_get))
        (:Is%20Not%20Valid
          (goto _label Break))))
    (:Completed
      (return))))

(fn DamageEnemies
  (params (GridTile :type BP%20Grid%20Tile%20Object%20Reference))
  (bind _occupyingactor (Variables|/Game/Blueprints/Grid/BP_GridTile.BP_GridTile_C|GetOccupyingActor GridTile))
  (Utilities|IsValid _occupyingactor
    (:Is%20Valid
      (if (Actor|ActorHasTag _occupyingactor "Enemy")
        (Game|Damage|ApplyDamage _occupyingactor (Variables|Default|GetBase%20Damage) 0 0)
        (Niagara|SpawnSystematLocation "/Game/Sci-Fi_Starter_VFX_Pack_Niagara/Niagara/Impact/NS_Impact_Metal_1.NS_Impact_Metal_1" (+ (Variables|/Game/Blueprints/Grid/BP_GridTile.BP_GridTile_C|GetGridWorldLocation GridTile) "0,0.000000,100.000000") "0, 0,-90.000000" "2.000000,2.000000,2.000000")))))

(fn GetPlayerTile
  (return 0))

(fn SetChargingAttack
  (params (IsChargingAttack :type Boolean))
  (return false))