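; Plasma Blaster second ability actor: an EMP blast that stuns and damages all enemies.
; On BeginPlay it gets the player's grid tile, spawns an EMP explosion effect above it and plays two sounds.
; DamageEnemies then stuns and applies damage to every BP_Enemy_Master tagged Enemy, regardless of position.
; GetTargetTiles can collect a line of eastward tiles but is never called here.
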(event EventBeginPlay
  (bind _playertile (Class|BPIAttackSystem|GetPlayerTile(Message) (Game|GetPlayerCharacter 0)))
  (bind _output_get (Variables|Default|SetStartingTile _playertile))
  (Niagara|SpawnSystematLocation "/Game/Sci-Fi_Starter_VFX_Pack_Niagara/Niagara/Explosion/NS_Explosion_EMP.NS_Explosion_EMP" (+ (Variables|/Game/Blueprints/Grid/BP_GridTile.BP_GridTile_C|GetGridWorldLocation _output_get) "0.000000,0,100.000000") "0, 0, 0" "1.500000,1.500000,1.500000")
  (Audio|PlaySound2D "/Game/Audio/SoundEffects/184648__isaac200000__cannon3.184648__isaac200000__cannon3" 1.0 1.0 0.0 0 0)
  (Audio|PlaySound2D "/Game/Audio/SoundEffects/417730__wcoltd__emplaser.417730__wcoltd__emplaser" 1.0 1.0 0.0 0 0)
  (CallFunction|DamageEnemies))

(fn ConstructionScript)

(fn GetTargetTiles
  (Utilities|FlowControl|ForLoopwithBreak 0 10 :!label _label
    (:LoopBody
      (Utilities|IsValid (Variables|/Game/Blueprints/Grid/BP_GridTile.BP_GridTile_C|GetNeighborEast (Variables|Default|GetCurrentTile))
        (:Is%20Valid
          (bind _output_get (Variables|Default|SetCurrentTile (Variables|/Game/Blueprints/Grid/BP_GridTile.BP_GridTile_C|GetNeighborEast (Variables|Default|GetCurrentTile))))
          (Utilities|Array|Add (Variables|Default|GetAbilityAOE) _output_get))
        (:Is%20Not%20Valid
          (goto _label Break))))
    (:Completed
      (return))))

(fn DamageEnemies
  (bind _outactors (Actor|GetAllActorswithTag "Enemy"))
  (for _array_element _outactors
    (bind _asbp_enemy_master (Utilities|Casting|CastToBP_Enemy_Master _array_element))
    (Default|SetStunned _asbp_enemy_master)
    (Game|Damage|ApplyDamage _asbp_enemy_master (Variables|Default|GetBase%20Damage) 0 0)))

(fn GetPlayerTile
  (return 0))

(fn SetChargingAttack
  (params (IsChargingAttack :type Boolean))
  (return false))