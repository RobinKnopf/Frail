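; Energy Blaster first ability: a grid attack that fires east from the player's tile and chains to a second enemy.
; On BeginPlay it gets the player's tile and walks NeighborEast links for a limited range until it finds an Enemy-tagged occupant.
; It damages that enemy and the nearest other tagged enemy, spawning both impact effects at the first hit tile.
; IncreaseDamageby% scales BaseDamage; GetPlayerTile and SetChargingAttack are stubs.
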(event EventBeginPlay
  (bind _asbp_player_character (Utilities|Casting|CastToBP_PlayerCharacter (Game|GetPlayerCharacter 0)))
  (bind _output_get (Variables|Default|SetCharacterRef _asbp_player_character))
  (bind _playertile (Class|BPIAttackSystem|GetPlayerTile(Message) _output_get))
  (Variables|Default|SetCurrentTile _playertile)
  (CallFunction|CheckDamage))

(fn ConstructionScript)

(fn CheckDamage
  (Utilities|FlowControl|ForLoopwithBreak 0 10 :!label _label
    (:LoopBody
      (Utilities|IsValid (Variables|/Game/Blueprints/Grid/BP_GridTile.BP_GridTile_C|GetNeighborEast (Variables|Default|GetCurrentTile))
        (:Is%20Valid
          (bind _output_get (Variables|Default|SetCurrentTile (Variables|/Game/Blueprints/Grid/BP_GridTile.BP_GridTile_C|GetNeighborEast (Variables|Default|GetCurrentTile))))
          (Utilities|IsValid (Variables|/Game/Blueprints/Grid/BP_GridTile.BP_GridTile_C|GetOccupyingActor _output_get)
            (:Is%20Valid
              (if (Actor|ActorHasTag (Variables|/Game/Blueprints/Grid/BP_GridTile.BP_GridTile_C|GetOccupyingActor _output_get) "Enemy")
                (Game|Damage|ApplyDamage (Variables|/Game/Blueprints/Grid/BP_GridTile.BP_GridTile_C|GetOccupyingActor _output_get) (Variables|Default|GetBase%20Damage) 0 0)
                (Niagara|SpawnSystematLocation "/Game/Sci-Fi_Starter_VFX_Pack_Niagara/Niagara/Impact/NS_Impact_Metal_1.NS_Impact_Metal_1" (+ (Variables|/Game/Blueprints/Grid/BP_GridTile.BP_GridTile_C|GetGridWorldLocation _output_get) "0,0.000000,100.000000") "0, 0,-90.000000" "0.800000,0.800000,0.800000")
                (Utilities|FlowControl|Sequence
                  (:then_0
                    (goto _label Break))
                  (:then_1
                    (bind _outactors (Actor|GetAllActorswithTag "Enemy"))
                    (bind _output_get_2 (LocalVariables|SetEnemies _outactors))
                    (Utilities|Array|RemoveItem _output_get_2 (Variables|/Game/Blueprints/Grid/BP_GridTile.BP_GridTile_C|GetOccupyingActor _output_get))
                    (Game|Damage|ApplyDamage (.ReturnValue (Actor|FindNearestActor (Variables|/Game/Blueprints/Grid/BP_GridTile.BP_GridTile_C|GetGridWorldLocation (Variables|Default|GetCurrentTile)) (LocalVariables|GetEnemies))) (Variables|Default|GetBase%20Damage) 0 0)
                    (Niagara|SpawnSystematLocation "/Game/Sci-Fi_Starter_VFX_Pack_Niagara/Niagara/Impact/NS_Impact_Metal_1.NS_Impact_Metal_1" (+ (Variables|/Game/Blueprints/Grid/BP_GridTile.BP_GridTile_C|GetGridWorldLocation (Variables|Default|GetCurrentTile)) "0,0.000000,100.000000") "0, 0,-90.000000" "0.800000,0.800000,0.800000")))))))
        (:Is%20Not%20Valid
          (goto _label Break))))))

(fn IncreaseDamageby%
  (params (Percentage :type Float%20%28double-precision%29))
  (Variables|Default|SetBase%20Damage (+ (Variables|Default|GetBase%20Damage) (* (Variables|Default|GetBase%20Damage) (/ Percentage 1e+02)))))

(fn GetPlayerTile
  (return 0))

(fn SetChargingAttack
  (params (IsChargingAttack :type Boolean))
  (return false))