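; Cannon second ability: a muzzle blast launches a three-tile-wide shockwave that marches east across the grid, damaging enemies.
; BeginPlay starts at a hardcoded GridManager tile, plays effects and hits the tile plus its north and south neighbors.
; A looping one-second timer steps the column through NeighborEast links, applying damage to "Enemy"-tagged occupants, then replaying rock impacts after a short delay.
; The actor destroys itself when no east tile remains.
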(event Custom|MoveShockwave
  (CallFunction|MovetoNextTile)
  (Utilities|FlowControl|Delay 0.2)
  (for _array_element (Variables|Default|GetShockwaves)
    (Niagara|ResetSystem _array_element)
    (Niagara|SpawnSystematLocation "/Game/Sci-Fi_Starter_VFX_Pack_Niagara/Niagara/Impact/NS_Impact_Rock_1.NS_Impact_Rock_1" (Transformation|GetWorldLocation _array_element) "0, 0, 0" "2.000000,2.000000,1.500000"))
  (Audio|PlaySound2D "/Game/Audio/SoundEffects/587189__derplayer__explosion_05.587189__derplayer__explosion_05" 1.0 1.0 0.0 0 0))

(event EventBeginPlay
  (bind _asbp_player_character (Utilities|Casting|CastToBP_PlayerCharacter (Game|GetPlayerCharacter 0)))
  (Variables|Default|SetCharacterRef _asbp_player_character)
  (bind _returnvalue (Actor|GetActorOfClass "/Game/Blueprints/Grid/BP_GridManager.BP_GridManager_C"))
  (Variables|Default|SetCurrentTile (Utilities|Array|Get(acopy) (Variables|/Game/Blueprints/Grid/BP_GridManager.BP_GridManager_C|GetGridArray _returnvalue) 13))
  (CallFunction|SetAOE)
  (CallFunction|SetSpawnLocation)
  (Audio|PlaySound2D "/Game/Audio/SoundEffects/78457__sancho82__bum.78457__sancho82__bum" 1.0 1.0 0.0 0 0)
  (Niagara|SpawnSystematLocation "/Game/Sci-Fi_Starter_VFX_Pack_Niagara/Niagara/MuzzleFlash/NS_MuzzleFlash_1.NS_MuzzleFlash_1" (Transformation|GetWorldLocation (Variables|/Game/Character/Attachments/BP_WeaponAttachment_Blaster.BP_WeaponAttachment_Blaster_C|GetMuzzleFlash (Variables|/Game/Character/BP_PlayerCharacter.BP_PlayerCharacter_C|GetWeaponAttached (Variables|Default|GetCharacterRef)))) "0, 0,90.000000" "2.000000,2.000000,2.000000")
  (CallFunction|CheckTargetHit)
  (Audio|PlaySound2D "/Game/Audio/SoundEffects/587189__derplayer__explosion_05.587189__derplayer__explosion_05" 1.0 1.0 0.0 0 0)
  (for _array_element (Variables|Default|GetShockwaves)
    (Niagara|SpawnSystematLocation "/Game/Sci-Fi_Starter_VFX_Pack_Niagara/Niagara/Impact/NS_Impact_Rock_1.NS_Impact_Rock_1" (Transformation|GetWorldLocation _array_element) "0, 0, 0" "2.000000,2.000000,1.500000"))
  (Utilities|Time|SetTimerbyEvent (delegate Custom|MoveShockwave) 1.0 true))

(fn ConstructionScript)

(fn MovetoNextTile
  (Utilities|IsValid (Variables|/Game/Blueprints/Grid/BP_GridTile.BP_GridTile_C|GetNeighborEast (Variables|Default|GetCurrentTile))
    (:Is%20Valid
      (bind _output_get (Variables|Default|SetCurrentTile (Variables|/Game/Blueprints/Grid/BP_GridTile.BP_GridTile_C|GetNeighborEast (Variables|Default|GetCurrentTile))))
      (Transformation|SetWorldLocation (Variables|Default|GetShockwave) (Variables|/Game/Blueprints/Grid/BP_GridTile.BP_GridTile_C|GetGridWorldLocation _output_get) false false)
      (CallFunction|SetNeighbors)
      (CallFunction|SetAOE)
      (CallFunction|CheckTargetHit)
      (return))
    (:Is%20Not%20Valid
      (Actor|DestroyActor))))

(fn CheckTargetHit
  (for _array_element (Variables|Default|GetAbilityAOE)
    (Utilities|IsValid (Variables|/Game/Blueprints/Grid/BP_GridTile.BP_GridTile_C|GetOccupyingActor _array_element)
      (:Is%20Valid
        (if (Actor|ActorHasTag (Variables|/Game/Blueprints/Grid/BP_GridTile.BP_GridTile_C|GetOccupyingActor _array_element) "Enemy")
          (Game|Damage|ApplyDamage (Variables|/Game/Blueprints/Grid/BP_GridTile.BP_GridTile_C|GetOccupyingActor _array_element) (Variables|Default|GetBase%20Damage) 0 0))))))

(fn SetSpawnLocation
  (Transformation|SetWorldLocation (Variables|Default|GetShockwave) (Variables|/Game/Blueprints/Grid/BP_GridTile.BP_GridTile_C|GetGridWorldLocation (Variables|Default|GetCurrentTile)) false false)
  (CallFunction|SetNeighbors))

(fn SetNeighbors
  (Transformation|SetWorldLocation (Variables|Default|GetShockwave2) (Variables|/Game/Blueprints/Grid/BP_GridTile.BP_GridTile_C|GetGridWorldLocation (Variables|/Game/Blueprints/Grid/BP_GridTile.BP_GridTile_C|GetNeighborNorth (Variables|Default|GetCurrentTile))) false false)
  (Transformation|SetWorldLocation (Variables|Default|GetShockwave1) (Variables|/Game/Blueprints/Grid/BP_GridTile.BP_GridTile_C|GetGridWorldLocation (Variables|/Game/Blueprints/Grid/BP_GridTile.BP_GridTile_C|GetNeighborSouth (Variables|Default|GetCurrentTile))) false false))

(fn SetAOE
  (bind _currenttile (Variables|Default|GetCurrentTile))
  (Variables|Default|SetAbilityAOE (Utilities|Array|MakeArray _currenttile (Variables|/Game/Blueprints/Grid/BP_GridTile.BP_GridTile_C|GetNeighborNorth _currenttile) (Variables|/Game/Blueprints/Grid/BP_GridTile.BP_GridTile_C|GetNeighborSouth _currenttile)))
  (Variables|Default|SetShockwaves (Utilities|Array|MakeArray (Variables|Default|GetShockwave) (Variables|Default|GetShockwave2) (Variables|Default|GetShockwave1))))

(fn GetPlayerTile
  (return 0))

(fn SetChargingAttack
  (params (IsChargingAttack :type Boolean))
  (return false))