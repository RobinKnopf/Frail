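; Particle cannon second ability actor: fires a delayed area strike on grid tiles east of the player.
; On BeginPlay it reads the player's tile, plays a muzzle flash, then walks east neighbours by AbilityRange plus one to pick the target tile.
; A laser effect marks that tile; after a short delay, enemy-tagged occupants of it and its surrounding tiles take damage, then an explosion plays.
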(event EventBeginPlay
  (bind _targettile (Variables|Default|GetTargetTile))
  (bind _gridworldlocation (Variables|/Game/Blueprints/Grid/BP_GridTile.BP_GridTile_C|GetGridWorldLocation _targettile))
  (bind _asbp_player_character (Utilities|Casting|CastToBP_PlayerCharacter (Game|GetPlayerCharacter 0)))
  (bind _output_get (Variables|Default|SetCharacterRef _asbp_player_character))
  (bind _playertile (Class|BPIAttackSystem|GetPlayerTile(Message) _output_get))
  (Variables|Default|SetCurrentTile _playertile)
  (CallFunction|SetSpawnLocation)
  (Niagara|SpawnSystematLocation "/Game/Sci-Fi_Starter_VFX_Pack_Niagara/Niagara/MuzzleFlash/NS_MuzzleFlash_2.NS_MuzzleFlash_2" (Transformation|GetWorldLocation (Variables|/Game/Character/Attachments/BP_WeaponAttachment_Blaster.BP_WeaponAttachment_Blaster_C|GetMuzzleFlash (Variables|/Game/Character/BP_PlayerCharacter.BP_PlayerCharacter_C|GetWeaponAttached (Variables|Default|GetCharacterRef)))) "0, 0,90.000000" "3.000000,3.000000,3.000000")
  (Audio|PlaySound2D "/Game/Audio/SoundEffects/567308__bigdino1995__plasmacannon.567308__bigdino1995__plasmacannon" 1.0 1.0 0.0 0 0)
  (CallFunction|GetTargetTile)
  (CallFunction|SetAbilityAOE)
  (bind _returnvalue (Niagara|SpawnSystematLocation "/Game/Sci-Fi_Starter_VFX_Pack_Niagara/Niagara/Laser/NS_Laser_4.NS_Laser_4" _gridworldlocation "0, 0, 0" "1.500000,1.500000,0.000000"))
  (Audio|PlaySound2D "/Game/Audio/SoundEffects/458690__jorgerosa__ufo-shield.458690__jorgerosa__ufo-shield" 1.0 1.0 0.0 0 0)
  (Utilities|FlowControl|Delay 0.8)
  (for _array_element (Variables|Default|GetAbilityAOE)
    (CallFunction|CheckDamage&Particle _array_element))
  (Components|DestroyComponent _returnvalue)
  (Niagara|SpawnSystematLocation "/Game/Sci-Fi_Starter_VFX_Pack_Niagara/Niagara/Explosion/NS_Explosion_C4_2.NS_Explosion_C4_2" _gridworldlocation "0, 0, 0" "0.500000,0.500000,0.500000")
  (Audio|PlaySound2D "/Game/Audio/SoundEffects/264031__veiler__low-mid-afar-explosion-1.264031__veiler__low-mid-afar-explosion-1" 1.0 1.0 0.0 0 0))

(fn ConstructionScript)

(fn GetTargetTile
  (for _index (range 0 (- (Variables|Default|GetAbilityRange) 1))
    (Variables|Default|SetCurrentTile (Variables|/Game/Blueprints/Grid/BP_GridTile.BP_GridTile_C|GetNeighborEast (Variables|Default|GetCurrentTile))))
  (Variables|Default|SetTargetTile (Variables|/Game/Blueprints/Grid/BP_GridTile.BP_GridTile_C|GetNeighborEast (Variables|Default|GetCurrentTile)))
  (return))

(fn SetAbilityAOE
  (bind _targettile (Variables|Default|GetTargetTile))
  (bind _output_get (Variables|Default|SetAbilityAOE (Variables|/Game/Blueprints/Grid/BP_GridTile.BP_GridTile_C|GetSurroundingTiles _targettile)))
  (Utilities|Array|Add _output_get _targettile))

(fn CheckDamage&Particle
  (params (GridTile :type BP%20Grid%20Tile%20Object%20Reference))
  (bind _occupyingactor (Variables|/Game/Blueprints/Grid/BP_GridTile.BP_GridTile_C|GetOccupyingActor GridTile))
  (Utilities|IsValid _occupyingactor
    (:Is%20Valid
      (if (Actor|ActorHasTag _occupyingactor "Enemy")
        (Game|Damage|ApplyDamage _occupyingactor (Variables|Default|GetBase%20Damage) 0 0)))))

(fn SetSpawnLocation
  (Transformation|SetWorldLocation (Variables|Default|GetCollisionComponent) (+ (Variables|/Game/Blueprints/Grid/BP_GridTile.BP_GridTile_C|GetGridWorldLocation (Variables|Default|GetCurrentTile)) "0, 0,100.000000") false false))

(fn GetPlayerTile
  (return 0))

(fn SetChargingAttack
  (params (IsChargingAttack :type Boolean))
  (return false))