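; Mega Blaster second ability: a bomb that falls on a grid tile a set range east of the player and damages enemies around it.
; On BeginPlay it gets the player's tile, walks east neighbors to the target, builds the blast area from that tile and its valid neighbors, and spawns a muzzle flash.
; The Fall timeline drops the bomb; on finish it damages Enemy-tagged occupants, plays explosion effects per tile, then destroys itself.
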(event EventBeginPlay
  (bind _asbp_player_character (Utilities|Casting|CastToBP_PlayerCharacter (Game|GetPlayerCharacter 0)))
  (bind _playertile (Class|BPIAttackSystem|GetPlayerTile(Message) _asbp_player_character))
  (Variables|Default|SetCurrentTile _playertile)
  (CallFunction|SetSpawnLocation)
  (CallFunction|GetTargetTile)
  (CallFunction|SetAbilityAOE)
  (Niagara|SpawnSystematLocation "/Game/Sci-Fi_Starter_VFX_Pack_Niagara/Niagara/MuzzleFlash/NS_MuzzleFlash_1.NS_MuzzleFlash_1" (Transformation|GetWorldLocation (Variables|/Game/Character/Attachments/BP_WeaponAttachment_Blaster.BP_WeaponAttachment_Blaster_C|GetMuzzleFlash (Variables|/Game/Character/BP_PlayerCharacter.BP_PlayerCharacter_C|GetWeaponAttached _asbp_player_character))) "0, 0,90.000000")
  (bind _falling (Timeline|Fall Play)
    (:Update
      (Transformation|SetWorldLocation (Variables|Default|GetBomb) (+ (Variables|/Game/Blueprints/Grid/BP_GridTile.BP_GridTile_C|GetGridWorldLocation (Variables|Default|GetTargetTile)) _falling) false false))
    (:Finished
      (for _array_element (Variables|Default|GetAbilityAOE)
        (CallFunction|CheckDamage&Particle _array_element))
      (Utilities|FlowControl|Delay 0.05)
      (for _array_element_2 (Variables|Default|GetAbilityAOE)
        (Niagara|SpawnSystematLocation "/Game/Sci-Fi_Starter_VFX_Pack_Niagara/Niagara/Explosion/NS_Explosion_C4_2.NS_Explosion_C4_2" (Variables|/Game/Blueprints/Grid/BP_GridTile.BP_GridTile_C|GetGridWorldLocation _array_element_2) "0, 0, 0" "0.200000,0.200000,0.200000")
        (Audio|PlaySoundatLocation "/Game/Audio/SoundEffects/Sci_Fi_Grenade_2.Sci_Fi_Grenade_2" "0, 0, 0" "0, 0, 0" 1.0 1.0 0.0 0 0 0 0))
      (Actor|DestroyActor))))

(fn ConstructionScript)

(fn GetTargetTile
  (for _index (range 0 (- (Variables|Default|GetAbilityRange) 1))
    (bind _output_get (Variables|Default|SetCurrentTile (Variables|/Game/Blueprints/Grid/BP_GridTile.BP_GridTile_C|GetNeighborEast (Variables|Default|GetCurrentTile)))))
  (Variables|Default|SetTargetTile _output_get)
  (return))

(fn SetAbilityAOE
  (bind _targettile (Variables|Default|GetTargetTile))
  (bind _output_get (Variables|Default|SetAbilityAOE (Variables|/Game/Blueprints/Grid/BP_GridTile.BP_GridTile_C|GetValidNeighbors _targettile)))
  (Utilities|Array|Add _output_get _targettile))

(fn CheckDamage&Particle
  (params (GridTile :type BP%20Grid%20Tile%20Object%20Reference))
  (bind _occupyingactor (Variables|/Game/Blueprints/Grid/BP_GridTile.BP_GridTile_C|GetOccupyingActor GridTile))
  (Utilities|IsValid _occupyingactor
    (:Is%20Valid
      (if (Actor|ActorHasTag _occupyingactor "Enemy")
        (Game|Damage|ApplyDamage _occupyingactor (Variables|Default|GetBase%20Damage) 0 0)))))

(fn SetSpawnLocation
  (Transformation|SetWorldLocation (Variables|Default|GetCollisionComponent) (+ (Variables|/Game/Blueprints/Grid/BP_GridTile.BP_GridTile_C|GetGridWorldLocation (Variables|Default|GetCurrentTile)) "0, 0,100.000000") false false))

(fn GetPlayerTile
  (return 0))

(fn SetChargingAttack
  (params (IsChargingAttack :type Boolean))
  (return false))