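; Energy Blaster second ability: fires a plasma ball east along the player's tile grid, leaving a damaging lightning field.
; BeginPlay picks the target up to four tiles away, caches it plus surrounding tiles, and moves the ball by timeline.
; While the lightning effect lives, Tick uses a Delay to repeatedly damage enemies there; destruction clears effect and sound.
; CheckMods reads Kinetic damage and explosive mods but is not called here.
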(event Custom|OnDestroyedEvent
  (params (DestroyedActor :type Actor%20Object%20Reference))
  (Components|DestroyComponent (stale EventBeginPlay _output_get_2))
  (Audio|Components|Audio|Stop (stale EventBeginPlay _returnvalue_2)))

(event EventBeginPlay
  (bind _asbp_player_character (Utilities|Casting|CastToBP_PlayerCharacter (Game|GetPlayerCharacter 0)))
  (bind _output_get (Variables|Default|SetCharacterRef _asbp_player_character))
  (bind _playertile (Class|BPIAttackSystem|GetPlayerTile(Message) _output_get))
  (Variables|Default|SetCurrentTile _playertile)
  (Audio|PlaySound2D "/Game/Audio/SoundEffects/Sci_Fi_Pistol_1.Sci_Fi_Pistol_1" 1.0 1.0 0.0 0 0)
  (Niagara|SpawnSystematLocation "/Game/Sci-Fi_Starter_VFX_Pack_Niagara/Niagara/MuzzleFlash/NS_MuzzleFlash_4.NS_MuzzleFlash_4" (Transformation|GetWorldLocation (Variables|/Game/Character/Attachments/BP_WeaponAttachment_Blaster.BP_WeaponAttachment_Blaster_C|GetMuzzleFlash (Variables|/Game/Character/BP_PlayerCharacter.BP_PlayerCharacter_C|GetWeaponAttached (Variables|Default|GetCharacterRef)))) "0, 0,90.000000" "2.000000,2.000000,1.000000")
  (CallFunction|SetRange&AOE)
  (bind _alpha (Timeline|Projectile Play)
    (:Update
      (Transformation|SetWorldLocation (Variables|Default|GetPlasmaBall) (Math|Vector|Lerp(Vector) (Transformation|GetWorldLocation (Variables|Default|GetPlasmaBall)) (Variables|/Game/Blueprints/Grid/BP_GridTile.BP_GridTile_C|GetGridWorldLocation (Variables|Default|GetCurrentTile)) _alpha) false false))
    (:Finished
      (bind _returnvalue (Niagara|SpawnSystematLocation "/Game/Sci-Fi_Starter_VFX_Pack_Niagara/Niagara/Environment/NS_Environment_Lightning_2.NS_Environment_Lightning_2" (Variables|/Game/Blueprints/Grid/BP_GridTile.BP_GridTile_C|GetGridWorldLocation (Variables|Default|GetCurrentTile)) "0, 0, 0" "0.750000,0.750000,0.750000"))
      (bind _output_get_2 (Variables|Default|SetParticle _returnvalue))
      (Game|AssignOnDestroyed (delegate Custom|OnDestroyedEvent))
      (bind _returnvalue_2 (Audio|SpawnSound2D "/Game/Audio/SoundEffects/657818__the-sacha-rush__electric-shock-4-hit.657818__the-sacha-rush__electric-shock-4-hit" 1.0 1.0 0.0 0)))))

(event EventTick
  (params (DeltaSeconds :type Float%20%28single-precision%29))
  (if (Utilities|IsValid (Variables|Default|GetParticle))
    (Utilities|FlowControl|Delay 0.25)
    (for _array_element (Variables|Default|GetAbilityAOE)
      (Utilities|IsValid (Variables|/Game/Blueprints/Grid/BP_GridTile.BP_GridTile_C|GetOccupyingActor _array_element)
        (:Is%20Valid
          (if (Actor|ActorHasTag (Variables|/Game/Blueprints/Grid/BP_GridTile.BP_GridTile_C|GetOccupyingActor _array_element) "Enemy")
            (Game|Damage|ApplyDamage (Variables|/Game/Blueprints/Grid/BP_GridTile.BP_GridTile_C|GetOccupyingActor _array_element) (Variables|Default|GetBase%20Damage) 0 0)))))))

(fn ConstructionScript)

(fn SetRange&AOE
  (Utilities|FlowControl|ForLoopwithBreak 0 3 :!label _label
    (:LoopBody
      (Utilities|IsValid (Variables|/Game/Blueprints/Grid/BP_GridTile.BP_GridTile_C|GetNeighborEast (Variables|Default|GetCurrentTile))
        (:Is%20Valid
          (Variables|Default|SetCurrentTile (Variables|/Game/Blueprints/Grid/BP_GridTile.BP_GridTile_C|GetNeighborEast (Variables|Default|GetCurrentTile))))
        (:Is%20Not%20Valid
          (goto _label Break))))
    (:Completed
      (bind _output_get (Variables|Default|SetAbilityAOE (Variables|/Game/Blueprints/Grid/BP_GridTile.BP_GridTile_C|GetSurroundingTiles (Variables|Default|GetCurrentTile))))
      (Utilities|Array|Add _output_get (Variables|Default|GetCurrentTile)))))

(fn CheckMods
  (Utilities|FlowControl|Sequence
    (:then_0
      (for _array_element (Actor|GetComponentsByClass (Variables|Default|GetCharacterRef) "/Game/Character/ModInventory/ModActors/BP_Mod_Kinetic_Hype.BP_Mod_Kinetic_Hype_C")
        (Utilities|IsValid _array_element
          (:Is%20Valid
            (bind _asbp_mod_kinetic_hype (Utilities|Casting|CastToBP_Mod_Kinetic_Hype _array_element))
            (CallFunction|IncreaseDamageby% (Variables|/Game/Character/ModInventory/ModActors/BP_Mod_Kinetic_Hype.BP_Mod_Kinetic_Hype_C|GetIncrease%25 _asbp_mod_kinetic_hype))))))
    (:then_1
      (for _array_element_2 (Actor|GetComponentsByClass (Variables|Default|GetCharacterRef) "/Game/Character/ModInventory/ModActors/BP_Mod_Kinetic_Explosive.BP_Mod_Kinetic_Explosive_C")
        (Utilities|IsValid _array_element_2
          (:Is%20Valid
            (bind _asbp_mod_kinetic_explosive (Utilities|Casting|CastToBP_Mod_Kinetic_Explosive _array_element_2))
            (Variables|Explosive|SetExplosive (Variables|/Game/Character/ModInventory/ModActors/BP_Mod_Kinetic_Explosive.BP_Mod_Kinetic_Explosive_C|GetExplosive _asbp_mod_kinetic_explosive))
            (Variables|Explosive|SetExplosive%20Value (Variables|/Game/Character/ModInventory/ModActors/BP_Mod_Kinetic_Explosive.BP_Mod_Kinetic_Explosive_C|GetExplosiveValue _asbp_mod_kinetic_explosive))))))
    (:then_2
      (return))))

(fn IncreaseDamageby%
  (params (Percentage :type Float%20%28double-precision%29))
  (Variables|Default|SetBase%20Damage (+ (Variables|Default|GetBase%20Damage) (* (Variables|Default|GetBase%20Damage) (/ Percentage 1e+02)))))

(fn GetPlayerTile
  (return 0))

(fn SetChargingAttack
  (params (IsChargingAttack :type Boolean))
  (return false))