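; Energy Cannon second ability actor that calls down a series of thunder strikes on random tiles in a fixed range of the grid.
; On BeginPlay it plays a muzzle flash and sound at the player's weapon, waits briefly, then loops SpawnThunder until NumberOfThunder runs out and destroys itself.
; Each strike picks a tile from BP_GridManager, damages any Enemy-tagged occupant with an explosion effect, and shows a short-lived laser with sound.
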(event EventBeginPlay
  (bind _asbp_player_character (Utilities|Casting|CastToBP_PlayerCharacter (Game|GetPlayerCharacter 0)))
  (Variables|Default|SetCharacterRef _asbp_player_character)
  (bind _returnvalue (Actor|GetActorOfClass "/Game/Blueprints/Grid/BP_GridManager.BP_GridManager_C"))
  (Variables|Default|SetGrid _returnvalue)
  (Niagara|SpawnSystematLocation "/Game/Sci-Fi_Starter_VFX_Pack_Niagara/Niagara/MuzzleFlash/NS_MuzzleFlash_4.NS_MuzzleFlash_4" (Transformation|GetWorldLocation (Variables|/Game/Character/Attachments/BP_WeaponAttachment_Blaster.BP_WeaponAttachment_Blaster_C|GetMuzzleFlash (Variables|/Game/Character/BP_PlayerCharacter.BP_PlayerCharacter_C|GetWeaponAttached (Variables|Default|GetCharacterRef)))) "0, 0,90.000000" "2.000000,2.000000,2.000000")
  (Audio|SpawnSound2D "/Game/Audio/SoundEffects/458690__jorgerosa__ufo-shield.458690__jorgerosa__ufo-shield" 1.0 1.0 0.0 0)
  (Utilities|FlowControl|Delay 1.0)
  (if (>= (Variables|Default|GetNumberOfThunder) 0) :!label _label
    (Utilities|SpawnThunder
      (:%20%20
        (goto _label)))
    (else
      (Actor|DestroyActor))))

(fn ConstructionScript)

(fn CheckDamage
  (params (GridTile :type BP%20Grid%20Tile%20Object%20Reference))
  (bind _occupyingactor (Variables|/Game/Blueprints/Grid/BP_GridTile.BP_GridTile_C|GetOccupyingActor GridTile))
  (Utilities|IsValid _occupyingactor
    (:Is%20Valid
      (if (Actor|ActorHasTag _occupyingactor "Enemy")
        (Game|Damage|ApplyDamage _occupyingactor (Variables|Default|GetBase%20Damage) 0 0)
        (Niagara|SpawnSystematLocation "/Game/Sci-Fi_Starter_VFX_Pack_Niagara/Niagara/Explosion/NS_Explosion_Small_2.NS_Explosion_Small_2" (Variables|/Game/Blueprints/Grid/BP_GridTile.BP_GridTile_C|GetGridWorldLocation GridTile) "0, 0, 0" "0.700000,0.700000,0.700000")))))

(fn GetRandomEnemyTile
  (return (Utilities|Array|Get(acopy) (Variables|/Game/Blueprints/Grid/BP_GridManager.BP_GridManager_C|GetGridArray (Variables|Default|GetGrid)) (Math|Random|RandomIntegerinRange 12 23))))

(fn GetPlayerTile
  (return 0))

(fn SetChargingAttack
  (params (IsChargingAttack :type Boolean))
  (return false))