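; Player energy cannon first attack: a plasma ball that travels east along the tile grid from the player's current tile.
; On spawn it plays sounds and a muzzle flash, then replays a timeline tile by tile through NeighborEast links, destroying itself at the row's end.
; A delay-throttled Tick damages Enemy-tagged occupants of the current and next tile, using tile lookups rather than collision.
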(event Custom|StopSound
  (params (DestroyedActor :type Actor%20Object%20Reference))
  (Audio|Components|Audio|Stop (stale EventBeginPlay _returnvalue)))

(event Custom|MoveAttack
  (Utilities|IsValid (Variables|/Game/Blueprints/Grid/BP_GridTile.BP_GridTile_C|GetNeighborEast (Variables|Default|GetCurrentTile)) :!label _label
    (:Is%20Valid
      (bind _output_get (Variables|Default|SetCurrentTile (Variables|/Game/Blueprints/Grid/BP_GridTile.BP_GridTile_C|GetNeighborEast (Variables|Default|GetCurrentTile))))
      (bind _movement (Timeline|ProjectileMov PlayFromStart)
        (:Update
          (Transformation|SetWorldLocation (Variables|Default|GetPlasmaBall) (+ _movement (+ (Variables|/Game/Blueprints/Grid/BP_GridTile.BP_GridTile_C|GetGridWorldLocation _output_get) "0,0,100.000000")) false false))
        (:Finished
          (goto _label))))
    (:Is%20Not%20Valid
      (Actor|DestroyActor))))

(event EventBeginPlay
  (bind _asbp_player_character (Utilities|Casting|CastToBP_PlayerCharacter (Game|GetPlayerCharacter 0)))
  (bind _output_get (Variables|Default|SetCharacterRef _asbp_player_character))
  (bind _playertile (Class|BPIAttackSystem|GetPlayerTile(Message) _output_get))
  (Variables|Default|SetCurrentTile _playertile)
  (Audio|PlaySound2D "/Game/Audio/SoundEffects/458690__jorgerosa__ufo-shield.458690__jorgerosa__ufo-shield" 1.0 1.0 0.0 0 0)
  (Niagara|SpawnSystematLocation "/Game/Sci-Fi_Starter_VFX_Pack_Niagara/Niagara/MuzzleFlash/NS_MuzzleFlash_4.NS_MuzzleFlash_4" (Transformation|GetWorldLocation (Variables|/Game/Character/Attachments/BP_WeaponAttachment_Blaster.BP_WeaponAttachment_Blaster_C|GetMuzzleFlash (Variables|/Game/Character/BP_PlayerCharacter.BP_PlayerCharacter_C|GetWeaponAttached (Variables|Default|GetCharacterRef)))) "0, 0,90.000000")
  (CallFunction|MoveAttack)
  (bind _returnvalue (Audio|SpawnSound2D "/Game/Audio/SoundEffects/657818__the-sacha-rush__electric-shock-4-hit.657818__the-sacha-rush__electric-shock-4-hit" 1.0 1.0 0.0 0))
  (Game|BindEventtoOnDestroyed (delegate Custom|StopSound)))

(event EventTick
  (params (DeltaSeconds :type Float%20%28single-precision%29))
  (bind _currenttile (Variables|Default|GetCurrentTile))
  (Utilities|FlowControl|Delay 0.3)
  (CallFunction|CheckDamage _currenttile)
  (bind _neighboreast (Variables|/Game/Blueprints/Grid/BP_GridTile.BP_GridTile_C|GetNeighborEast _currenttile)
    (:then
      (CallFunction|CheckDamage _neighboreast))
    (:else)))

(fn ConstructionScript)

(fn CheckDamage
  (params (Actor :type BP%20Grid%20Tile%20Object%20Reference))
  (bind _occupyingactor (Variables|/Game/Blueprints/Grid/BP_GridTile.BP_GridTile_C|GetOccupyingActor Actor))
  (Utilities|IsValid _occupyingactor
    (:Is%20Valid
      (if (Actor|ActorHasTag _occupyingactor "Enemy")
        (Game|Damage|ApplyDamage _occupyingactor (Variables|Default|GetBase%20Damage) 0 0)))))

(fn GetPlayerTile
  (return 0))

(fn SetChargingAttack
  (params (IsChargingAttack :type Boolean))
  (return false))