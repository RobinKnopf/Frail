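; Player cannon basic attack for grid combat, resolved instantly on BeginPlay with sound and muzzle flash.
; It applies the player's Kinetic mod components first: Hype raises base damage by a percentage, Explosive enables splash.
; It then walks up to four tiles east from the player's tile, damaging the first enemy found.
; With Explosive, surrounding tiles get effects until one enemy is found and takes a percentage of the damage.
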(event EventBeginPlay
  (bind _asbp_player_character (Utilities|Casting|CastToBP_PlayerCharacter (Game|GetPlayerCharacter 0)))
  (bind _output_get (Variables|Default|SetCharacterRef _asbp_player_character))
  (bind _playertile (Class|BPIAttackSystem|GetPlayerTile(Message) _output_get))
  (Variables|Default|SetCurrentTile _playertile)
  (Audio|PlaySound2D "/Game/Audio/SoundEffects/78457__sancho82__bum.78457__sancho82__bum" 1.0 1.0 0.0 0 0)
  (Niagara|SpawnSystematLocation "/Game/Sci-Fi_Starter_VFX_Pack_Niagara/Niagara/MuzzleFlash/NS_MuzzleFlash_1.NS_MuzzleFlash_1" (Transformation|GetWorldLocation (Variables|/Game/Character/Attachments/BP_WeaponAttachment_Blaster.BP_WeaponAttachment_Blaster_C|GetMuzzleFlash (Variables|/Game/Character/BP_PlayerCharacter.BP_PlayerCharacter_C|GetWeaponAttached (Variables|Default|GetCharacterRef)))) "0, 0,90.000000")
  (CallFunction|CheckMods)
  (CallFunction|CheckDamage))

(fn ConstructionScript)

(fn CheckDamage
  (Utilities|FlowControl|ForLoopwithBreak 0 3 :!label _label
    (:LoopBody
      (Utilities|IsValid (Variables|/Game/Blueprints/Grid/BP_GridTile.BP_GridTile_C|GetNeighborEast (Variables|Default|GetCurrentTile))
        (:Is%20Valid
          (bind _output_get (Variables|Default|SetCurrentTile (Variables|/Game/Blueprints/Grid/BP_GridTile.BP_GridTile_C|GetNeighborEast (Variables|Default|GetCurrentTile))))
          (Utilities|IsValid (Variables|/Game/Blueprints/Grid/BP_GridTile.BP_GridTile_C|GetOccupyingActor _output_get)
            (:Is%20Valid
              (if (Actor|ActorHasTag (Variables|/Game/Blueprints/Grid/BP_GridTile.BP_GridTile_C|GetOccupyingActor _output_get) "Enemy")
                (Game|Damage|ApplyDamage (Variables|/Game/Blueprints/Grid/BP_GridTile.BP_GridTile_C|GetOccupyingActor _output_get) (Variables|Default|GetBase%20Damage) 0 0)
                (Niagara|SpawnSystematLocation "/Game/Sci-Fi_Starter_VFX_Pack_Niagara/Niagara/Impact/NS_Impact_Metal_1.NS_Impact_Metal_1" (+ (Variables|/Game/Blueprints/Grid/BP_GridTile.BP_GridTile_C|GetGridWorldLocation _output_get) "0,0.000000,100.000000") "0, 0,-90.000000" "0.800000,0.800000,0.800000")
                (Utilities|FlowControl|Sequence
                  (:then_0
                    (goto _label Break))
                  (:then_1
                    (if (Variables|Explosive|GetExplosive)
                      (for _array_element (Variables|/Game/Blueprints/Grid/BP_GridTile.BP_GridTile_C|GetSurroundingTiles (Variables|Default|GetCurrentTile))
                        (Niagara|SpawnSystematLocation "/Game/Sci-Fi_Starter_VFX_Pack_Niagara/Niagara/Blood/NS_Blood_Mesh_5.NS_Blood_Mesh_5" (Variables|/Game/Blueprints/Grid/BP_GridTile.BP_GridTile_C|GetGridWorldLocation _array_element))
                        (Utilities|IsValid (Variables|/Game/Blueprints/Grid/BP_GridTile.BP_GridTile_C|GetOccupyingActor _array_element)
                          (:Is%20Valid
                            (if (Actor|ActorHasTag (Variables|/Game/Blueprints/Grid/BP_GridTile.BP_GridTile_C|GetOccupyingActor _array_element) "Enemy")
                              (Game|Damage|ApplyDamage (Variables|/Game/Blueprints/Grid/BP_GridTile.BP_GridTile_C|GetOccupyingActor _array_element) (CallFunction|GetExplosiveDamage) 0 0)
                              (goto _label Break))))))))))))
        (:Is%20Not%20Valid
          (goto _label Break))))))

(fn CheckMods
  (Utilities|FlowControl|Sequence
    (:then_0
      (for _array_element (Actor|GetComponentsByClass (Variables|Default|GetCharacterRef) "/Game/Character/ModInventory/ModActors/BP_Mod_Kinetic_Hype.BP_Mod_Kinetic_Hype_C")
        (Utilities|IsValid _array_element
          (:Is%20Valid
            (bind _asbp_mod_kinetic_hype (Utilities|Casting|CastToBP_Mod_Kinetic_Hype _array_element))
            (CallFunction|IncreaseDamageby% (Variables|/Game/Character/ModInventory/ModActors/BP_Mod_Kinetic_Hype.BP_Mod_Kinetic_Hype_C|GetIncrease%25 _asbp_mod_kinetic_hype))))))
    (:then_1
      (for _array_element_2 (Actor|GetComponentsByClass (Variables|Default|GetCharacterRef) "/Game/Character/ModInventory/ModActors/BP_Mod_Kinetic_Explosive.BP_Mod_Kinetic_Explosive_C")
        (Utilities|IsValid _array_element_2
          (:Is%20Valid
            (bind _asbp_mod_kinetic_explosive (Utilities|Casting|CastToBP_Mod_Kinetic_Explosive _array_element_2))
            (Variables|Explosive|SetExplosive (Variables|/Game/Character/ModInventory/ModActors/BP_Mod_Kinetic_Explosive.BP_Mod_Kinetic_Explosive_C|GetExplosive _asbp_mod_kinetic_explosive))
            (Variables|Explosive|SetExplosive%20Value (Variables|/Game/Character/ModInventory/ModActors/BP_Mod_Kinetic_Explosive.BP_Mod_Kinetic_Explosive_C|GetExplosiveValue _asbp_mod_kinetic_explosive))))))
    (:then_2
      (return))))

(fn IncreaseDamageby%
  (params (Percentage :type Float%20%28double-precision%29))
  (Variables|Default|SetBase%20Damage (+ (Variables|Default|GetBase%20Damage) (* (Variables|Default|GetBase%20Damage) (/ Percentage 1e+02)))))

(fn GetExplosiveDamage
  (return (* (Variables|Default|GetBase%20Damage) (/ (Variables|Explosive|GetExplosive%20Value) 1e+02))))

(fn GetPlayerTile
  (return 0))

(fn SetChargingAttack
  (params (IsChargingAttack :type Boolean))
  (return false))