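; Particle cannon first-ability attack actor: a shockwave that travels east along the tile grid from the player, damaging Enemy-tagged occupants.
; On BeginPlay it takes the player's tile, places its collision on the east neighbor and plays muzzle flash and firing sound.
; A looping timer steps it through east-neighbor links, checking each tile's occupant directly rather than using overlaps.
; It destroys itself when no east tile remains.
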(event Custom|MoveShockwave
  (CallFunction|MovetoNextTile))

(event EventBeginPlay
  (bind _asbp_player_character (Utilities|Casting|CastToBP_PlayerCharacter (Game|GetPlayerCharacter 0)))
  (bind _output_get (Variables|Default|SetCharacterRef _asbp_player_character))
  (bind _playertile (Class|BPIAttackSystem|GetPlayerTile(Message) _output_get))
  (Variables|Default|SetCurrentTile _playertile)
  (CallFunction|SetSpawnLocation)
  (Niagara|SpawnSystematLocation "/Game/Sci-Fi_Starter_VFX_Pack_Niagara/Niagara/MuzzleFlash/NS_MuzzleFlash_2.NS_MuzzleFlash_2" (Transformation|GetWorldLocation (Variables|/Game/Character/Attachments/BP_WeaponAttachment_Blaster.BP_WeaponAttachment_Blaster_C|GetMuzzleFlash (Variables|/Game/Character/BP_PlayerCharacter.BP_PlayerCharacter_C|GetWeaponAttached (Variables|Default|GetCharacterRef)))) "0, 0,90.000000" "2.000000,2.000000,2.000000")
  (Audio|PlaySound2D "/Game/Audio/SoundEffects/567308__bigdino1995__plasmacannon.567308__bigdino1995__plasmacannon" 1.0 1.0 0.0 0 0)
  (CallFunction|CheckTargetHit)
  (Utilities|Time|SetTimerbyEvent (delegate Custom|MoveShockwave) 0.5 true))

(fn ConstructionScript)

(fn MovetoNextTile
  (Utilities|IsValid (Variables|/Game/Blueprints/Grid/BP_GridTile.BP_GridTile_C|GetNeighborEast (Variables|Default|GetCurrentTile))
    (:Is%20Valid
      (Transformation|SetWorldLocation (Variables|Default|GetCollisionComponent) (Variables|/Game/Blueprints/Grid/BP_GridTile.BP_GridTile_C|GetGridWorldLocation (Variables|/Game/Blueprints/Grid/BP_GridTile.BP_GridTile_C|GetNeighborEast (Variables|Default|GetCurrentTile))) false false)
      (Audio|PlaySound2D "/Game/Audio/SoundEffects/584173__unfa__landing-forcefield.584173__unfa__landing-forcefield" 1.0 1.0 0.0 0 0)
      (Variables|Default|SetCurrentTile (Variables|/Game/Blueprints/Grid/BP_GridTile.BP_GridTile_C|GetNeighborEast (Variables|Default|GetCurrentTile)))
      (CallFunction|CheckTargetHit)
      (return))
    (:Is%20Not%20Valid
      (Actor|DestroyActor))))

(fn CheckTargetHit
  (bind _currenttile (Variables|Default|GetCurrentTile))
  (bind _occupyingactor (Variables|/Game/Blueprints/Grid/BP_GridTile.BP_GridTile_C|GetOccupyingActor _currenttile))
  (Utilities|IsValid _occupyingactor
    (:Is%20Valid
      (if (Actor|ActorHasTag _occupyingactor "Enemy")
        (Game|Damage|ApplyDamage _occupyingactor (Variables|Default|GetBase%20Damage) 0 0)))))

(fn SetSpawnLocation
  (Transformation|SetWorldLocation (Variables|Default|GetCollisionComponent) (Variables|/Game/Blueprints/Grid/BP_GridTile.BP_GridTile_C|GetGridWorldLocation (Variables|/Game/Blueprints/Grid/BP_GridTile.BP_GridTile_C|GetNeighborEast (Variables|Default|GetCurrentTile))) false false))

(fn GetPlayerTile
  (return 0))

(fn SetChargingAttack
  (params (IsChargingAttack :type Boolean))
  (return false))