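; BP_Attack_Pulse is a pulse attack that fires east along the tile grid from the player's tile.
; On BeginPlay it places its collision above that tile, plays a shot sound and resolves damage immediately.
; CheckDamage walks a bounded chain of east neighbors, damaging only the first Enemy-tagged occupant.
; Hitting an enemy only destroys the Niagara effect, so damage is independent of collision.
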(event EventBeginPlay
  (bind _playertile (Class|BPIAttackSystem|GetPlayerTile(Message) (Game|GetPlayerCharacter 0)))
  (bind _output_get (Variables|Default|SetCurrentTile _playertile))
  (Transformation|SetWorldLocation (Variables|Default|GetCollisionComponent) (+ (Variables|/Game/Blueprints/Grid/BP_GridTile.BP_GridTile_C|GetGridWorldLocation _output_get) "0,0.000000,100.000000") false false)
  (Audio|PlaySound2D "/Game/Audio/SoundEffects/Sci_Fi_Assault_Rifle_4.Sci_Fi_Assault_Rifle_4" 1.0 1.0 0.0 0 0)
  (CallFunction|CheckDamage))

(event Collision|EventHit
  (params (MyComp :type Primitive%20Component%20Object%20Reference) (Other :type Actor%20Object%20Reference) (OtherComp :type Primitive%20Component%20Object%20Reference) (bSelfMoved :type Boolean) (HitLocation :type Vector :default "0, 0, 0") (HitNormal :type Vector :default "0, 0, 0") (NormalImpulse :type Vector :default "0, 0, 0") (Hit :type Hit%20Result%20Structure%20%28by%20ref%29))
  (if (Actor|ActorHasTag Other "Enemy")
    (Components|DestroyComponent (Variables|Default|GetNiagara))))

(fn ConstructionScript)

(fn CheckDamage
  (Utilities|FlowControl|ForLoopwithBreak 0 10 :!label _label
    (:LoopBody
      (Utilities|IsValid (Variables|/Game/Blueprints/Grid/BP_GridTile.BP_GridTile_C|GetNeighborEast (Variables|Default|GetCurrentTile))
        (:Is%20Valid
          (bind _output_get (Variables|Default|SetCurrentTile (Variables|/Game/Blueprints/Grid/BP_GridTile.BP_GridTile_C|GetNeighborEast (Variables|Default|GetCurrentTile))))
          (Utilities|IsValid (Variables|/Game/Blueprints/Grid/BP_GridTile.BP_GridTile_C|GetOccupyingActor _output_get)
            (:Is%20Valid
              (if (Actor|ActorHasTag (Variables|/Game/Blueprints/Grid/BP_GridTile.BP_GridTile_C|GetOccupyingActor _output_get) "Enemy")
                (Game|Damage|ApplyDamage (Variables|/Game/Blueprints/Grid/BP_GridTile.BP_GridTile_C|GetOccupyingActor _output_get) (Variables|Default|GetBase%20Damage) 0 0)
                (goto _label Break)))))
        (:Is%20Not%20Valid
          (goto _label Break))))))

(fn GetPlayerTile
  (return 0))

(fn SetChargingAttack
  (params (IsChargingAttack :type Boolean))
  (return false))