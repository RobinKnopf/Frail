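; Grid-based shockwave attack that spawns one tile east of the player and damages an Enemy-tagged occupant.
; BeginPlay gets the player's tile and positions the collision component on its east neighbor, leaving CurrentTile unchanged.
; A non-looping timer later calls MoveToNextTile once, which advances CurrentTile east onto that spawn tile and checks for a hit, or destroys the actor without a neighbor.
; GetPlayerTile and SetChargingAttack are stubs.
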(event Custom|MoveShockwave
  (CallFunction|MovetoNextTile))

(event EventBeginPlay
  (bind _playertile (Class|BPIAttackSystem|GetPlayerTile(Message) (Game|GetPlayerCharacter 0)))
  (Variables|Default|SetCurrentTile _playertile)
  (CallFunction|SetSpawnLocation)
  (Utilities|Time|SetTimerbyEvent (delegate Custom|MoveShockwave) 2.0))

(fn ConstructionScript)

(fn MovetoNextTile
  (Utilities|IsValid (Variables|/Game/Blueprints/Grid/BP_GridTile.BP_GridTile_C|GetNeighborEast (Variables|Default|GetCurrentTile))
    (:Is%20Valid
      (Transformation|SetWorldLocation (Variables|Default|GetCollisionComponent) (Variables|/Game/Blueprints/Grid/BP_GridTile.BP_GridTile_C|GetGridWorldLocation (Variables|/Game/Blueprints/Grid/BP_GridTile.BP_GridTile_C|GetNeighborEast (Variables|Default|GetCurrentTile))) false false)
      (Variables|Default|SetCurrentTile (Variables|/Game/Blueprints/Grid/BP_GridTile.BP_GridTile_C|GetNeighborEast (Variables|Default|GetCurrentTile)))
      (CallFunction|CheckTargetHit)
      (return))
    (:Is%20Not%20Valid
      (Actor|DestroyActor))))

(fn CheckTargetHit
  (bind _currenttile (Variables|Default|GetCurrentTile))
  (bind _occupyingactor (Variables|/Game/Blueprints/Grid/BP_GridTile.BP_GridTile_C|GetOccupyingActor _currenttile))
  (Utilities|IsValid _occupyingactor
    (:Is%20Valid
      (if (Actor|ActorHasTag _occupyingactor "Enemy")
        (Game|Damage|ApplyDamage _occupyingactor (Variables|Default|GetBase%20Damage) 0 0)))))

(fn SetSpawnLocation
  (Transformation|SetWorldLocation (Variables|Default|GetCollisionComponent) (Variables|/Game/Blueprints/Grid/BP_GridTile.BP_GridTile_C|GetGridWorldLocation (Variables|/Game/Blueprints/Grid/BP_GridTile.BP_GridTile_C|GetNeighborEast (Variables|Default|GetCurrentTile))) false false))

(fn GetPlayerTile
  (return 0))

(fn SetChargingAttack
  (params (IsChargingAttack :type Boolean))
  (return false))