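; BP_Attack_Drill is a short-lived grid attack actor that strikes the tile east of the player character.
; On BeginPlay it reads the east neighbor from the player's tile message and moves its root just above that tile.
; It applies BaseDamage to the tile's occupying actor if tagged Enemy, then destroys itself after a brief delay.
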(event EventBeginPlay
  (bind _playertile (Class|BPIAttackSystem|GetPlayerTile(Message) (Game|GetPlayerCharacter 0)))
  (bind _output_get (Variables|Default|SetCurrentTile (Variables|/Game/Blueprints/Grid/BP_GridTile.BP_GridTile_C|GetNeighborEast _playertile)))
  (Transformation|SetWorldLocation (Variables|Default|GetDefaultSceneRoot) (+ (Variables|/Game/Blueprints/Grid/BP_GridTile.BP_GridTile_C|GetGridWorldLocation _output_get) "0, 0,100.000000") false false)
  (CallFunction|CheckDamage)
  (Utilities|FlowControl|Delay 0.5)
  (Actor|DestroyActor))

(fn ConstructionScript)

(fn CheckDamage
  (bind _currenttile (Variables|Default|GetCurrentTile))
  (bind _occupyingactor (Variables|/Game/Blueprints/Grid/BP_GridTile.BP_GridTile_C|GetOccupyingActor _currenttile))
  (Utilities|IsValid _occupyingactor
    (:Is%20Valid
      (if (Actor|ActorHasTag _occupyingactor "Enemy")
        (Game|Damage|ApplyDamage _occupyingactor (Variables|Default|GetBase%20Damage) 0 0)))))